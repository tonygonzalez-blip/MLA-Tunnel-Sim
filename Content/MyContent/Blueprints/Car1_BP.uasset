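; Car actor for a car wash: spawns as a random or chosen SUV, truck or sedan with a wash order, tags itself and joins the visual queue.
; Timelines drive acceleration and braking, with timed line traces stopping it behind obstacles and roller triggers handing movement to the tunnel conveyor.
; Trigger boxes along the body forward overlaps to wash machines.
; Invisible and short-lived low-LOD "silly" variants reuse the same spawn path.
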(event `Inv Car Step1`
  (for _array_element (`|MakeArray` (`self.Front Of Car`) (`self.Rear Of Car`) (`self.Rear Tires`) (`self.Front Tires`) (`self.Middle Of Car`) (`self.OverlapInsurance`)) :!label _label
    (`PrimitiveComponent.IgnoreActorWhenMoving` _array_element self true)))

(event `Spawn`
  (bind _overlapinsurance (`self.OverlapInsurance`))
  (bind _vehicle_body (`self.Vehicle Body`))
  (bind _vq_carselection (`self.VQ_CarSelection`))
  (bind _tags (`self.Tags`))
  (bind (_origin _boxextent) (`KismetSystemLibrary.GetComponentBounds` (`self.CollisionHull`)))
  (if (`self.Make Inv`)
    (`self.Inv Car Step1`)
    (`ActorComponent.K2_DestroyComponent` (`self.CollisionHull`))
    (`self.Car RNG`)
    (`self.Inv Car Step2`)
    (`self.Inv Car Step3`)
    (set `self.Services I was given` (`|MakeArray` (`self.VQ_Wash Ordered`)))
    (set `self.In Tunnel` true)
    (set `self.Driving Speed (cm/s)` (* (`self.Conveyor Speed`) 4.5))
    (else
      (`|ExecutionSequence` :!label _label_2
        (:`then_0`
          (goto _label))
        (:`then_1`
          (`self.Car RNG`)
          (`self.Set Meshes`)
          (`self.Start Run Check for Proxy Timer`))
        (:`then_2`
          (`StaticMeshComponent.SetStaticMesh` (`self.CollisionHull`) (select `int` (`self.VQ_CarSelection`) :`0` "/Game/MyContent/Meshes/Cars/SUV_Hull.SUV_Hull" :`1` "/Game/MyContent/Meshes/Cars/Truck_Hull.Truck_Hull" :`2` "/Game/MyContent/Meshes/Cars/Sedan_Hull.Sedan_Hull" :!type "StaticMesh Object Reference"))
          (for _array_element (`|MakeArray` (`self.Front Of Car`) (`self.Rear Of Car`) (`self.Rear Tires`) (`self.Front Tires`) (`self.Middle Of Car`) (`self.OverlapInsurance`))
            (`SceneComponent.K2_AttachToComponent` _array_element _vehicle_body "None" "KeepRelative" "KeepRelative" "KeepRelative" true))
          (`SceneComponent.K2_AttachToComponent` (`self.CollisionHull`) _vehicle_body "None" "KeepRelative" "KeepRelative" "KeepRelative" true))
        (:`then_3`
          (`BoxComponent.SetBoxExtent` _overlapinsurance _boxextent true :!label _label_3)
          (`SceneComponent.K2_SetWorldLocation` _overlapinsurance _origin false false)
          (for (_array_element_2 _array_index) (`|MakeArray` (`self.Front Of Car`) (`self.Rear Of Car`) (`self.Middle Of Car`) (`self.Front Tires`) (`self.Rear Tires`))
            (`SceneComponent.K2_SetRelativeLocation` _array_element_2 (`KismetMathLibrary.MakeVector` 0.0 (`|GetArrayItem` (select `int` (`self.VQ_CarSelection`) :`0` (`|MakeArray` -248.0 248.0 14.0 -161.0 140.0) :`1` (`|MakeArray` -240.0 303.0 90.0 -161.0 185.0) :`2` (`|MakeArray` -257.0 245.0 14.0 -161.0 138.0)) _array_index) 100.0) false false)))
        (:`then_4`
          ; CarID Tag (Index 2)
          (`KismetArrayLibrary.Array_Add` (`self.Tags`) (`KismetStringLibrary.Conv_StringToName` (`KismetStringLibrary.Conv_DoubleToString` (`GameplayStatics.GetRealTimeSeconds`))) :!label _label_4)
          (`KismetArrayLibrary.Array_Add` _tags (select `int` _vq_carselection :`0` "SUV" :`1` "Truck" :`2` "Sedan"))
          (if (== _vq_carselection 1)
            (`KismetArrayLibrary.Array_Add` _tags "PickupBed"))
          (`self.K2_AddActorLocalOffset` (select `int` (`self.VQ_CarSelection`) :`0` (0.0 0.0 0.0) :`1` (8.0 0.0 0.0) :`2` (0.0 0.0 0.0) :!type "Vector Structure")))
        (:`then_5`
          (if (`self.Is Silly`)
            (`self.Reconfigure for Silly Car`)))))))

(event `self.ReceiveBeginPlay`
  (if (`self.Enable Tick`)
    (if (`self.Is For Level Sequence`)
      (goto _label_2))
    (else
      (`self.SetActorTickEnabled` false))))

(event `self.Front Of Car.OnComponentBeginOverlap`
  (params (OverlappedComponent :type "PrimitiveComponent Object Reference") (OtherActor :type "Actor Object Reference") (OtherComp :type "PrimitiveComponent Object Reference") (OtherBodyIndex :type Integer) (bFromSweep :type Boolean) (SweepResult :type "HitResult Structure (by ref)"))
  (`self.Car Overlap Event Dispatch` OverlappedComponent OtherActor OtherComp self))

(event `self.Front Tires.OnComponentBeginOverlap`
  (params (OverlappedComponent :type "PrimitiveComponent Object Reference") (OtherActor :type "Actor Object Reference") (OtherComp :type "PrimitiveComponent Object Reference") (OtherBodyIndex :type Integer) (bFromSweep :type Boolean) (SweepResult :type "HitResult Structure (by ref)"))
  (`self.Car Overlap Event Dispatch` OverlappedComponent OtherActor OtherComp self))

(event `Inv Car Step3`
  (goto _label_4))

(event `Inv Car Step2`
  (goto _label_3))

(event `self.Rear Of Car.OnComponentBeginOverlap`
  (params (OverlappedComponent :type "PrimitiveComponent Object Reference") (OtherActor :type "Actor Object Reference") (OtherComp :type "PrimitiveComponent Object Reference") (OtherBodyIndex :type Integer) (bFromSweep :type Boolean) (SweepResult :type "HitResult Structure (by ref)"))
  (`self.Car Overlap Event Dispatch` OverlappedComponent OtherActor OtherComp self))

(event `self.Rear Tires.OnComponentBeginOverlap`
  (params (OverlappedComponent :type "PrimitiveComponent Object Reference") (OtherActor :type "Actor Object Reference") (OtherComp :type "PrimitiveComponent Object Reference") (OtherBodyIndex :type Integer) (bFromSweep :type Boolean) (SweepResult :type "HitResult Structure (by ref)"))
  (`self.Car Overlap Event Dispatch` OverlappedComponent OtherActor OtherComp self))

(event `self.Middle Of Car.OnComponentBeginOverlap`
  (params (OverlappedComponent :type "PrimitiveComponent Object Reference") (OtherActor :type "Actor Object Reference") (OtherComp :type "PrimitiveComponent Object Reference") (OtherBodyIndex :type Integer) (bFromSweep :type Boolean) (SweepResult :type "HitResult Structure (by ref)"))
  (`self.Car Overlap Event Dispatch` OverlappedComponent OtherActor OtherComp self))

(event `Car Summon`
  (params (`Is Silly` :type Boolean) (`Car Selection` :type Integer :default -1) (`Wash Selection` :type Integer :default -1) (`Make Inv` :type Boolean))
  (set `self.VQ_CarSelection` `Car Selection`)
  (set `self.VQ_Wash Ordered` `Wash Selection`)
  (set `self.Make Inv` `Make Inv`)
  (bind _output_get (set `self.Is Silly` `Is Silly`))
  (if _output_get
    (set `self.Tags` (`|MakeArray` "sillyCar" :!type "Name"))
    (`PrimitiveComponent.SetCollisionResponseToChannel` (`self.CollisionHull`) "ECC_WorldStatic" "ECR_Ignore")
    (`self.Spawn`)
    (`self.Start Accelerating`)
    (`KismetSystemLibrary.Delay` 8.0)
    (`self.K2_DestroyActor`)
    (else
      (`|ExecutionSequence`
        (:`then_0`
          (`self.Spawn`))
        (:`then_1`
          (bind _outactors (`GameplayStatics.GetAllActorsOfClass` "/Game/MyContent/Blueprints/ConfigurableMachines/TunnelConveyorRollers_BP.TunnelConveyorRollers_BP_C"))
          (if (`KismetArrayLibrary.Array_IsNotEmpty` _outactors)
            (`self.Set Conveyor Speed` (`/Game/MyContent/Blueprints/ConfigurableMachines/TunnelConveyorRollers_BP.Conveyor Speed` (`|GetArrayItem` _outactors)))))
        (:`then_2`
          (`self.Attempt to Add Self to VQ`))
        (:`then_3`
          (`self.Start Accelerating`)
          (if (`self.Make Inv`)
            (set `self.Timeline Finished_0` true)
            (for _array_element (`self.Tags`)
              (`KismetSystemLibrary.PrintString` (`KismetStringLibrary.Conv_NameToString` _array_element)))))))))

(event `Increment Decal Sort Order`
  (`/Engine/EditorBlueprintResources/StandardMacros.IncrementInt` (`self.Current Decal Sort Order`)))

(event `Start Accelerating`
  (bind _returnvalue (`self.K2_GetActorLocation` self))
  ; Accelerate
  (bind (_direction _lerp) (`Timeline|Timeline` :!label _label_5)
    (:`Update`
      (`self.K2_SetActorLocation` (`KismetMathLibrary.VLerp` _returnvalue (+ _returnvalue (* (`self.GetActorRightVector` self) (* (* (`GameplayStatics.GetWorldDeltaSeconds`) (`self.Driving Speed (cm/s)`)) (`KismetMathLibrary.SelectFloat` -50.0 -1.0 (`self.Is Silly`))))) _lerp) :!label _label_6))
    (:`Finished`
      (if (`|EnumEquality` _direction "Forward")
        (set `self.Timeline Finished` true)
        (if (not (`self.In Tunnel`))
          (`self.Start Gradual Spd Up Timer`))
        (else
          (set `self.Timeline Finished` false)
          (`KismetSystemLibrary.K2_ClearAndInvalidateTimerHandle` (`self.Gradual Speed increase Timer Ref`)))))))

(event `/Game/FirstPerson/Blueprints/ConfigMachine_BPI.Conveyor Turned On`
  (if (`self.In Tunnel`)
    (`self.SetActorTickEnabled` true)))

(event `self.ReceiveTick`
  (params (DeltaSeconds :type "Float (single-precision)"))
  (if (not (`GameplayStatics.IsGamePaused`))
    (`|ExecutionSequence`
      (:`then_0`
        (`self.Drive`))
      (:`then_1`
        (if (not (`self.Make Inv`))
          ; Tire Rotation
          (for _array_element (`self.Vehicle Wheels`)
            (bind (_returnvalue_x _returnvalue_y) (`KismetMathLibrary.BreakVector` (`SceneComponent.K2_GetComponentLocation` _array_element)))
            (`SceneComponent.K2_SetRelativeRotation` _array_element (`KismetMathLibrary.MakeRotator` (* _returnvalue_y 1.67)) false false))))
      (:`then_2`
        (`self.Roll with Conveyor`)))))

(event `Start Decelerating`
  ; Accelerate
  (set `self.Timeline Finished` false)
  (goto _label_5 :!via `Reverse`))

(event `/Game/FirstPerson/Blueprints/ConfigMachine_BPI.Conveyor Turned Off`
  (if (`self.In Tunnel`)
    (`self.SetActorTickEnabled` false)))

(event `Drive`
  ; Accelerate
  (if (`self.Timeline Finished`)
    (goto _label_6)))

(event `Roller Trig Reached`
  ; Accelerate
  (`/Engine/EditorBlueprintResources/StandardMacros.DoOnce` (`self.Make Inv`)
    (:`Completed`
      (set `self.In Tunnel` true)
      (`self.Start Decelerating`)
      (`KismetSystemLibrary.K2_ClearAndInvalidateTimerHandle` (`self.Run Check for Proxy Timer Ref`)))))

(event `Send Car`
  (params (`Services I was given` :type "Array of Integer"))
  (set `self.Services I was given` `Services I was given`)
  (bind _outactors (`GameplayStatics.GetAllActorsOfClassWithTag` "/Script/Engine.TriggerVolume" "car_QueueHere"))
  (`KismetArrayLibrary.Array_Add` (`self.Actors to Ignore (Proxy Check)`) (`|GetArrayItem` _outactors))
  (`self.Start Accelerating`)
  (set `self.Was Breaking` false)
  (`KismetSystemLibrary.K2_ClearAndInvalidateTimerHandle` (`self.Gradual Speed increase Timer Ref`))
  (set `self.Driving Speed (cm/s)` (`self.Driving Speed (cm/s)_Default`)))

(event `Start Gradual Spd Up Timer`
  ; Accelerate
  (bind _returnvalue (`KismetSystemLibrary.K2_SetTimerDelegate` (delegate `Gradual speed increase`) 2.0 true))
  (set `self.Gradual Speed increase Timer Ref` _returnvalue))

(event `Go`
  ; Accelerate
  (if (not (`self.In Tunnel`)) :!label _label_7
    (set `self.Driving Speed (cm/s)` (`self.Driving Speed (cm/s)_Default`))
    (`self.Start Accelerating`)
    (else
      (`KismetSystemLibrary.Delay` 0.2)
      (goto _label_7))))

(event `Start Run Check for Proxy Timer`
  (bind _returnvalue (`KismetSystemLibrary.K2_SetTimerDelegate` (delegate `Run Check for Proximity`) 1.0 true))
  (set `self.Run Check for Proxy Timer Ref` _returnvalue))

(event `Gradual speed increase`
  (bind _driving_speed__cm_s_ (`self.Driving Speed (cm/s)`))
  ; Accelerate
  (bind (_direction _lerp) (`Timeline|Timeline_1` :!via `PlayFromStart`)
    (:`Update`
      (set `self.Driving Speed (cm/s)` (`KismetMathLibrary.Lerp` _driving_speed__cm_s_ (+ _driving_speed__cm_s_ 0.2) _lerp)))
    (:`Finished`
      (set `self.Driving Speed (cm/s)` (`self.Driving Speed (cm/s)_Default`)))))

(event `Roll with Conveyor`
  (bind _returnvalue (`self.K2_GetActorLocation` self))
  ; Roll with conveyor
  (if (`self.Timeline Finished_0`)
    (`self.K2_SetActorLocation` (`KismetMathLibrary.VLerp` _returnvalue (+ _returnvalue (* (`self.GetActorRightVector` self) (* (`GameplayStatics.GetWorldDeltaSeconds`) (* (`self.Conveyor Speed`) -4.5)))) (stale `self.CollisionHull.OnComponentHit` _lerp)) true true :!label _label_8)))

(event `Wait`
  ; Accelerate
  (if (not (`self.In Tunnel`))
    (`self.Start Decelerating`)))

(event `Run Check for Proximity`
  (`self.Check for proximity`))

(event `self.CollisionHull.OnComponentHit`
  (params (HitComponent :type "PrimitiveComponent Object Reference") (OtherActor :type "Actor Object Reference") (OtherComp :type "PrimitiveComponent Object Reference") (NormalImpulse :type "Vector Structure") (Hit :type "HitResult Structure (by ref)"))
  (if (and (`ActorComponent.ComponentHasTag` OtherComp "roller") (`self.In Tunnel`))
    (`/Engine/EditorBlueprintResources/StandardMacros.DoOnce` false
      (:`Completed`
        ; Roll with conveyor
        (set `self.Timeline Finished` false)
        (set `self.Driving Speed (cm/s)` (`self.Conveyor Speed`))
        (bind (_direction _lerp) (`Timeline|Timeline_0` :!via `PlayFromStart`)
          (:`Update`
            (goto _label_8))
          (:`Finished`
            (bind _isa (`/Engine/EditorBlueprintResources/StandardMacros.FlipFlop`)
              (:`A`
                _)
              (:`B`
                _))
            (set `self.Timeline Finished_0` _isa)))))))

(event `/Game/FirstPerson/Blueprints/ConfigMachine_BPI.Reset all save data`
  ; Roll with conveyor
  (set `self.Conveyor Speed` 5.0))

(event `Roller Finished`
  (`/Engine/EditorBlueprintResources/StandardMacros.DoOnce` false
    (:`Completed`
      (`self.Start Run Check for Proxy Timer`)
      (`self.Start Gradual Spd Up Timer`)
      (set `self.In Tunnel` false)
      (bind _foundwidgets (`WidgetBlueprintLibrary.GetAllWidgetsOfClass` "/Game/FirstPerson/Blueprints/VisualQueue_WBP.VisualQueue_WBP_C"))
      (`/Game/FirstPerson/Blueprints/VisualQueue_WBP.Update Controller Queue` (`|GetArrayItem` _foundwidgets) (`|GetArrayItem` (`self.Tags`) 2) false))))

(event `Set Conveyor Speed`
  (params (`Conveyor Speed` :type "Float (double-precision)"))
  ; Roll with conveyor
  (set `self.Conveyor Speed` `Conveyor Speed`))

(fn `Attempt to Add Self to VQ`
  (locals (Attempts :type Integer))
  (if (not (`self.Make Inv`))
    (bind _foundwidgets (`WidgetBlueprintLibrary.GetAllWidgetsOfClass` "/Game/FirstPerson/Blueprints/VisualQueue_WBP.VisualQueue_WBP_C" :!label _label))
    (bind _result (`/Engine/EditorBlueprintResources/StandardMacros.IncrementInt` (`local.Attempts`))
      (:`  `
        (if (< _result 3)
          (if (`KismetArrayLibrary.Array_IsNotEmpty` _foundwidgets)
            (`/Game/FirstPerson/Blueprints/VisualQueue_WBP.Add Ticket to Queue` (`|GetArrayItem` _foundwidgets) (`self.VQ_CarSelection`) (`self.VQ_Wash Ordered`) (`|GetArrayItem` (`self.Tags`) 2))
            (else
              (bind _asbp_first_person_character (cast `/Game/FirstPerson/Blueprints/BP_FirstPersonCharacter` (`GameplayStatics.GetPlayerCharacter` 0)))
              (`/Game/FirstPerson/Blueprints/BP_FirstPersonCharacter.Close VQ Menu` _asbp_first_person_character false)
              (goto _label)))
          (else
            ; Added in response to an infinite loop I experienced while attempting to open/close a menu while a car was spawning. Something about setting the player state.
            (`KismetSystemLibrary.PrintString` "Car failed to find VQ, destroying self!" true true (struct :`R` 1.0 :`G` 1.0 :`A` 1.0) 5.0)
            (`self.K2_DestroyActor` self)))))))

(fn `Car Overlap Event Dispatch`
  (params (`Overlapped Component` :type "PrimitiveComponent Object Reference") (`Other Actor` :type "Actor Object Reference") (`Other Component` :type "PrimitiveComponent Object Reference") (`Self Ref` :type "/Game/MyContent/Blueprints/Car1_BP Object Reference"))
  (locals (`Master Machine Modifiers` :type "Array of /Game/MyContent/Blueprints/ModifierProperties_STRUCT Structure") (`Master Machine Relay` :type Integer :default 0) (`Matching trig Index` :type Integer))
  (for _array_element (`|MakeArray` "Trig_On" "Trig_Off" "Trig_Distance" "Trig_Duration" "Trig_Modifier" "Trig_Extra" :!type "Name")
    (bind _returnvalue (!= (`KismetArrayLibrary.Array_Find` (`ActorComponent.ComponentTags` `Other Component`) _array_element) -1))
    (if _returnvalue
      (break)))
  (if _returnvalue
    (bind _asmaster_machine_bp (cast `/Game/MyContent/Blueprints/ConfigurableMachines/MasterMachine_BP` (`local.Other Actor`)))
    (`/Game/MyContent/Blueprints/ConfigurableMachines/MasterMachine_BP.Trig Overlapped` _asmaster_machine_bp (`local.Self Ref`) (`ActorComponent.ComponentTags` `Other Component`) (`|GetArrayItem` (`ActorComponent.ComponentTags` (`local.Overlapped Component`))))))

(fn `Car RNG`
  (locals (`Car_RNG table` :type "Array of Integer") (`Available Washes Service #'s` :type "Array of Integer"))
  (`|ExecutionSequence`
    (:`then_0`
      (bind _asmain_game_instance_gi (cast `/Game/FirstPerson/Blueprints/MainGameInstance_GI` (`GameplayStatics.GetGameInstance`)))
      (bind _services (`/Game/FirstPerson/Blueprints/MainGameInstance_GI.Services` _asmain_game_instance_gi))
      (for _array_element _services
        (bind _returnvalue (== (`.Type_9_578A34BE475ACCAAFBE34397A0D878EC` (break `/Game/FirstPerson/Blueprints/ServiceProperties_STRUCT` _array_element)) 3))
        (if _returnvalue
          (break)))
      (if _returnvalue
        (for _array_element_2 _services
          (bind (_none _description _type) (break `/Game/FirstPerson/Blueprints/ServiceProperties_STRUCT` _array_element_2))
          (if (== _type 3)
            (`KismetArrayLibrary.Array_Add` (`local.Available Washes Service #'s`) _none)))))
    (:`then_1`
      (if (== (`self.VQ_Wash Ordered`) -1)
        (set `self.VQ_Wash Ordered` (`KismetArrayLibrary.Array_Random` (`local.Available Washes Service #'s`)))))
    (:`then_2`
      (if (== (`self.VQ_CarSelection`) -1)
        (`KismetArrayLibrary.Array_Clear` (`local.Car_RNG table`))
        (for _index (range 100)
          (if (> _index 34)
            (if (> _index 69)
              (`KismetArrayLibrary.Array_Add` (`local.Car_RNG table`) 2)
              (else
                (`KismetArrayLibrary.Array_Add` (`local.Car_RNG table`) 1)))
            (else
              (`KismetArrayLibrary.Array_Add` (`local.Car_RNG table`)))))
        (set `self.VQ_CarSelection` (`KismetArrayLibrary.Array_Random` (`local.Car_RNG table`)))))))

(fn `Check for proximity`
  (locals (`Line Trace X Offset` :type "Float (double-precision)") (`Actor was hit` :type Boolean))
  (bind _line_trace_x_offset (`local.Line Trace X Offset`))
  (bind _front_of_car (`self.Front Of Car`))
  (bind _returnvalue (`SceneComponent.K2_GetComponentLocation` _front_of_car))
  (set `local.Line Trace X Offset` 210.0)
  (for _ (range 5)
    (set `local.Line Trace X Offset` (- (`local.Line Trace X Offset`) 70.0))
    (bind (_outhit _returnvalue_2) (`KismetSystemLibrary.LineTraceSingle` (+ _returnvalue (`KismetMathLibrary.MakeVector` (/ _line_trace_x_offset 2.0))) (+ (+ _returnvalue (* (`SceneComponent.GetRightVector` _front_of_car) (* (`self.Driving Speed (cm/s)`) -3.0))) (`KismetMathLibrary.MakeVector` _line_trace_x_offset)) "TraceTypeQuery2" false (`self.Actors to Ignore (Proxy Check)`) "None" true (struct :`R` 1.0 :`A` 1.0) (struct :`G` 1.0 :`A` 1.0) 1.0))
    (if _returnvalue_2
      (bind (_bblockinghit _binitialoverlap _time _distance _location _impactpoint _normal _impactnormal _physmat _hitactor _hitcomponent) (`GameplayStatics.BreakHitResult` _outhit))
      (if (or (`self.ActorHasTag` _hitactor "car") (`self.ActorHasTag` _hitactor "car_QueueHere") (`self.ActorHasTag` _hitactor "player") (`ActorComponent.ComponentHasTag` _hitcomponent "CarWaitForRollers"))
        (set `local.Actor was hit` true)
        (break))))
  (`|ExecutionSequence`
    (:`then_0`
      (if (`local.Actor was hit`)
        (if (not (`self.Was Breaking`))
          (`self.Start Decelerating`)
          (set `self.Was Breaking` true))
        (elif (`self.Was Breaking`)
          (`self.Start Accelerating`)
          (set `self.Was Breaking` false))))
    (:`then_1`
      (set `local.Actor was hit` false))))

(fn `Reconfigure for Silly Car`
  (`|ExecutionSequence`
    (:`then_0`
      (`|ExecutionSequence`
        (:`then_0`
          (`StaticMeshComponent.SetForcedLodModel` (`self.Vehicle Body`) 3))
        (:`then_1`
          (for _array_element (`self.Vehicle Wheel Assemblys`)
            (`StaticMeshComponent.SetForcedLodModel` _array_element 3)))
        (:`then_2`
          (for _array_element_2 (`self.Vehicle Wheels`)
            (`StaticMeshComponent.SetForcedLodModel` _array_element_2 3)))))
    (:`then_1`
      (`KismetSystemLibrary.K2_ClearAndInvalidateTimerHandle` (`self.Run Check for Proxy Timer Ref`))
      (for _array_element_3 (`|MakeArray` (`self.Rear Tires`) (`self.Front Tires`) (`self.Rear Of Car`) (`self.Front Of Car`) (`self.Middle Of Car`) (`self.OverlapInsurance`) :!type "ActorComponent Object Reference")
        (`ActorComponent.K2_DestroyComponent` _array_element_3)))))

(fn `Set Meshes`
  (locals (`Wheel Assembly Sockets` :type "Array of Name") (`Wheel Sockets` :type "Array of Name"))
  (`|ExecutionSequence`
    (:`then_0`
      (bind _returnvalue (`AddComponent|NODE_AddStaticMeshComponent-1`))
      (`StaticMeshComponent.SetStaticMesh` _returnvalue (select `int` (`self.VQ_CarSelection`) :`0` "/Game/MyContent/Meshes/Cars/SUV_Body_MESH.SUV_Body_MESH" :`1` "/Game/MyContent/Meshes/Cars/Truck_Body_MESH.Truck_Body_MESH" :`2` "/Game/MyContent/Meshes/Cars/Sedan_Body_MESH.Sedan_Body_MESH" :!type "StaticMesh Object Reference"))
      (bind _output_get (set `self.Vehicle Body` _returnvalue))
      (`PrimitiveComponent.SetAffectDynamicIndirectLighting` _output_get false)
      (`PrimitiveComponent.SetRenderCustomDepth` _output_get true)
      (`PrimitiveComponent.SetCustomDepthStencilValue` _output_get 2)
      (set `PrimitiveComponent.bGenerateOverlapEvents` true _output_get)
      (bind _returnvalue_2 (`GameplayStatics.SpawnDecalAttached` "/Game/MyContent/maskExclusionDecal.maskExclusionDecal" (select `int` (`self.VQ_CarSelection`) :`0` (60.0 280.0 100.0) :`1` (39.0 300.0 120.0) :`2` (50.0 250.0 105.0) :!type "Vector Structure") _output_get "None" (select `int` (`self.VQ_CarSelection`) :`0` (0.0 0.0 50.0) :`1` (0.0 30.0 35.0) :`2` (0.0 -10.0 50.0) :!type "Vector Structure") (struct :`Pitch` 90.0)))
      (`DecalComponent.SetSortOrder` _returnvalue_2 999))
    (:`then_1`
      (for _array_element (`SceneComponent.GetAllSocketNames` (`self.Vehicle Body`))
        (if (`KismetStringLibrary.Contains` (`KismetStringLibrary.Conv_NameToString` _array_element) "Assembly")
          (`KismetArrayLibrary.Array_Add` (`local.Wheel Assembly Sockets`) _array_element)
          (else
            (`KismetArrayLibrary.Array_Add` (`local.Wheel Sockets`) _array_element)))))
    (:`then_2`
      (`KismetArrayLibrary.Array_Clear` (`self.Vehicle Wheel Assemblys`))
      (for _index (range 4)
        (bind _returnvalue_3 (`AddComponent|NODE_AddStaticMeshComponent-3`))
        (`StaticMeshComponent.SetStaticMesh` _returnvalue_3 (select `int` (`self.VQ_CarSelection`) :`0` "/Game/MyContent/Meshes/Cars/SUV_Wheel_Assembly_MESH.SUV_Wheel_Assembly_MESH" :`1` "/Game/MyContent/Meshes/Cars/Truck_Wheel_Assembly_MESH.Truck_Wheel_Assembly_MESH" :`2` "/Game/MyContent/Meshes/Cars/Sedan_Wheel_Assembly_MESH.Sedan_Wheel_Assembly_MESH" :!type "StaticMesh Object Reference"))
        (`PrimitiveComponent.SetAffectDynamicIndirectLighting` _returnvalue_3 false)
        (`PrimitiveComponent.SetRenderCustomDepth` _returnvalue_3 true)
        (`PrimitiveComponent.SetCustomDepthStencilValue` _returnvalue_3 2)
        (set `PrimitiveComponent.bGenerateOverlapEvents` false _returnvalue_3)
        (bind _output (`|GetArrayItem` (`local.Wheel Assembly Sockets`) _index))
        (if (!= _output "None")
          (`SceneComponent.K2_AttachToComponent` _returnvalue_3 (`self.Vehicle Body`) _output "KeepRelative" "KeepRelative" "KeepRelative" true)
          (`KismetArrayLibrary.Array_Add` (`self.Vehicle Wheel Assemblys`) _returnvalue_3))))
    (:`then_3`
      (`KismetArrayLibrary.Array_Clear` (`self.Vehicle Wheels`))
      (for _index_2 (range 4)
        (bind _returnvalue_4 (`AddComponent|NODE_AddStaticMeshComponent-4`))
        (`StaticMeshComponent.SetStaticMesh` _returnvalue_4 (select `int` (`self.VQ_CarSelection`) :`0` "/Game/MyContent/Meshes/Cars/SUV_Wheel_MESH.SUV_Wheel_MESH" :`1` "/Game/MyContent/Meshes/Cars/Truck_Wheel_MESH.Truck_Wheel_MESH" :`2` "/Game/MyContent/Meshes/Cars/Sedan_Wheel_MESH.Sedan_Wheel_MESH" :!type "StaticMesh Object Reference"))
        (`PrimitiveComponent.SetAffectDynamicIndirectLighting` _returnvalue_4 false)
        (`PrimitiveComponent.SetRenderCustomDepth` _returnvalue_4 true)
        (`PrimitiveComponent.SetCustomDepthStencilValue` _returnvalue_4 2)
        (set `PrimitiveComponent.bGenerateOverlapEvents` false _returnvalue_4)
        (bind _output_2 (`|GetArrayItem` (`local.Wheel Sockets`) _index_2))
        (if (and (!= _output_2 "None") (`KismetSystemLibrary.IsValid` (`|GetArrayItem` (`self.Vehicle Wheel Assemblys`) _index_2)))
          (`SceneComponent.K2_AttachToComponent` _returnvalue_4 (`self.Vehicle Body`) _output_2 "KeepRelative" "KeepRelative" "KeepRelative" true)
          (`KismetArrayLibrary.Array_Add` (`self.Vehicle Wheels`) _returnvalue_4))))))

(fn `UserConstructionScript`
  (bind _collisionhull (`self.CollisionHull`))
  (set `self.Tags` (`|MakeArray` "car" "nograb" :!type "Name"))
  (`PrimitiveComponent.SetRenderInMainPass` _collisionhull false)
  (`PrimitiveComponent.SetRenderInDepthPass` _collisionhull false))