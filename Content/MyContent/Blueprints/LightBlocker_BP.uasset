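; Light blocker actor that toggles whether hidden static meshes affect indirect lighting, based on first-person character presence in its Trigger.
; On BeginPlay it gathers recursively attached StaticMeshActors, hides them in game and disables their collision.
; It checks existing overlaps one tick later, then updates on begin and end overlap via SetAffectIndirectLightingWhileHidden.
; By default meshes affect lighting while the character is inside; InvertOperation reverses this.
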(event `self.ReceiveBeginPlay`
  (bind _invert_operation (`self.Invert Operation`))
  (for _array_element (`self.GetAttachedActors` true true)
    (bind _asstatic_mesh_actor (cast `StaticMeshActor` _array_element))
    (`KismetArrayLibrary.Array_Add` (`self.Attached Actors`) _asstatic_mesh_actor))
  (for _array_element_2 (`self.Attached Actors`)
    (`PrimitiveComponent.SetAffectIndirectLightingWhileHidden` (`StaticMeshActor.StaticMeshComponent` _array_element_2) true)
    (`self.SetActorEnableCollision` _array_element_2 false)
    (`self.SetActorHiddenInGame` _array_element_2 true))
  (`KismetSystemLibrary.DelayUntilNextTick`)
  (if (`KismetArrayLibrary.Array_IsNotEmpty` (`PrimitiveComponent.GetOverlappingActors` (`self.Trigger`) "/Game/FirstPerson/Blueprints/BP_FirstPersonCharacter.BP_FirstPersonCharacter_C"))
    (for _array_element_3 (`self.Attached Actors`) :!label _label
      (`PrimitiveComponent.SetAffectIndirectLightingWhileHidden` (`StaticMeshActor.StaticMeshComponent` _array_element_3) (not _invert_operation)))
    (else
      (for _array_element_4 (`self.Attached Actors`) :!label _label_2
        (`PrimitiveComponent.SetAffectIndirectLightingWhileHidden` (`StaticMeshActor.StaticMeshComponent` _array_element_4) _invert_operation)))))

(event `self.Trigger.OnComponentBeginOverlap`
  (params (OverlappedComponent :type "PrimitiveComponent Object Reference") (OtherActor :type "Actor Object Reference") (OtherComp :type "PrimitiveComponent Object Reference") (OtherBodyIndex :type Integer) (bFromSweep :type Boolean) (SweepResult :type "HitResult Structure (by ref)"))
  (`KismetSystemLibrary.IsObjectOfSoftClass` OtherActor "/Game/FirstPerson/Blueprints/BP_FirstPersonCharacter.BP_FirstPersonCharacter_C"
    (:`True`
      (goto _label))))

(event `self.Trigger.OnComponentEndOverlap`
  (params (OverlappedComponent :type "PrimitiveComponent Object Reference") (OtherActor :type "Actor Object Reference") (OtherComp :type "PrimitiveComponent Object Reference") (OtherBodyIndex :type Integer))
  (`KismetSystemLibrary.IsObjectOfSoftClass` OtherActor "/Game/FirstPerson/Blueprints/BP_FirstPersonCharacter.BP_FirstPersonCharacter_C"
    (:`True`
      (goto _label_2))))

(fn `UserConstructionScript`)