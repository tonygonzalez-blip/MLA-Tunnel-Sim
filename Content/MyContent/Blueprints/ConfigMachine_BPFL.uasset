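; Blueprint function library of shared helpers for car wash machines.
; Lookups read relay and service data from MainGameInstance_GI and find MasterMachine_BP actors by relay, default relay, dummy tag or object name.
; Mask decals attach to cars, stretch between start and end marker components tracked in maps by car ID, and have a fallback removing the last entry.
; Other helpers aim pistons, set cable ends and flip signs by PhotoEyes position.
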(fn `Cable Construction Script`
  (params (`Self Ref` :type "Actor Object Reference") (Cable :type "CableComponent Object Reference") (Cable1 :type "CableComponent Object Reference"))
  (bind _returnvalue (`Actor.K2_GetActorLocation` `Self Ref`))
  (bind _cable (`local.Cable`))
  (bind _cable1 (`local.Cable1`))
  (bind _asmaster_machine_bp (cast `/Game/MyContent/Blueprints/ConfigurableMachines/MasterMachine_BP` (`Actor.GetOwner` `Self Ref`)))
  (`|ExecutionSequence`
    (:`then_0`
      (bind (_returnvalue_x _returnvalue_y _returnvalue_z) (`KismetMathLibrary.BreakVector` (- (`/Game/MyContent/Blueprints/ConfigurableMachines/MasterMachine_BP.Cable End Location` _asmaster_machine_bp) _returnvalue)))
      (bind _returnvalue_2 (`KismetMathLibrary.SelectFloat` -1.0 1.0 (`/Game/MyContent/Blueprints/ConfigurableMachines/MasterMachine_BP.Im Backwards` _asmaster_machine_bp)))
      (set `CableComponent.EndLocation` (`KismetMathLibrary.MakeVector` _returnvalue_x (* _returnvalue_y _returnvalue_2) _returnvalue_z) _cable)
      (bind _cable_length (`/Game/MyContent/Blueprints/ConfigurableMachines/MasterMachine_BP.Cable Length` _asmaster_machine_bp))
      (set `CableComponent.CableLength` _cable_length _cable))
    (:`then_1`
      (`/Engine/EditorBlueprintResources/StandardMacros.IsValid` (`local.Cable1`)
        (:`Is Valid`
          (bind (_returnvalue_x_2 _returnvalue_y_2 _returnvalue_z_2) (`KismetMathLibrary.BreakVector` (- (`/Game/MyContent/Blueprints/ConfigurableMachines/MasterMachine_BP.Cable End Location2` _asmaster_machine_bp) _returnvalue)))
          (set `CableComponent.EndLocation` (`KismetMathLibrary.MakeVector` _returnvalue_x_2 (* _returnvalue_y_2 _returnvalue_2) _returnvalue_z_2) _cable1)
          (set `CableComponent.CableLength` _cable_length _cable1))))))

(fn `Destroy Attached Mask Decal`
  (params (`Car ID` :type "Name (by ref)") (`Decal Start Positions In` :type "Map of Name to BoxComponent Object Reference (by ref)") (`Decal End Positions In` :type "Map of Name to BoxComponent Object Reference (by ref)") (`Spawned Decals In` :type "Map of Name to DecalComponent Object Reference (by ref)") (`Self Ref` :type "Actor Object Reference"))
  (returns (`Decal Start Positions Out` :type "Map of Name to BoxComponent Object Reference (by ref)") (`Decal End Positions Out` :type "Map of Name to BoxComponent Object Reference (by ref)") (`Spawned Decals Out` :type "Map of Name to DecalComponent Object Reference (by ref)"))
  (locals (`Dec Starts` :type "Map of Name to BoxComponent Object Reference") (`Dec Ends` :type "Map of Name to BoxComponent Object Reference") (`Spwnd Decs` :type "Map of Name to DecalComponent Object Reference") (`Dec Start Comp to Destroy` :type "BoxComponent Object Reference") (`Dec End Comp to Destroy` :type "BoxComponent Object Reference") (`Dec Component to Destroy` :type "DecalComponent Object Reference"))
  (bind _dec_ends (`local.Dec Ends`))
  (bind _spwnd_decs (`local.Spwnd Decs`))
  (bind _car_id (`local.Car ID`))
  (bind _car_id_2 (`local.Car ID`))
  (bind _dec_starts (`local.Dec Starts`))
  (bind (_value _returnvalue) (`BlueprintMapLibrary.Map_Find` (`local.Dec Starts`) _car_id_2))
  (bind (_value_2 _returnvalue_2) (`BlueprintMapLibrary.Map_Find` (`local.Dec Ends`) _car_id_2))
  (bind (_value_3 _returnvalue_3) (`BlueprintMapLibrary.Map_Find` (`local.Spwnd Decs`) _car_id_2))
  (bind _returnvalue_4 (`KismetStringLibrary.Conv_NameToString` _car_id_2))
  (bind (_key _value_4) (`BlueprintMapLibrary.Map_GetKeyValueByIndex` _spwnd_decs (`BlueprintMapLibrary.Map_GetLastIndex` _spwnd_decs)))
  (bind (_key_2 _value_5) (`BlueprintMapLibrary.Map_GetKeyValueByIndex` _dec_starts (`BlueprintMapLibrary.Map_GetLastIndex` _dec_starts)))
  (bind (_key_3 _value_6) (`BlueprintMapLibrary.Map_GetKeyValueByIndex` _dec_ends (`BlueprintMapLibrary.Map_GetLastIndex` _dec_ends)))
  (`|ExecutionSequence`
    (:`then_0`
      (`BlueprintMapLibrary.Map_Clear` (`local.Dec Starts`))
      (`BlueprintMapLibrary.Map_Clear` (`local.Dec Ends`))
      (`BlueprintMapLibrary.Map_Clear` (`local.Spwnd Decs`))
      (set `local.Dec Starts` (`local.Decal Start Positions In`))
      (set `local.Dec Ends` (`local.Decal End Positions In`))
      (set `local.Spwnd Decs` (`local.Spawned Decals In`)))
    (:`then_1`
      (if (!= (`local.Car ID`) "None")
        (if (and (`BlueprintMapLibrary.Map_Contains` (`local.Dec Starts`) _car_id) (`BlueprintMapLibrary.Map_Contains` (`local.Dec Ends`) _car_id) (`BlueprintMapLibrary.Map_Contains` (`local.Spwnd Decs`) _car_id))
          (`|ExecutionSequence`
            (:`then_0`
              (if _returnvalue
                (set `local.Dec Start Comp to Destroy` _value)
                (bind _returnvalue_5 (`BlueprintMapLibrary.Map_Remove` (`local.Dec Starts`) _car_id_2))
                (if _returnvalue_5
                  (`ActorComponent.K2_DestroyComponent` (`local.Dec Start Comp to Destroy`))
                  (else
                    (`KismetSystemLibrary.PrintString` null (`KismetStringLibrary.Concat_StrStr` (`KismetSystemLibrary.GetDisplayName` (`local.Self Ref`)) " failed to remove Decal Start Pos from Car" _returnvalue_4) true true (struct :`R` 1.0 :`A` 1.0) 5.0 :!label _label)))
                (else
                  (goto _label))))
            (:`then_1`
              (if _returnvalue_2
                (set `local.Dec End Comp to Destroy` _value_2)
                (bind _returnvalue_6 (`BlueprintMapLibrary.Map_Remove` (`local.Dec Ends`) _car_id_2))
                (if _returnvalue_6
                  (`ActorComponent.K2_DestroyComponent` (`local.Dec End Comp to Destroy`))
                  (else
                    (`KismetSystemLibrary.PrintString` null (`KismetStringLibrary.Concat_StrStr` (`KismetSystemLibrary.GetDisplayName` (`local.Self Ref`)) " failed to remove Decal End Pos from Car" _returnvalue_4) true true (struct :`R` 1.0 :`A` 1.0) 5.0 :!label _label_2)))
                (else
                  (goto _label_2))))
            (:`then_2`
              (if _returnvalue_3
                (set `local.Dec Component to Destroy` _value_3)
                (bind _returnvalue_7 (`BlueprintMapLibrary.Map_Remove` (`local.Spwnd Decs`) _car_id_2))
                (if _returnvalue_7
                  (`ActorComponent.K2_DestroyComponent` (`local.Dec Component to Destroy`))
                  (else
                    (`KismetSystemLibrary.PrintString` null (`KismetStringLibrary.Concat_StrStr` (`KismetSystemLibrary.GetDisplayName` (`local.Self Ref`)) " failed to remove Decal from Car" _returnvalue_4) true true (struct :`R` 1.0 :`A` 1.0) 5.0 :!label _label_3)))
                (else
                  (goto _label_3))))))
        (else
          (`KismetSystemLibrary.PrintString` null (`KismetStringLibrary.Concat_StrStr` (`KismetSystemLibrary.GetDisplayName` (`local.Self Ref`)) " executed Emergency Decal Killer.") true true (struct :`R` 1.0 :`G` 1.0 :`A` 1.0) 5.0)
          (`|ExecutionSequence`
            (:`then_0`
              (`/Engine/EditorBlueprintResources/StandardMacros.IsValid` _value_5
                (:`Is Valid`
                  (set `local.Dec Start Comp to Destroy` _value_5)
                  (bind _returnvalue_8 (`BlueprintMapLibrary.Map_Remove` (`local.Dec Starts`) _key_2))
                  (if _returnvalue_8
                    (`ActorComponent.K2_DestroyComponent` (`local.Dec Start Comp to Destroy`))
                    (else
                      (goto _label))))
                (:`Is Not Valid`
                  (goto _label))))
            (:`then_1`
              (`/Engine/EditorBlueprintResources/StandardMacros.IsValid` _value_6
                (:`Is Valid`
                  (set `local.Dec End Comp to Destroy` _value_6)
                  (bind _returnvalue_9 (`BlueprintMapLibrary.Map_Remove` (`local.Dec Ends`) _key_3))
                  (if _returnvalue_9
                    (`ActorComponent.K2_DestroyComponent` (`local.Dec End Comp to Destroy`))
                    (else
                      (goto _label_2))))
                (:`Is Not Valid`
                  (goto _label_2))))
            (:`then_2`
              (`/Engine/EditorBlueprintResources/StandardMacros.IsValid` _value_4
                (:`Is Valid`
                  (set `local.Dec Component to Destroy` _value_4)
                  (bind _returnvalue_10 (`BlueprintMapLibrary.Map_Remove` (`local.Spwnd Decs`) _key))
                  (if _returnvalue_10
                    (`ActorComponent.K2_DestroyComponent` (`local.Dec Component to Destroy`))
                    (else
                      (goto _label_3))))
                (:`Is Not Valid`
                  (goto _label_3))))))))
    (:`then_2`
      (return (`local.Dec Starts`) (`local.Dec Ends`) (`local.Spwnd Decs`)))))

(fn `Destroy Decal Actor and Refresh List`
  (params (`Spawned Decals In` :type "Array of DecalComponent Object Reference") (`Other Actor` :type "Actor Object Reference"))
  (returns (`Spawned Decals Out` :type "Array of DecalComponent Object Reference"))
  (locals (`Array Indexes to Purge` :type "Array of Integer") (`Other Actor Static Mesh Components` :type "Array of StaticMeshComponent Object Reference") (`Spawned Decals` :type "Array of DecalComponent Object Reference"))
  (bind _spawned_decals (`local.Spawned Decals`))
  (`|ExecutionSequence`
    (:`then_0`
      (set `local.Spawned Decals` `Spawned Decals In`)
      (set `local.Other Actor Static Mesh Components` (`Actor.K2_GetComponentsByClass` `Other Actor` "/Script/Engine.StaticMeshComponent")))
    (:`then_1`
      (for (_array_element _array_index) (`local.Spawned Decals`)
        (`/Engine/EditorBlueprintResources/StandardMacros.IsValid` _array_element
          (:`Is Valid`
            (bind _asstatic_mesh_component (cast `StaticMeshComponent` (`SceneComponent.GetAttachParent` _array_element)))
            (if (!= (`KismetArrayLibrary.Array_Find` (`local.Other Actor Static Mesh Components`) _asstatic_mesh_component) -1)
              (`KismetArrayLibrary.Array_AddUnique` (`local.Array Indexes to Purge`) (`KismetArrayLibrary.Array_Find` (`local.Spawned Decals`) _array_element))))
          (:`Is Not Valid`
            (`KismetArrayLibrary.Array_AddUnique` (`local.Array Indexes to Purge`) _array_index)))))
    (:`then_2`
      (for _array_element_2 (`local.Array Indexes to Purge`)
        (bind _output (`|GetArrayItem` _spawned_decals _array_element_2))
        (`/Engine/EditorBlueprintResources/StandardMacros.IsValid` _output
          (:`Is Valid`
            (`ActorComponent.K2_DestroyComponent` _output))
          (:`Is Not Valid`
            _))
        (`KismetArrayLibrary.Array_Remove` _spawned_decals _array_element_2)))
    (:`then_3`
      (return (`local.Spawned Decals`)))))

(fn `Does This Matser Machine Exist in Game Instance Relays List`
  (params (`Master machine` :type "/Game/MyContent/Blueprints/ConfigurableMachines/MasterMachine_BP Object Reference"))
  (returns (Found :type Boolean))
  (locals (`Loaded Relays` :type "Array of /Game/MyContent/Blueprints/RelayProperties_SRUCT Structure"))
  (`|ExecutionSequence`
    (:`then_0`
      (bind _asmain_game_instance_gi (cast `/Game/FirstPerson/Blueprints/MainGameInstance_GI` (`GameplayStatics.GetGameInstance` null)))
      (set `local.Loaded Relays` (`/Game/FirstPerson/Blueprints/MainGameInstance_GI.Relays` _asmain_game_instance_gi)))
    (:`then_1`
      (for _array_element (`local.Loaded Relays`)
        (bind _returnvalue (== (`.RelayNumber_96_64CD80424F05A7615DE542B6729BE91A` (break `/Game/MyContent/Blueprints/RelayProperties_SRUCT` _array_element)) (`.RelayNumber_96_64CD80424F05A7615DE542B6729BE91A` (break `/Game/MyContent/Blueprints/RelayProperties_SRUCT` (`/Game/MyContent/Blueprints/ConfigurableMachines/MasterMachine_BP.Relay Properties` `Master machine`)))))
        (if _returnvalue
          (break)))
      (return _returnvalue))))

(fn `Get All Relay Data`
  (returns (`Relay Properties` :type "Array of /Game/MyContent/Blueprints/RelayProperties_SRUCT Structure"))
  (bind _asmain_game_instance_gi (cast `/Game/FirstPerson/Blueprints/MainGameInstance_GI` (`GameplayStatics.GetGameInstance` null)))
  (return (`/Game/FirstPerson/Blueprints/MainGameInstance_GI.Relays` _asmain_game_instance_gi)))

(fn `Get All Service Data`
  (returns (`Service Properties` :type "Array of /Game/FirstPerson/Blueprints/ServiceProperties_STRUCT Structure"))
  (bind _asmain_game_instance_gi (cast `/Game/FirstPerson/Blueprints/MainGameInstance_GI` (`GameplayStatics.GetGameInstance` null)))
  (return (`/Game/FirstPerson/Blueprints/MainGameInstance_GI.Services` _asmain_game_instance_gi)))

(fn `Get Last Wash Service in List`
  (returns (`Last Wash Service` :type "/Game/FirstPerson/Blueprints/ServiceProperties_STRUCT Structure"))
  (locals (`Last Wash Service Stored` :type "/Game/FirstPerson/Blueprints/ServiceProperties_STRUCT Structure"))
  (bind _asmain_game_instance_gi (cast `/Game/FirstPerson/Blueprints/MainGameInstance_GI` (`GameplayStatics.GetGameInstance` null)))
  (for _array_element (`/Game/FirstPerson/Blueprints/MainGameInstance_GI.Services` _asmain_game_instance_gi)
    (if (== (`.Type_9_578A34BE475ACCAAFBE34397A0D878EC` (break `/Game/FirstPerson/Blueprints/ServiceProperties_STRUCT` _array_element)) 3)
      (set `local.Last Wash Service Stored` _array_element)))
  (return (`local.Last Wash Service Stored`)))

(fn `Get Relay Data`
  (params (`Relay #` :type Integer))
  (returns (`Relay Properties` :type "/Game/MyContent/Blueprints/RelayProperties_SRUCT Structure") (`Array Index` :type Integer))
  (bind _asmain_game_instance_gi (cast `/Game/FirstPerson/Blueprints/MainGameInstance_GI` (`GameplayStatics.GetGameInstance` null)))
  (for (_array_element _array_index) (`/Game/FirstPerson/Blueprints/MainGameInstance_GI.Relays` _asmain_game_instance_gi)
    (bind _returnvalue (== (`.RelayNumber_96_64CD80424F05A7615DE542B6729BE91A` (break `/Game/MyContent/Blueprints/RelayProperties_SRUCT` _array_element)) (`local.Relay #`)))
    (if _returnvalue
      (break)))
  (if _returnvalue
    (return _array_element _array_index)
    (else
      (return (make `/Game/MyContent/Blueprints/RelayProperties_SRUCT` -1) -1))))

(fn `Get Service Data`
  (params (`Service #` :type Integer))
  (returns (`Service Properties` :type "/Game/FirstPerson/Blueprints/ServiceProperties_STRUCT Structure") (`Array Index` :type Integer))
  (bind _asmain_game_instance_gi (cast `/Game/FirstPerson/Blueprints/MainGameInstance_GI` (`GameplayStatics.GetGameInstance` null)))
  (for (_array_element _array_index) (`/Game/FirstPerson/Blueprints/MainGameInstance_GI.Services` _asmain_game_instance_gi)
    (bind _returnvalue (== (`.None_3_D44345FA44860F184161BEBDDCDC87CC` (break `/Game/FirstPerson/Blueprints/ServiceProperties_STRUCT` _array_element)) (`local.Service #`)))
    (if _returnvalue
      (break)))
  (if _returnvalue
    (return _array_element _array_index)
    (else
      (return (make `/Game/FirstPerson/Blueprints/ServiceProperties_STRUCT` -1) -1))))

(fn `Invert Float Based On Photo Eyes Y pos`
  (params (In :type "Float (double-precision)"))
  (returns (Out :type "Float (double-precision)"))
  (bind _outactors (`GameplayStatics.GetAllActorsOfClass` null "/Game/MyContent/Blueprints/PhotoEyes_BP.PhotoEyes_BP_C"))
  (bind (_returnvalue_x _returnvalue_y) (`KismetMathLibrary.BreakVector` (`Actor.K2_GetActorLocation` (`|GetArrayItem` _outactors))))
  (return (* (`KismetMathLibrary.SelectFloat` -1.0 1.0 (< _returnvalue_y 0.0)) In)))

(fn `Piston Aim Math`
  (params (`Piston Mount` :type "SceneComponent Object Reference") (`Piston Extender` :type "SceneComponent Object Reference"))
  (bind (_returnvalue_location _returnvalue_rotation) (`KismetMathLibrary.BreakTransform` (`KismetAnimationLibrary.K2_LookAt` (`SceneComponent.K2_GetComponentToWorld` (`local.Piston Mount`)) (`SceneComponent.K2_GetComponentLocation` (`local.Piston Extender`)) (0.0 0.0 -1.0) false (1.0 0.0 0.0))))
  (bind (_returnvalue_location_2 _returnvalue_rotation_2) (`KismetMathLibrary.BreakTransform` (`KismetAnimationLibrary.K2_LookAt` (`SceneComponent.K2_GetComponentToWorld` (`local.Piston Extender`)) (`SceneComponent.K2_GetComponentLocation` (`local.Piston Mount`)) (0.0 0.0 1.0) false (1.0 0.0 0.0))))
  (`SceneComponent.K2_SetWorldRotation` (`local.Piston Mount`) _returnvalue_rotation false false)
  (`SceneComponent.K2_SetWorldRotation` (`local.Piston Extender`) _returnvalue_rotation_2 false false))

(fn `Search for Dummy Machine by Relay #`
  (params (`Relay #` :type Integer))
  (returns (`Matching Master Machine` :type "/Game/MyContent/Blueprints/ConfigurableMachines/MasterMachine_BP Object Reference"))
  (bind _outactors (`GameplayStatics.GetAllActorsOfClass` null "/Game/MyContent/Blueprints/ConfigurableMachines/MasterMachine_BP.MasterMachine_BP_C"))
  (for _array_element _outactors
    (bind _returnvalue (and (== (`.RelayNumber_96_64CD80424F05A7615DE542B6729BE91A` (break `/Game/MyContent/Blueprints/RelayProperties_SRUCT` (`/Game/MyContent/Blueprints/ConfigurableMachines/MasterMachine_BP.Relay Properties` _array_element))) `Relay #`) (`Actor.ActorHasTag` _array_element "Dummy")))
    (if _returnvalue
      (break)))
  (if _returnvalue
    (return _array_element)
    (else
      (return null))))

(fn `Search for Master Machine by Default Relay #`
  (params (`Default Relay #` :type Integer))
  (returns (`Matching Master Machine` :type "/Game/MyContent/Blueprints/ConfigurableMachines/MasterMachine_BP Object Reference"))
  (bind _outactors (`GameplayStatics.GetAllActorsOfClass` null "/Game/MyContent/Blueprints/ConfigurableMachines/MasterMachine_BP.MasterMachine_BP_C"))
  (for _array_element _outactors
    (bind _returnvalue (== (`/Game/MyContent/Blueprints/ConfigurableMachines/MasterMachine_BP.Relay_Default` _array_element) `Default Relay #`))
    (if _returnvalue
      (break)))
  (if _returnvalue
    (return _array_element)
    (else
      (return null))))

(fn `Search for Master Machine by Object Name`
  (params (`Object Name` :type String))
  (returns (`Matching Master Machine` :type "/Game/MyContent/Blueprints/ConfigurableMachines/MasterMachine_BP Object Reference"))
  (bind _outactors (`GameplayStatics.GetAllActorsOfClass` null "/Game/MyContent/Blueprints/ConfigurableMachines/MasterMachine_BP.MasterMachine_BP_C"))
  (for _array_element _outactors
    (bind _returnvalue (`KismetStringLibrary.EqualEqual_StrStr` `Object Name` (`KismetSystemLibrary.GetObjectName` _array_element)))
    (if _returnvalue
      (break)))
  (if _returnvalue
    (return _array_element)
    (else
      (return null))))

(fn `Search for Master Machine by Relay #`
  (params (`Relay #` :type Integer))
  (returns (`Matching Master Machine` :type "/Game/MyContent/Blueprints/ConfigurableMachines/MasterMachine_BP Object Reference") (`Object Name` :type String))
  (bind _outactors (`GameplayStatics.GetAllActorsOfClass` null "/Game/MyContent/Blueprints/ConfigurableMachines/MasterMachine_BP.MasterMachine_BP_C"))
  (for _array_element _outactors
    (bind _returnvalue (== (`.RelayNumber_96_64CD80424F05A7615DE542B6729BE91A` (break `/Game/MyContent/Blueprints/RelayProperties_SRUCT` (`/Game/MyContent/Blueprints/ConfigurableMachines/MasterMachine_BP.Relay Properties` _array_element))) `Relay #`))
    (if _returnvalue
      (break)))
  (if _returnvalue
    (return _array_element (`KismetSystemLibrary.GetObjectName` _array_element))
    (else
      (return null "INVALID"))))

(fn `Spawn Attached Mask Decal`
  (params (`Other Actor` :type "Actor Object Reference") (`Sprayer Location` :type "SceneComponent Object Reference") (DecalMaterial :type "MaterialInterface Object Reference") (`Self Ref` :type "Actor Object Reference") (`Use Custom Transform` :type Boolean :default false) (`Custom Transform` :type "Transform Structure (by ref)"))
  (returns (`Decal Start Pos Out` :type "BoxComponent Object Reference") (`Decal End Pos Out` :type "BoxComponent Object Reference") (`Spawned Decal Out` :type "DecalComponent Object Reference") (`Car ID Tag Out` :type Name))
  (locals (`Component Decal Attached to` :type "BoxComponent Object Reference") (`Car ID Tag` :type Name) (`Decal Start Pos` :type "BoxComponent Object Reference") (`Decal End Pos` :type "BoxComponent Object Reference") (`Spawned Decal` :type "DecalComponent Object Reference"))
  (bind (_returnvalue_x _returnvalue_y) (`KismetMathLibrary.BreakVector` (`SceneComponent.K2_GetComponentLocation` (`local.Component Decal Attached to`))))
  (bind (_returnvalue_x_2 _returnvalue_y_2) (`KismetMathLibrary.BreakVector` (`SceneComponent.K2_GetComponentLocation` (`local.Sprayer Location`))))
  (`|ExecutionSequence`
    (:`then_0`
      (set `local.Component Decal Attached to` (`Actor.GetComponentByClass` `Other Actor` "/Script/Engine.BoxComponent"))
      (set `local.Car ID Tag` (`|GetArrayItem` (`Actor.Tags` `Other Actor`) 2)))
    (:`then_1`
      (bind _returnvalue (`|AddComponentByClass` (`local.Self Ref`) "/Script/Engine.BoxComponent" false (`SceneComponent.GetRelativeTransform` (`local.Sprayer Location`))))
      (`BoxComponent.SetBoxExtent` _returnvalue (1.0 1.0 1.0) true)
      (`SceneComponent.K2_AttachToComponent` _returnvalue (`local.Component Decal Attached to`) "None" "KeepWorld" "KeepWorld" "KeepWorld" true)
      (set `local.Decal Start Pos` _returnvalue)
      (bind _returnvalue_2 (`|AddComponentByClass` (`local.Self Ref`) "/Script/Engine.BoxComponent" false (`SceneComponent.GetRelativeTransform` (`local.Sprayer Location`))))
      (`BoxComponent.SetBoxExtent` _returnvalue_2 (1.0 1.0 1.0) true)
      (set `local.Decal End Pos` _returnvalue_2)
      (bind _returnvalue_3 (`GameplayStatics.SpawnDecalAttached` (`local.DecalMaterial`) (.scale (`KismetMathLibrary.SelectTransform` (`local.Custom Transform`) (`KismetMathLibrary.MakeTransform` (0.0 0.0 100.0) (struct :`Pitch` -90.0 :`Yaw` 180.0) (300.0 1.0 300.0)) (`local.Use Custom Transform`))) (`local.Component Decal Attached to`) "None" (`KismetMathLibrary.MakeVector` (.x (.location (`KismetMathLibrary.SelectTransform` (`local.Custom Transform`) (`KismetMathLibrary.MakeTransform` (0.0 0.0 100.0) (struct :`Pitch` -90.0 :`Yaw` 180.0) (300.0 1.0 300.0)) (`local.Use Custom Transform`)))) (- _returnvalue_y_2 _returnvalue_y 0.0) (.z (.location (`KismetMathLibrary.SelectTransform` (`local.Custom Transform`) (`KismetMathLibrary.MakeTransform` (0.0 0.0 100.0) (struct :`Pitch` -90.0 :`Yaw` 180.0) (300.0 1.0 300.0)) (`local.Use Custom Transform`))))) (`KismetMathLibrary.MakeRotator` (.roll (.rotation (`KismetMathLibrary.SelectTransform` (`local.Custom Transform`) (`KismetMathLibrary.MakeTransform` (0.0 0.0 100.0) (struct :`Pitch` -90.0 :`Yaw` 180.0) (300.0 1.0 300.0)) (`local.Use Custom Transform`)))) (.pitch (.rotation (`KismetMathLibrary.SelectTransform` (`local.Custom Transform`) (`KismetMathLibrary.MakeTransform` (0.0 0.0 100.0) (struct :`Pitch` -90.0 :`Yaw` 180.0) (300.0 1.0 300.0)) (`local.Use Custom Transform`)))) (.yaw (.rotation (`KismetMathLibrary.SelectTransform` (`local.Custom Transform`) (`KismetMathLibrary.MakeTransform` (0.0 0.0 100.0) (struct :`Pitch` -90.0 :`Yaw` 180.0) (300.0 1.0 300.0)) (`local.Use Custom Transform`)))))))
      (set `local.Spawned Decal` _returnvalue_3))
    (:`then_2`
      (return (`local.Decal Start Pos`) (`local.Decal End Pos`) (`local.Spawned Decal`) (`local.Car ID Tag`)))))

(fn `Transform Attached Mask Decal`
  (params (`Decal Start Positions` :type "Map of Name to BoxComponent Object Reference (by ref)") (`Decal End Positions` :type "Map of Name to BoxComponent Object Reference (by ref)") (`Spawned Decals` :type "Map of Name to DecalComponent Object Reference (by ref)") (`Self Ref` :type "Actor Object Reference"))
  (returns (`Was Valid` :type Boolean))
  (`|ExecutionSequence`
    (:`then_0`
      (if (not (or (`BlueprintMapLibrary.Map_IsEmpty` `Decal Start Positions`) (`BlueprintMapLibrary.Map_IsEmpty` `Decal End Positions`) (`BlueprintMapLibrary.Map_IsEmpty` `Spawned Decals`)))
        (bind (_keypin _valuepin) (`|MapForEach` (`local.Spawned Decals`))
          (:`then`
            (`/Engine/EditorBlueprintResources/StandardMacros.IsValid` _valuepin
              (:`Is Valid`
                (bind (_relativescale3d_x _relativescale3d_y _relativescale3d_z) (`KismetMathLibrary.BreakVector` (`SceneComponent.RelativeScale3D` _valuepin)))
                (bind (_returnvalue_x _returnvalue_y) (`KismetMathLibrary.BreakVector` (`SceneComponent.K2_GetComponentLocation` (`BlueprintMapLibrary.Map_Find` (`local.Decal End Positions`) _keypin))))
                (bind (_returnvalue_x_2 _returnvalue_y_2) (`KismetMathLibrary.BreakVector` (`SceneComponent.K2_GetComponentLocation` (`BlueprintMapLibrary.Map_Find` (`local.Decal Start Positions`) _keypin))))
                (bind _returnvalue (/ (- (`KismetMathLibrary.Abs` _returnvalue_y) (`KismetMathLibrary.Abs` _returnvalue_y_2)) 2.0))
                (`SceneComponent.SetRelativeScale3D` _valuepin (`KismetMathLibrary.MakeVector` _relativescale3d_x (+ _returnvalue (* _returnvalue 0.2)) _relativescale3d_z))
                (bind (_returnvalue_x_3 _returnvalue_y_3 _returnvalue_z) (`KismetMathLibrary.BreakVector` (`SceneComponent.K2_GetComponentLocation` _valuepin)))
                (`SceneComponent.K2_SetWorldLocation` _valuepin (`KismetMathLibrary.MakeVector` _returnvalue_x_3 (/ (+ _returnvalue_y _returnvalue_y_2) 2.0) _returnvalue_z) false false))
              (:`Is Not Valid`
                (`KismetSystemLibrary.PrintString` null (`KismetStringLibrary.Concat_StrStr` "Warning: " (`KismetSystemLibrary.GetDisplayName` (`local.Self Ref`)) " tried to transform an invalid decal!") true false (struct :`R` 1.0 :`A` 1.0) 5.0)
                (return false)))))))
    (:`then_1`
      (return true))))