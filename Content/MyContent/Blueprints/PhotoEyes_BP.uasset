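; Photo-eye sensor that spawns an "Inv" Car1_BP, presumably invisible, when the first-person character stays in its laser box.
; Overlap starts a three-second one-shot timer, cleared when the player leaves.
; The timer spawns the car at the InvCarSpawnPoint-tagged TriggerVolume and summons it with the last wash service in the list.
; EStop cancels the timer and blocks new ones until EStopDisengage; the construction script tags the actor PhotoEyes.
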(event `self.Box_PhotoLazer.OnComponentBeginOverlap`
  (params (OverlappedComponent :type "PrimitiveComponent Object Reference") (OtherActor :type "Actor Object Reference") (OtherComp :type "PrimitiveComponent Object Reference") (OtherBodyIndex :type Integer) (bFromSweep :type Boolean) (SweepResult :type "HitResult Structure (by ref)"))
  (if (and (== (`GameplayStatics.GetObjectClass` OtherActor) "/Game/FirstPerson/Blueprints/BP_FirstPersonCharacter.BP_FirstPersonCharacter_C") (not (`self.E Stop Override`)))
    (`self.Set Spawn Inv Car Timer`)))

(event `self.Box_PhotoLazer.OnComponentEndOverlap`
  (params (OverlappedComponent :type "PrimitiveComponent Object Reference") (OtherActor :type "Actor Object Reference") (OtherComp :type "PrimitiveComponent Object Reference") (OtherBodyIndex :type Integer))
  (if (== (`GameplayStatics.GetObjectClass` OtherActor) "/Game/FirstPerson/Blueprints/BP_FirstPersonCharacter.BP_FirstPersonCharacter_C")
    (`KismetSystemLibrary.K2_ClearAndInvalidateTimerHandle` (`self.Spawn Inv Car Timer Ref`) :!label _label)))

(event `/Game/FirstPerson/Blueprints/ConfigMachine_BPI.E Stop`
  (set `self.E Stop Override` true)
  (goto _label))

(event `Set Spawn Inv Car Timer`
  (bind _returnvalue (`KismetSystemLibrary.K2_SetTimerDelegate` (delegate `Spawn Inv Car`) 3.0 false true))
  (set `self.Spawn Inv Car Timer Ref` _returnvalue))

(event `/Game/FirstPerson/Blueprints/ConfigMachine_BPI.E Stop_Disengage`
  (set `self.E Stop Override` false))

(event `Spawn Inv Car`
  (bind _outactors (`GameplayStatics.GetAllActorsOfClassWithTag` "/Script/Engine.TriggerVolume" "InvCarSpawnPoint"))
  (bind _returnvalue (`|SpawnActorFromClass` "/Game/MyContent/Blueprints/Car1_BP.Car1_BP_C" (`self.GetTransform` (`|GetArrayItem` _outactors)) "Undefined" "MultiplyWithRoot" null null))
  (bind _last_wash_service (`/Game/MyContent/Blueprints/ConfigMachine_BPFL.Get Last Wash Service in List`))
  (`/Game/MyContent/Blueprints/Car1_BP.Car Summon` _returnvalue false 0 (`.None_3_D44345FA44860F184161BEBDDCDC87CC` (break `/Game/FirstPerson/Blueprints/ServiceProperties_STRUCT` _last_wash_service)) true))

(fn `UserConstructionScript`
  (set `self.Tags` (`|MakeArray` "PhotoEyes" :!type "Name")))