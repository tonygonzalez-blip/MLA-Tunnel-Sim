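; Interactive emergency-stop button that a tagged player toggles with IA_Interact while inside its trigger box.
; A Timeline animates the button's push and twist, playing forward or in reverse, with a flag and DoOnce gates blocking input mid-animation.
; When it finishes, the button sends engage or disengage messages to all ConfigMachine_BPI actors and the VisualQueue_WBP widget.
; EStop events lock an unpressed button through Override until disengaged.
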(event `/Game/FirstPerson/Blueprints/ConfigMachine_BPI.E Stop`
  (if (not (`self.IWasPressed`))
    (set `self.Override` true)))

(event `/Game/FirstPerson/Blueprints/ConfigMachine_BPI.E Stop_Disengage`
  (set `self.Override` false))

(event `EnhancedInput|/Game/Input/Actions/IA_Interact`
  (params (ActionValue :type Boolean) (ElapsedSeconds :type "Float (double-precision)") (TriggeredSeconds :type "Float (double-precision)") (InputAction :type "InputAction Object Reference" :default "/Game/Input/Actions/IA_Interact.IA_Interact"))
  (bind _estopbutton_button_mesh (`self.EstopButton_Button_MESH`))
  (bind (_relativelocation_x _relativelocation_y _relativelocation_z) (`KismetMathLibrary.BreakVector` (`SceneComponent.RelativeLocation` _estopbutton_button_mesh)))
  (:`Started`
    (if (or (`self.Wait for Anim`) (`self.Override`))
      _
      (elif (`self.IWasPressed`)
        (`|ExecutionSequence`
          (:`then_0`
            (set `self.IWasPressed` false))
          (:`then_1`
            (`/Engine/EditorBlueprintResources/StandardMacros.DoOnce` false :!label _label
              (:`Completed`
                (set `self.Wait for Anim` true)
                (bind (_direction _twist _push) (`Timeline|Timeline` :!via `ReverseFromEnd` :!label _label_2)
                  (:`Update`
                    (`SceneComponent.K2_SetRelativeTransform` (`self.EstopButton_Button_MESH`) (`KismetMathLibrary.MakeTransform` (`KismetMathLibrary.MakeVector` _relativelocation_x (`KismetMathLibrary.Lerp` 2.2 0.0 _push) _relativelocation_z) (`KismetMathLibrary.MakeRotator` 0.0 (`KismetMathLibrary.Lerp` 0.0 40.0 _twist)) (`SceneComponent.RelativeScale3D` _estopbutton_button_mesh)) false false))
                  (:`Finished`
                    (`|ExecutionSequence`
                      (:`then_0`
                        (if (`self.IWasPressed`)
                          (bind _outactors (`GameplayStatics.GetAllActorsWithInterface` "/Game/FirstPerson/Blueprints/ConfigMachine_BPI.ConfigMachine_BPI_C"))
                          (for _array_element _outactors
                            (message `/Game/FirstPerson/Blueprints/ConfigMachine_BPI.E Stop` _array_element))
                          (bind _foundwidgets (`WidgetBlueprintLibrary.GetAllWidgetsOfClass` "/Game/FirstPerson/Blueprints/VisualQueue_WBP.VisualQueue_WBP_C"))
                          (`/Game/FirstPerson/Blueprints/VisualQueue_WBP.E Stop` (`|GetArrayItem` _foundwidgets))
                          (else
                            (bind _outactors_2 (`GameplayStatics.GetAllActorsWithInterface` "/Game/FirstPerson/Blueprints/ConfigMachine_BPI.ConfigMachine_BPI_C"))
                            (for _array_element_2 _outactors_2
                              (message `/Game/FirstPerson/Blueprints/ConfigMachine_BPI.E Stop_Disengage` _array_element_2))
                            (bind _foundwidgets_2 (`WidgetBlueprintLibrary.GetAllWidgetsOfClass` "/Game/FirstPerson/Blueprints/VisualQueue_WBP.VisualQueue_WBP_C"))
                            (`/Game/FirstPerson/Blueprints/VisualQueue_WBP.E Stop_Disengage` (`|GetArrayItem` _foundwidgets_2)))))
                      (:`then_1`
                        (set `self.Wait for Anim` false))
                      (:`then_2`
                        (`|ExecutionSequence`
                          (:`then_0`
                            (goto _label_3 :!via `Reset`))
                          (:`then_1`
                            (goto _label :!via `Reset`)))))))))))
        (else
          (`|ExecutionSequence`
            (:`then_0`
              (set `self.IWasPressed` true))
            (:`then_1`
              (`/Engine/EditorBlueprintResources/StandardMacros.DoOnce` false :!label _label_3
                (:`Completed`
                  (set `self.Wait for Anim` true)
                  (goto _label_2 :!via `PlayFromStart`))))))))))

(event `self.TrigBox.OnComponentBeginOverlap`
  (params (OverlappedComponent :type "PrimitiveComponent Object Reference") (OtherActor :type "Actor Object Reference") (OtherComp :type "PrimitiveComponent Object Reference") (OtherBodyIndex :type Integer) (bFromSweep :type Boolean) (SweepResult :type "HitResult Structure (by ref)"))
  (if (`self.ActorHasTag` OtherActor "player")
    (`self.EnableInput` (`GameplayStatics.GetPlayerController` 0))))

(event `self.TrigBox.OnComponentEndOverlap`
  (params (OverlappedComponent :type "PrimitiveComponent Object Reference") (OtherActor :type "Actor Object Reference") (OtherComp :type "PrimitiveComponent Object Reference") (OtherBodyIndex :type Integer))
  (if (`self.ActorHasTag` OtherActor "player")
    (`self.DisableInput` (`GameplayStatics.GetPlayerController` 0))))

(fn `UserConstructionScript`)