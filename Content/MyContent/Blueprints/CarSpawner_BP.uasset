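; CarSpawner_BP is a placed spawner that creates Car1_BP cars at its own transform.
; Unless the game instance's Scenario1 flag is set, it waits a configurable delay, then starts a looping timer for spawn attempts.
; Each attempt passes a percentage roll and requires an empty Box overlap before spawning a car and calling CarSummon.
; ForceSpawnaCar skips both checks and passes silliness, car and wash selections to CarSummon.
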(event `Force Spawn a Car`
  (params (`Is Silly` :type Boolean) (`Car Selection` :type Integer :default -1) (`Wash Selection` :type Integer :default -1))
  (bind _returnvalue (`|SpawnActorFromClass` "/Game/MyContent/Blueprints/Car1_BP.Car1_BP_C" (`self.GetTransform`) "Undefined" "MultiplyWithRoot" null null))
  (`/Game/MyContent/Blueprints/Car1_BP.Car Summon` _returnvalue `Is Silly` `Car Selection` `Wash Selection` false))

(event `self.ReceiveBeginPlay`
  (bind _asmain_game_instance_gi (cast `/Game/FirstPerson/Blueprints/MainGameInstance_GI` (`GameplayStatics.GetGameInstance`)))
  (if (not (`/Game/FirstPerson/Blueprints/MainGameInstance_GI.Scenario1` _asmain_game_instance_gi))
    (`KismetSystemLibrary.Delay` (`self.Delay before cars can begin spawning`))
    (`KismetSystemLibrary.K2_SetTimerDelegate` (delegate `Attempt to spawn car`) 10.0 true true)))

(event `Attempt to spawn car`
  (if (and (<= (+ (`KismetMathLibrary.RandomInteger` 100) 1) (`self.Percent chance of cars spawning`)) (`KismetArrayLibrary.Array_IsEmpty` (`PrimitiveComponent.GetOverlappingActors` (`self.Box`) "/Script/Engine.Actor")))
    (bind _returnvalue (`|SpawnActorFromClass` "/Game/MyContent/Blueprints/Car1_BP.Car1_BP_C" (`self.GetTransform`) "Undefined" "MultiplyWithRoot" null null))
    (`/Game/MyContent/Blueprints/Car1_BP.Car Summon` _returnvalue false -1 -1 false)
    (`KismetSystemLibrary.PrintString` "Car Spawned!" true true (struct :`G` 1.0 :`A` 1.0))))

(fn `UserConstructionScript`)