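; Car wash-style brush arm that ramps a swing target in on Start and out on End.
; Per-frame delay loops step the target at adjustable speeds.
; Brush imposter overlaps back the arm off tagged car collision while enabled; otherwise a rear-of-car tag moves it in and briefly ignores collision on a timer.
; The yaw interpolation that would apply the target is disconnected, with Tick and BeginPlay empty.
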(event `Move Brush0 In`
  (set `self.Brush0 Going In` true)
  (`self.Set Target` true (`self.By`) :!label _label)
  (`KismetSystemLibrary.DelayUntilNextTick`)
  (if (not (or (>= (`self.Target`) 1.0) (not (`self.Brush0 Going In`))))
    (goto _label)))

(event `self.ReceiveBeginPlay`)

(event `Move Brush0 Out`
  (set `self.Brush0 Going In` false)
  (`self.Set Target` false (`self.By`) :!label _label_2)
  (`KismetSystemLibrary.DelayUntilNextTick`)
  (if (not (or (<= (`self.Target`) 0.0) (`self.Brush0 Going In`)))
    (goto _label_2)))

(event `self.ReceiveTick`
  (params (DeltaSeconds :type "Float (single-precision)")))

(event `self.Start`
  (params (`Other Actor` :type "Actor Object Reference"))
  (`|ExecutionSequence`
    (:`then_0`
      (`KismetSystemLibrary.K2_ClearAndInvalidateTimerHandle` (`self.RHBICR Event Timer Ref`))
      (`self.Reset Hit Brush Imposter Collision Response`))
    (:`then_1`
      (set `self.By` 0.2)
      (set `self.Interp Speed` 3.0)
      (set `self.Enable Collision Movement` true)
      (`self.Move Brush0 In`)
      (`self.SetActorTickEnabled` true))))

(event `self.End`
  (`KismetSystemLibrary.K2_ClearAndInvalidateTimerHandle` (`self.RHBICR Event Timer Ref`))
  (set `self.By` 0.2)
  (set `self.Interp Speed` 3.0)
  (set `self.Enable Collision Movement` false)
  (`self.Move Brush0 Out`))

(event `self.Hit_Brush_Imposter.OnComponentBeginOverlap`
  (params (OverlappedComponent :type "PrimitiveComponent Object Reference") (OtherActor :type "Actor Object Reference") (OtherComp :type "PrimitiveComponent Object Reference") (OtherBodyIndex :type Integer) (bFromSweep :type Boolean) (SweepResult :type "HitResult Structure (by ref)"))
  (if (and (`ActorComponent.ComponentHasTag` OtherComp "carCollision") (`self.Enable Collision Movement`))
    (`self.Move Brush0 Out`)
    (set `self.By` 0.1)
    (set `self.Interp Speed` 1.5)
    (elif (`ActorComponent.ComponentHasTag` OtherComp "Rear Of Car")
      (set `self.By` 0.1)
      (set `self.Interp Speed` 1.5)
      (`self.Move Brush0 In`)
      (`PrimitiveComponent.SetCollisionResponseToAllChannels` (`self.Hit_Brush_Imposter`) "ECR_Ignore")
      (bind _returnvalue (`KismetSystemLibrary.K2_SetTimerDelegate` (delegate `Reset Hit Brush Imposter Collision Response`) 2.0))
      (set `self.RHBICR Event Timer Ref` _returnvalue))))

(event `Reset Hit Brush Imposter Collision Response`
  (`PrimitiveComponent.SetCollisionResponseToAllChannels` (`self.Hit_Brush_Imposter`) "ECR_Overlap"))

(event `self.Hit_Brush_Imposter.OnComponentEndOverlap`
  (params (OverlappedComponent :type "PrimitiveComponent Object Reference") (OtherActor :type "Actor Object Reference") (OtherComp :type "PrimitiveComponent Object Reference") (OtherBodyIndex :type Integer))
  (if (and (`ActorComponent.ComponentHasTag` OtherComp "carCollision") (`self.Enable Collision Movement`))
    (set `self.Brush0 Going In` true)))

(fn `Set Target`
  (params (Add :type Boolean) (By :type "Float (double-precision)" :default 0.1))
  (if Add
    (set `self.Target` (+ (`self.Target`) (* By (`GameplayStatics.GetWorldDeltaSeconds`))))
    (else
      (set `self.Target` (- (`self.Target`) (* By (`GameplayStatics.GetWorldDeltaSeconds`)))))))

(fn `UserConstructionScript`
  (set `ActorComponent.ComponentTags` (`|MakeArray` "grab" "setInFront" :!type "Name") (`self.MacNeilBrushArm_MESH`)))