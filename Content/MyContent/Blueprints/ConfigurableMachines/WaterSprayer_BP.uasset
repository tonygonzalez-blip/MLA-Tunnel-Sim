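; Configurable car wash water sprayer arch that toggles particle emitters and paints a water mask decal onto passing cars.
; Start spawns a decal per car, stored in maps keyed by car tag with incrementing sort order, and Tick stretches it between start and end points.
; When the car's rear exits, the end point attaches alongside the start and spraying stops.
; A movable DestroyDecal trigger removes decals, with emergency cleanup if updating fails.
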(event `self.ReceiveTick`
  (params (DeltaSeconds :type "Float (single-precision)"))
  (bind _was_valid (`/Game/MyContent/Blueprints/ConfigMachine_BPFL.Transform Attached Mask Decal` (`self.Decal Start Positions`) (`self.Decal End Positions`) (`self.Spawned Decals`) self))
  (if (not _was_valid)
    (`self.Emergency Decal Killer`)))

(event `Force Start`
  (for _array_element (`self.Particle Emitters`) :!label _label
    (`ActorComponent.Activate` _array_element false))
  (`self.SetActorTickEnabled` true))

(event `/Game/FirstPerson/Blueprints/ConfigMachine_BPI.Moment On Start`
  (goto _label))

(event `/Game/FirstPerson/Blueprints/ConfigMachine_BPI.Start`
  (params (`Other Actor` :type "Actor Object Reference"))
  (`|ExecutionSequence`
    (:`then_0`
      (`SceneComponent.K2_SetWorldLocation` (`self.DestroyDecal`) (`self.Destroy Decal Default World Location`) false false)
      (set `self.Destroy Decal Moved` false)
      (bind _ascar_1_bp (cast `/Game/MyContent/Blueprints/Car1_BP` `Other Actor`))
      (`/Game/MyContent/Blueprints/Car1_BP.Increment Decal Sort Order` _ascar_1_bp)
      (set `self.Sort Order` (`/Game/MyContent/Blueprints/Car1_BP.Current Decal Sort Order` _ascar_1_bp))
      (set `self.Car ID` (`|GetArrayItem` (`Actor.Tags` `Other Actor`) 2)))
    (:`then_1`
      (bind (_decal_start_pos_out _decal_end_pos_out _spawned_decal_out _car_id_tag_out) (`/Game/MyContent/Blueprints/ConfigMachine_BPFL.Spawn Attached Mask Decal` `Other Actor` (`self.SprayerLocation`) "/Game/MyContent/waterMaskDecal.waterMaskDecal" self))
      (`BlueprintMapLibrary.Map_Add` (`self.Decal Start Positions`) _car_id_tag_out _decal_start_pos_out)
      (`BlueprintMapLibrary.Map_Add` (`self.Decal End Positions`) _car_id_tag_out _decal_end_pos_out)
      (`DecalComponent.SetSortOrder` _spawned_decal_out (`self.Sort Order`))
      (`BlueprintMapLibrary.Map_Add` (`self.Spawned Decals`) _car_id_tag_out _spawned_decal_out)
      (goto _label))))

(event `/Game/FirstPerson/Blueprints/ConfigMachine_BPI.Moment On End`
  (for _array_element (`self.Particle Emitters`) :!label _label_2
    (`ActorComponent.Deactivate` _array_element))
  (`self.SetActorTickEnabled` false))

(event `self.SprayerLocation.OnComponentBeginOverlap`
  (params (OverlappedComponent :type "PrimitiveComponent Object Reference") (OtherActor :type "Actor Object Reference") (OtherComp :type "PrimitiveComponent Object Reference") (OtherBodyIndex :type Integer) (bFromSweep :type Boolean) (SweepResult :type "HitResult Structure (by ref)"))
  ; See SoapSprayer_BP
)

(event `self.SprayerLocation.OnComponentEndOverlap`
  (params (OverlappedComponent :type "PrimitiveComponent Object Reference") (OtherActor :type "Actor Object Reference") (OtherComp :type "PrimitiveComponent Object Reference") (OtherBodyIndex :type Integer))
  (bind _car_id (`self.Car ID`))
  (bind (_value _returnvalue) (`BlueprintMapLibrary.Map_Find` (`self.Decal End Positions`) _car_id))
  (bind (_value_2 _returnvalue_2) (`BlueprintMapLibrary.Map_Find` (`self.Decal Start Positions`) _car_id))
  (bind _output (`|GetArrayItem` (`Actor.Tags` OtherActor) 2))
  (if (`ActorComponent.ComponentHasTag` OtherComp "Rear Of Car")
    (`|ExecutionSequence`
      (:`then_0`
        (if (!= _output "None")
          (set `self.Car ID` _output)))
      (:`then_1`
        (`|ExecutionSequence` :!label _label_3
          (:`then_0`
            (if (and _returnvalue _returnvalue_2)
              (`SceneComponent.K2_AttachToComponent` _value (`SceneComponent.GetAttachParent` _value_2) "None" "KeepWorld" "KeepWorld" "KeepWorld" true)))
          (:`then_1`
            (goto _label_2)))))))

(event `/Game/FirstPerson/Blueprints/ConfigMachine_BPI.End`
  (goto _label_3))

(event `self.DestroyDecal.OnComponentBeginOverlap`
  (params (OverlappedComponent :type "PrimitiveComponent Object Reference") (OtherActor :type "Actor Object Reference") (OtherComp :type "PrimitiveComponent Object Reference") (OtherBodyIndex :type Integer) (bFromSweep :type Boolean) (SweepResult :type "HitResult Structure (by ref)"))
  (if (`ActorComponent.ComponentHasTag` OtherComp "Rear Of Car")
    (bind (_decal_start_positions_out _decal_end_positions_out _spawned_decals_out) (`/Game/MyContent/Blueprints/ConfigMachine_BPFL.Destroy Attached Mask Decal` (`|GetArrayItem` (`Actor.Tags` OtherActor) 2) (`self.Decal Start Positions`) (`self.Decal End Positions`) (`self.Spawned Decals`) self))
    (set `self.Decal Start Positions` _decal_start_positions_out)
    (set `self.Decal End Positions` _decal_end_positions_out)
    (set `self.Spawned Decals` _spawned_decals_out)))

(event `Emergency Decal Killer`
  (bind (_decal_start_positions_out _decal_end_positions_out _spawned_decals_out) (`/Game/MyContent/Blueprints/ConfigMachine_BPFL.Destroy Attached Mask Decal` "None" (`self.Decal Start Positions`) (`self.Decal End Positions`) (`self.Spawned Decals`) self))
  (set `self.Decal Start Positions` _decal_start_positions_out)
  (set `self.Decal End Positions` _decal_end_positions_out)
  (set `self.Spawned Decals` _spawned_decals_out))

(event `/Game/FirstPerson/Blueprints/ConfigMachine_BPI.Set DestroyDecal Location`
  (params (`Destroy Decal` :type "BoxComponent Object Reference") (`Destroy Decal Locaiton` :type "Vector Structure"))
  (if (not (`self.Destroy Decal Moved`))
    (`SceneComponent.K2_SetWorldLocation` (`self.DestroyDecal`) (+ (`KismetMathLibrary.SelectVector` (`SceneComponent.K2_GetComponentLocation` `Destroy Decal`) `Destroy Decal Locaiton` (== `Destroy Decal Locaiton` (0.0 0.0 0.0) :`ErrorTolerance` 1.0)) (0.0 10.0 0.0)) false false)
    (set `self.Destroy Decal Moved` true)))

(fn `UserConstructionScript`
  (bind _waterarch_mesh (`self.WaterArch_MESH`))
  (`|ExecutionSequence`
    (:`then_0`
      (set `ActorComponent.ComponentTags` (`|MakeArray` "grab" "setInFront" :!type "Name") _waterarch_mesh)
      (set `self.Particle Emitters` (`SceneComponent.GetChildrenComponents` _waterarch_mesh false)))
    (:`then_1`
      (set `ActorComponent.ComponentTags` (`|MakeArray` "passGrab" :!type "Name") (`self.MESH_GenericArch`)))
    (:`then_2`
      (bind _outactors (`GameplayStatics.GetAllActorsOfClassWithTag` "/Script/Engine.Actor" "DestroyDecalDefaultLocation"))
      (bind _output_get (set `self.Destroy Decal Default World Location` (`self.K2_GetActorLocation` (`|GetArrayItem` _outactors))))
      (`SceneComponent.K2_SetWorldLocation` (`self.DestroyDecal`) _output_get false false))
    (:`then_3`
      (`/Game/MyContent/Blueprints/ConfigMachine_BPFL.Cable Construction Script` self (`self.Cable`)))))