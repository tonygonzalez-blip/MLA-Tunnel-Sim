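; Blower machine that runs Niagara effects and applies a mask exclusion decal to passing cars.
; On BeginPlay it attaches to its parent MasterMachine's socket, whose number selects mesh, emitters, offsets, decal transform and rattle strength.
; Start spawns decals tracked per car ID and enables Tick, which updates them and rattles the mesh via FlipFlop.
; Rear-of-car overlap exits pin decal ends or destroy decals, with an emergency cleanup when updates fail.
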(event `self.ReceiveTick`
  (params (DeltaSeconds :type "Float (single-precision)"))
  (bind _blower_mesh (`self.Blower_MESH`))
  (bind _rattle_anim_value (`self.Rattle Anim Value`))
  (bind (_relativerotation_roll _relativerotation_pitch _relativerotation_yaw) (`KismetMathLibrary.BreakRotator` (`SceneComponent.RelativeRotation` _blower_mesh)))
  (`|ExecutionSequence`
    (:`then_0`
      (bind _was_valid (`/Game/MyContent/Blueprints/ConfigMachine_BPFL.Transform Attached Mask Decal` (`self.Decal Start Positions`) (`self.Decal End Positions`) (`self.Spawned Decals`) self))
      (if (not _was_valid)
        (`self.Emergency Decal Killer`)))
    (:`then_1`
      (bind _isa (`/Engine/EditorBlueprintResources/StandardMacros.FlipFlop`)
        (:`A`
          _)
        (:`B`
          _))
      (`SceneComponent.K2_SetRelativeRotation` _blower_mesh (`KismetMathLibrary.MakeRotator` _relativerotation_roll (+ _relativerotation_pitch (`KismetMathLibrary.SelectFloat` _rattle_anim_value (* _rattle_anim_value -1.0) _isa)) _relativerotation_yaw) false false))))

(event `self.ReceiveBeginPlay`
  (bind (_relativerotation_roll _relativerotation_pitch) (`KismetMathLibrary.BreakRotator` (`SceneComponent.RelativeRotation` (`self.Blower_MESH`))))
  (`self.Initialize Blower on Begin Play`)
  (set `self.Blower MESH Relative Pitch Default` _relativerotation_pitch))

(event `self.Start`
  (params (`Other Actor` :type "Actor Object Reference"))
  (bind _blower_mesh (`self.Blower_MESH`))
  (bind (_relativerotation_roll _relativerotation_pitch _relativerotation_yaw) (`KismetMathLibrary.BreakRotator` (`SceneComponent.RelativeRotation` _blower_mesh)))
  (`|ExecutionSequence`
    (:`then_0`
      (set `self.Car ID` (`|GetArrayItem` (`Actor.Tags` `Other Actor`) 2)))
    (:`then_1`
      (bind (_decal_start_pos_out _decal_end_pos_out _spawned_decal_out _car_id_tag_out) (`/Game/MyContent/Blueprints/ConfigMachine_BPFL.Spawn Attached Mask Decal` `Other Actor` (`self.SprayerLocation`) "/Game/MyContent/maskExclusionDecal.maskExclusionDecal" self true (`self.Custom Decal Transform`)))
      (`BlueprintMapLibrary.Map_Add` (`self.Decal Start Positions`) _car_id_tag_out _decal_start_pos_out)
      (`BlueprintMapLibrary.Map_Add` (`self.Decal End Positions`) _car_id_tag_out _decal_end_pos_out)
      (`DecalComponent.SetFadeIn` _spawned_decal_out 0.0 2.0)
      (`DecalComponent.SetSortOrder` _spawned_decal_out 999)
      (`BlueprintMapLibrary.Map_Add` (`self.Spawned Decals`) _car_id_tag_out _spawned_decal_out)
      (for _array_element (`self.Particle Emitters`)
        (`ActorComponent.Activate` _array_element false))
      (`self.SetActorTickEnabled` true)
      (`SceneComponent.K2_SetRelativeRotation` _blower_mesh (`KismetMathLibrary.MakeRotator` _relativerotation_roll (`self.Blower MESH Relative Pitch Default`) _relativerotation_yaw) false false :!label _label))))

(event `self.Moment On Start`
  (for _array_element (`self.Particle Emitters`)
    (`ActorComponent.Activate` _array_element false)))

(event `self.Moment On End`
  (for _array_element (`self.Particle Emitters`) :!label _label_2
    (`ActorComponent.Deactivate` _array_element))
  (`self.SetActorTickEnabled` false)
  (goto _label))

(event `self.SprayerLocation.OnComponentEndOverlap`
  (params (OverlappedComponent :type "PrimitiveComponent Object Reference") (OtherActor :type "Actor Object Reference") (OtherComp :type "PrimitiveComponent Object Reference") (OtherBodyIndex :type Integer))
  (bind _car_id (`self.Car ID`))
  (bind (_value _returnvalue) (`BlueprintMapLibrary.Map_Find` (`self.Decal End Positions`) _car_id))
  (bind (_value_2 _returnvalue_2) (`BlueprintMapLibrary.Map_Find` (`self.Decal Start Positions`) _car_id))
  (bind _output (`|GetArrayItem` (`Actor.Tags` OtherActor) 2))
  (if (`ActorComponent.ComponentHasTag` OverlappedComponent "Rear Of Car")
    (`|ExecutionSequence`
      (:`then_0`
        (if (!= _output "None")
          (set `self.Car ID` _output)))
      (:`then_1`
        (if (and _returnvalue _returnvalue_2) :!label _label_3
          (`SceneComponent.K2_AttachToComponent` _value (`SceneComponent.GetAttachParent` _value_2) "None" "KeepWorld" "KeepWorld" "KeepWorld" true))))))

(event `self.End`
  (`|ExecutionSequence`
    (:`then_0`
      (goto _label_3))
    (:`then_1`
      (goto _label_2))))

(event `self.DestroyDecal.OnComponentEndOverlap`
  (params (OverlappedComponent :type "PrimitiveComponent Object Reference") (OtherActor :type "Actor Object Reference") (OtherComp :type "PrimitiveComponent Object Reference") (OtherBodyIndex :type Integer))
  (if (`ActorComponent.ComponentHasTag` OtherComp "Rear Of Car")
    (bind (_decal_start_positions_out _decal_end_positions_out _spawned_decals_out) (`/Game/MyContent/Blueprints/ConfigMachine_BPFL.Destroy Attached Mask Decal` (`|GetArrayItem` (`Actor.Tags` OtherActor) 2) (`self.Decal Start Positions`) (`self.Decal End Positions`) (`self.Spawned Decals`) self))
    (set `self.Decal Start Positions` _decal_start_positions_out)
    (set `self.Decal End Positions` _decal_end_positions_out)
    (set `self.Spawned Decals` _spawned_decals_out)))

(event `Emergency Decal Killer`
  (bind (_decal_start_positions_out _decal_end_positions_out _spawned_decals_out) (`/Game/MyContent/Blueprints/ConfigMachine_BPFL.Destroy Attached Mask Decal` "None" (`self.Decal Start Positions`) (`self.Decal End Positions`) (`self.Spawned Decals`) self))
  (set `self.Decal Start Positions` _decal_start_positions_out)
  (set `self.Decal End Positions` _decal_end_positions_out)
  (set `self.Spawned Decals` _spawned_decals_out))

(fn `Initialize Blower on Begin Play`
  (locals (`Socket Number` :type Integer :default 0))
  (bind _returnvalue (`KismetMathLibrary.MakeTransform` (0.0 0.0 100.0) (struct :`Pitch` -90.0 :`Yaw` 180.0) (300.0 1.0 110.0)))
  (bind _socket_number (`local.Socket Number`))
  (bind _socket_number_2 (`local.Socket Number`))
  (bind _array (`|MakeArray` (`self.Niagara1`) (`self.Niagara2`) (`self.Niagara3`) (`self.Niagara4`) (`self.Niagara5`) (`self.Niagara6`) :!type "SceneComponent Object Reference"))
  (bind _asmaster_machine_bp (cast `/Game/MyContent/Blueprints/ConfigurableMachines/MasterMachine_BP` (`self.GetParentActor`)))
  (`|ExecutionSequence`
    (:`then_0`
      (bind _in_which_socket (`/Game/MyContent/Blueprints/ConfigurableMachines/MasterMachine_BP.In which socket` _asmaster_machine_bp))
      (set `local.Socket Number` (`KismetStringLibrary.Conv_StringToInt` (`KismetStringLibrary.Right` (`KismetStringLibrary.Conv_NameToString` _in_which_socket) 1)))
      (`SceneComponent.K2_AttachToComponent` (`self.Blower_MESH`) (`self.GetComponentByClass` (`/Game/MyContent/Blueprints/ConfigurableMachines/MasterMachine_BP.Actor to attach to` _asmaster_machine_bp) "/Script/Engine.StaticMeshComponent") _in_which_socket "KeepRelative" "KeepRelative" "KeepRelative" false)
      (`|ExecutionSequence`
        (:`then_0`
          (if (or (== _socket_number_2 1) (== _socket_number_2 6))
            (`StaticMeshComponent.SetStaticMesh` (`self.Blower_MESH`) "/Game/MyContent/Meshes/Blowers/Blower_2_MESH.Blower_2_MESH")
            (set `self.Particle Emitters` _array)
            (`ActorComponent.K2_DestroyComponent` (`self.Niagara10`))
            (else
              (set `self.Particle Emitters` (`|MakeArray` (`self.Niagara10`) :!type "SceneComponent Object Reference"))
              (for _array_element _array
                (`ActorComponent.K2_DestroyComponent` _array_element)))))
        (:`then_1`
          (`SceneComponent.K2_AddLocalTransform` (`self.Blower_MESH`) (`KismetMathLibrary.MakeTransform` (select `int` _socket_number :`0` (0.0 0.0 0.0) :`1` (0.0 0.0 0.0) :`2` (6.5 0.0 1.25) :`3` (0.0 0.0 0.0) :`4` (0.0 0.0 0.0) :`5` (-6.5 0.0 1.25) :`6` (0.0 0.0 0.0) :!type "Vector Structure") (`KismetMathLibrary.MakeRotator` 0.0 (select `int` _socket_number :`0` 0.0 :`1` 0.0 :`2` 25.0 :`3` 0.0 :`4` 0.0 :`5` -25.0 :`6` 0.0 :!type "Float (single-precision)")) (`KismetMathLibrary.MakeVector` (select `int` _socket_number :`0` 1.0 :`1` 1.0 :`2` -1.0 :`3` 1.0 :`4` -1.0 :`5` 1.0 :`6` -1.0 :!type "Float (single-precision)") 1.0 1.0)) false false)
          (for _array_element_2 (`self.Particle Emitters`)
            (`SceneComponent.K2_AddWorldRotation` _array_element_2 (`KismetMathLibrary.MakeRotator` 0.0 (select `int` _socket_number :`0` 0.0 :`1` 0.0 :`2` 180.0 :`3` 0.0 :`4` 180.0 :`5` 0.0 :`6` 180.0 :!type "Float (single-precision)")) false false)))
        (:`then_2`
          (set `self.Custom Decal Transform` (select `int` (`local.Socket Number`) :`0` (`KismetMathLibrary.MakeTransform` (0.0 0.0 100.0) (struct :`Pitch` -90.0 :`Yaw` 180.0) (300.0 1.0 300.0)) :`1` (`KismetMathLibrary.MakeTransform` (-250.0 0.0 100.0) (struct :`Pitch` -90.0 :`Yaw` 180.0) (300.0 1.0 300.0)) :`2` (`KismetMathLibrary.MakeTransform` (-100.0 0.0 100.0) (struct :`Pitch` -70.0 :`Yaw` 360.0) (300.0 1.0 110.0)) :`3` _returnvalue :`4` _returnvalue :`5` (`KismetMathLibrary.MakeTransform` (100.0 0.0 100.0) (struct :`Pitch` -70.0 :`Yaw` 180.0) (300.0 1.0 110.0)) :`6` (`KismetMathLibrary.MakeTransform` (250.0 0.0 100.0) (struct :`Pitch` -90.0 :`Yaw` 180.0) (300.0 1.0 300.0))))
          (set `self.Rattle Anim Value` (select `int` (`local.Socket Number`) :`0` 0.5 :`1` 0.25 :`2` 0.5 :`3` 0.5 :`4` 0.5 :`5` 0.5 :`6` 0.25 :!type "Float (single-precision)")))))
    (:`then_1`
      (set `self.Master Machines to Link With` (`/Game/MyContent/Blueprints/ConfigurableMachines/MasterMachine_BP.Machines to Link With` _asmaster_machine_bp)))))

(fn `UserConstructionScript`
  (`|ExecutionSequence`
    (:`then_0`
      (set `ActorComponent.ComponentTags` (`|MakeArray` "grab" "setInFront" :!type "Name") (`self.Blower_MESH`)))
    (:`then_1`
      ;[0.15 0.1244 0.03967 0.5] This wouldn't be necessary if destroy decal was working as intended.
      (bind _outactors (`GameplayStatics.GetAllActorsOfClassWithTag` "/Script/Engine.Actor" "DestroyDecalDefaultLocation"))
      (bind _output_get (set `self.Destroy Decal Default World Location` (`self.K2_GetActorLocation` (`|GetArrayItem` _outactors))))
      (`SceneComponent.K2_SetWorldLocation` (`self.DestroyDecal`) _output_get false false))))