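; Configurable tire brush machine, apparently for a car wash, with two Control Rig-driven frames that move in on Start and retract on End or Reverse.
; One frame eases toward a per-frame ramped Target via FInterpTo, halting the ramp when its imposter hitbox overlaps car collision; the other follows a Timeline.
; Tick runs only from Start until the interpolated brush is back home.
; Construction tags hitboxes and frames for grabbing.
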(event `self.ReceiveBeginPlay`
  ; I don't know why this BP is starting with tick enabled. I told it not to, but it won't obey, so this is what it gets.
  (`self.SetActorTickEnabled` false))

(event `self.Start`
  (params (`Other Actor` :type "Actor Object Reference"))
  (`|ExecutionSequence`
    (:`then_0`
      (set `self.Brush Going In` true))
    (:`then_1`
      (`self.SetActorTickEnabled` true))
    (:`then_2`
      (`self.Set Target` true (`self.By`) :!label _label)
      (`KismetSystemLibrary.DelayUntilNextTick`)
      (if (not (or (>= (`self.Target`) 1.0) (not (`self.Brush Going In`))))
        (goto _label)))
    (:`then_3`
      (bind (_direction _alpha) (`Timeline|Timeline` :!label _label_2)
        (:`Update`
          (`ControlRigComponent.SetControlPosition` (`self.ControlRig1`) "Control" (`KismetMathLibrary.MakeVector` (`KismetMathLibrary.Lerp` -85.0 -66.0 _alpha)) "LocalSpace"))))))

(event `self.ReceiveTick`
  (params (DeltaSeconds :type "Float (single-precision)"))
  (bind _returnvalue_x (`KismetMathLibrary.BreakVector` (`ControlRigComponent.GetControlPosition` (`self.ControlRig`) "Control" "LocalSpace")))
  (bind _returnvalue (`KismetMathLibrary.FInterpTo` (`self.Current`) (`self.Target`) (`GameplayStatics.GetWorldDeltaSeconds`) (`self.Interp Speed`)))
  (`|ExecutionSequence`
    (:`then_0`
      (`KismetSystemLibrary.Delay` 1.0)
      (if (and (`KismetMathLibrary.NearlyEqual_FloatFloat` _returnvalue_x -85.0 1.5) (not (`self.Brush Going In`)))
        (`self.SetActorTickEnabled` false)))
    (:`then_1`
      (set `self.Current` _returnvalue)
      (`ControlRigComponent.SetControlPosition` (`self.ControlRig`) "Control" (`KismetMathLibrary.MakeVector` (`KismetMathLibrary.Lerp` -85.0 -30.0 _returnvalue)) "LocalSpace"))))

(event `self.End`
  (`|ExecutionSequence` :!label _label_3
    (:`then_0`
      (set `self.Brush Going In` false))
    (:`then_1`
      (`self.Set Target` false (`self.By`) :!label _label_4)
      (`KismetSystemLibrary.DelayUntilNextTick`)
      (if (not (or (<= (`self.Target`) 0.0) (`self.Brush Going In`)))
        (goto _label_4)))
    (:`then_2`
      (goto _label_2 :!via `Reverse`))))

(event `Reverse`
  (goto _label_3))

(event `self.Hit_Brush_Imposter.OnComponentBeginOverlap`
  (params (OverlappedComponent :type "PrimitiveComponent Object Reference") (OtherActor :type "Actor Object Reference") (OtherComp :type "PrimitiveComponent Object Reference") (OtherBodyIndex :type Integer) (bFromSweep :type Boolean) (SweepResult :type "HitResult Structure (by ref)"))
  (if (`ActorComponent.ComponentHasTag` OtherComp "carCollision")
    (set `self.Brush Going In` false)))

(event `self.ControlRig.OnPreInitializeDelegate`
  (params (Component :type "ControlRigComponent Object Reference"))
  (`ControlRigComponent.AddMappedCompleteSkeletalMesh` Component (`self.TireBrushFrame_MESH`) "Output"))

(event `self.ControlRig1.OnPreInitializeDelegate`
  (params (Component :type "ControlRigComponent Object Reference"))
  (`ControlRigComponent.AddMappedCompleteSkeletalMesh` Component (`self.TireBrushFrame_MESH1`) "Output"))

(fn `Set Target`
  (params (Add :type Boolean) (By :type "Float (double-precision)" :default 0.2))
  (if Add
    (set `self.Target` (+ (`self.Target`) (* By (`GameplayStatics.GetWorldDeltaSeconds`))))
    (else
      (set `self.Target` (- (`self.Target`) (* By (`GameplayStatics.GetWorldDeltaSeconds`)))))))

(fn `UserConstructionScript`
  (for _array_element (`|MakeArray` (`self.Hitbox_Frame`) (`self.Hitbox_Frame1`))
    (set `ActorComponent.ComponentTags` (`|MakeArray` "grab" :!type "Name") _array_element)
    (set `ActorComponent.ComponentTags` (`|MakeArray` "nograb" "setInFront" "Frame_R" :!type "Name") (`self.TireBrushFrame_MESH`))
    (set `ActorComponent.ComponentTags` (`|MakeArray` "nograb" "setInFront" "Frame_L" :!type "Name") (`self.TireBrushFrame_MESH1`))))