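; Tire brush sprayer part of a configurable machine, providing two sprayer meshes and four low-pressure water Niagara effects.
; On BeginPlay it reads the parent MasterMachine_BP's ActorToAttachTo and snaps each mesh to a tagged left or right box on that actor's first child actor.
; Start and End switch all water effects on or off through ToggleSprayers.
; The construction script tags hit boxes as grabbable and meshes as non-grabbable, set-in-front.
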(event `self.ReceiveBeginPlay`
  (bind _asmaster_machine_bp (cast `/Game/MyContent/Blueprints/ConfigurableMachines/MasterMachine_BP` (`self.GetParentActor`)))
  (bind _output (`|GetArrayItem` (`self.GetAllChildActors` (`/Game/MyContent/Blueprints/ConfigurableMachines/MasterMachine_BP.Actor to attach to` _asmaster_machine_bp) false)))
  (`SceneComponent.K2_AttachToComponent` (`self.Sprayer_MESH`) (`|GetArrayItem` (`self.GetComponentsByTag` _output "/Script/Engine.BoxComponent" "H20_Attach_L")) "H20_Attach" "SnapToTarget" "KeepRelative" "KeepRelative" true)
  (`SceneComponent.K2_AttachToComponent` (`self.Sprayer_MESH1`) (`|GetArrayItem` (`self.GetComponentsByTag` _output "/Script/Engine.BoxComponent" "H20_Attach_R")) "H20_Attach1" "SnapToTarget" "KeepRelative" "KeepRelative" true))

(event `self.Start`
  (params (`Other Actor` :type "Actor Object Reference"))
  (`self.Toggle Sprayers` true))

(event `Toggle Sprayers`
  (params (On :type Boolean))
  (for _array_element (`|MakeArray` (`self.LowPressureWater_NS`) (`self.LowPressureWater_NS1`) (`self.LowPressureWater_NS3`) (`self.LowPressureWater_NS2`))
    (if On
      (`ActorComponent.Activate` _array_element false)
      (else
        (`ActorComponent.Deactivate` _array_element)))))

(event `self.End`
  (`self.Toggle Sprayers` false))

(fn `UserConstructionScript`
  (for _array_element (`|MakeArray` (`self.HitBox_Sprayer`) (`self.HitBox_Sprayer1`))
    (set `ActorComponent.ComponentTags` (`|MakeArray` "grab" :!type "Name") _array_element))
  (for _array_element_2 (`|MakeArray` (`self.Sprayer_MESH`) (`self.Sprayer_MESH1`))
    (set `ActorComponent.ComponentTags` (`|MakeArray` "nograb" "setInFront" :!type "Name") _array_element_2)))