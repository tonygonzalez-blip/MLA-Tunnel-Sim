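; Car wash blower machine that toggles particle emitters and spawns mask-exclusion decals on passing cars.
; Start stores each decal and its start/end points in maps keyed by car ID tag; Tick transforms them, clearing on failure.
; End or rear-of-car exit attaches the end point alongside the start.
; The DestroyDecal volume, shared with machines linked through the parent MasterMachine_BP, removes decals when the car's rear leaves it.
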(event `self.ReceiveBeginPlay`
  (bind _asmaster_machine_bp (cast `/Game/MyContent/Blueprints/ConfigurableMachines/MasterMachine_BP` (`self.GetParentActor`)))
  (set `self.Master Machines to Link With` (`/Game/MyContent/Blueprints/ConfigurableMachines/MasterMachine_BP.Machines to Link With` _asmaster_machine_bp)))

(event `self.ReceiveTick`
  (params (DeltaSeconds :type "Float (single-precision)"))
  (bind _was_valid (`/Game/MyContent/Blueprints/ConfigMachine_BPFL.Transform Attached Mask Decal` (`self.Decal Start Positions`) (`self.Decal End Positions`) (`self.Spawned Decals`) self))
  (if (not _was_valid)
    (`self.Emergency Decal Killer`)))

(event `/Game/FirstPerson/Blueprints/ConfigMachine_BPI.Start`
  (params (`Other Actor` :type "Actor Object Reference"))
  (`|ExecutionSequence`
    (:`then_0`
      (set `self.Car ID` (`|GetArrayItem` (`Actor.Tags` `Other Actor`) 2)))
    (:`then_1`
      (bind (_decal_start_pos_out _decal_end_pos_out _spawned_decal_out _car_id_tag_out) (`/Game/MyContent/Blueprints/ConfigMachine_BPFL.Spawn Attached Mask Decal` `Other Actor` (`self.SprayerLocation`) "/Game/MyContent/maskExclusionDecal.maskExclusionDecal" self))
      (`BlueprintMapLibrary.Map_Add` (`self.Decal Start Positions`) _car_id_tag_out _decal_start_pos_out)
      (`BlueprintMapLibrary.Map_Add` (`self.Decal End Positions`) _car_id_tag_out _decal_end_pos_out)
      (`DecalComponent.SetFadeIn` _spawned_decal_out 0.0 2.0)
      (`DecalComponent.SetSortOrder` _spawned_decal_out 999)
      (`BlueprintMapLibrary.Map_Add` (`self.Spawned Decals`) _car_id_tag_out _spawned_decal_out)
      (for _array_element (`self.Particle Emitters`)
        (`ActorComponent.Activate` _array_element false))
      (for _array_element_2 (`self.Master Machines to Link With`)
        (message `/Game/FirstPerson/Blueprints/ConfigMachine_BPI.Set DestroyDecal Location` _array_element_2 (`self.DestroyDecal`) (0.0 0.0 0.0))))))

(event `/Game/FirstPerson/Blueprints/ConfigMachine_BPI.Moment On End`
  (for _array_element (`self.Particle Emitters`) :!label _label
    (`ActorComponent.Deactivate` _array_element)))

(event `/Game/FirstPerson/Blueprints/ConfigMachine_BPI.Moment On Start`
  (for _array_element (`self.Particle Emitters`)
    (`ActorComponent.Activate` _array_element false)))

(event `self.SprayerLocation.OnComponentBeginOverlap`
  (params (OverlappedComponent :type "PrimitiveComponent Object Reference") (OtherActor :type "Actor Object Reference") (OtherComp :type "PrimitiveComponent Object Reference") (OtherBodyIndex :type Integer) (bFromSweep :type Boolean) (SweepResult :type "HitResult Structure (by ref)"))
  ; See SoapSprayer_BP
)

(event `self.SprayerLocation.OnComponentEndOverlap`
  (params (OverlappedComponent :type "PrimitiveComponent Object Reference") (OtherActor :type "Actor Object Reference") (OtherComp :type "PrimitiveComponent Object Reference") (OtherBodyIndex :type Integer))
  (bind _car_id (`self.Car ID`))
  (bind (_value _returnvalue) (`BlueprintMapLibrary.Map_Find` (`self.Decal End Positions`) _car_id))
  (bind (_value_2 _returnvalue_2) (`BlueprintMapLibrary.Map_Find` (`self.Decal Start Positions`) _car_id))
  (bind _output (`|GetArrayItem` (`Actor.Tags` OtherActor) 2))
  (if (`ActorComponent.ComponentHasTag` OverlappedComponent "Rear Of Car")
    (`|ExecutionSequence`
      (:`then_0`
        (if (!= _output "None")
          (set `self.Car ID` _output)))
      (:`then_1`
        (if (and _returnvalue _returnvalue_2) :!label _label_2
          (`SceneComponent.K2_AttachToComponent` _value (`SceneComponent.GetAttachParent` _value_2) "None" "KeepWorld" "KeepWorld" "KeepWorld" true))))))

(event `/Game/FirstPerson/Blueprints/ConfigMachine_BPI.End`
  (`|ExecutionSequence`
    (:`then_0`
      (goto _label_2))
    (:`then_1`
      (goto _label))))

(event `self.DestroyDecal.OnComponentEndOverlap`
  (params (OverlappedComponent :type "PrimitiveComponent Object Reference") (OtherActor :type "Actor Object Reference") (OtherComp :type "PrimitiveComponent Object Reference") (OtherBodyIndex :type Integer))
  (if (`ActorComponent.ComponentHasTag` OtherComp "Rear Of Car")
    (bind (_decal_start_positions_out _decal_end_positions_out _spawned_decals_out) (`/Game/MyContent/Blueprints/ConfigMachine_BPFL.Destroy Attached Mask Decal` (`|GetArrayItem` (`Actor.Tags` OtherActor) 2) (`self.Decal Start Positions`) (`self.Decal End Positions`) (`self.Spawned Decals`) self))
    (set `self.Decal Start Positions` _decal_start_positions_out)
    (set `self.Decal End Positions` _decal_end_positions_out)
    (set `self.Spawned Decals` _spawned_decals_out)))

(event `Emergency Decal Killer`
  (bind (_decal_start_positions_out _decal_end_positions_out _spawned_decals_out) (`/Game/MyContent/Blueprints/ConfigMachine_BPFL.Destroy Attached Mask Decal` "None" (`self.Decal Start Positions`) (`self.Decal End Positions`) (`self.Spawned Decals`) self))
  (set `self.Decal Start Positions` _decal_start_positions_out)
  (set `self.Decal End Positions` _decal_end_positions_out)
  (set `self.Spawned Decals` _spawned_decals_out))

(fn `UserConstructionScript`
  (bind _blowers_mesh (`self.Blowers_MESH`))
  (`|ExecutionSequence`
    (:`then_0`
      (set `ActorComponent.ComponentTags` (`|MakeArray` "passGrab" :!type "Name") (`self.MESH_GenericArch`))
      (set `ActorComponent.ComponentTags` (`|MakeArray` "grab" "setInFront" :!type "Name") _blowers_mesh)
      (set `self.Particle Emitters` (`SceneComponent.GetChildrenComponents` _blowers_mesh false)))
    (:`then_1`
      ;[0.15 0.1244 0.03967 0.5] This wouldn't be necessary if destroy decal was working as intended.
      (bind _outactors (`GameplayStatics.GetAllActorsOfClassWithTag` "/Script/Engine.Actor" "DestroyDecalDefaultLocation"))
      (bind _output_get (set `self.Destroy Decal Default World Location` (`self.K2_GetActorLocation` (`|GetArrayItem` _outactors))))
      (`SceneComponent.K2_SetWorldLocation` (`self.DestroyDecal`) _output_get false false))))