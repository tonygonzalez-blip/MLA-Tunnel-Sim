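; Car wash brush arm machine part that swings in on Start, retracts on End, and reacts to passing cars.
; Per-tick loops ramp a target alpha that Tick eases into arm yaw, aiming the piston and disabling tick once parked.
; An imposter overlap backs the arm off car collision, or swings it in at the rear while briefly ignoring collisions.
; Construction mirrors the stand from the parent MasterMachine_BP, tags components and sets up the cable.
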(event `Move Brush0 In`
  (set `self.Brush0 Going In` true)
  (`self.Set Target` true (`self.By`) :!label _label)
  (`KismetSystemLibrary.DelayUntilNextTick`)
  (if (not (or (>= (`self.Target`) 1.0) (not (`self.Brush0 Going In`))))
    (goto _label)))

(event `self.ReceiveBeginPlay`
  (bind (_relativerotation_roll _relativerotation_pitch _relativerotation_yaw) (`KismetMathLibrary.BreakRotator` (`SceneComponent.RelativeRotation` (`self.BrushArm_MESH`))))
  (set `self.Brush0 End` -35.0)
  (bind _output_get (set `self.Brush0 Start` _relativerotation_yaw))
  (set `self.Brush0 Start_Default` _output_get))

(event `Move Brush0 Out`
  (set `self.Brush0 Going In` false)
  (`self.Set Target` false (`self.By`) :!label _label_2)
  (`KismetSystemLibrary.DelayUntilNextTick`)
  (if (not (or (<= (`self.Target`) 0.0) (`self.Brush0 Going In`)))
    (goto _label_2)))

(event `self.ReceiveTick`
  (params (DeltaSeconds :type "Float (single-precision)"))
  (bind _returnvalue (`KismetMathLibrary.FInterpTo` (`self.Current`) (`self.Target`) (`GameplayStatics.GetWorldDeltaSeconds`) (`self.Interp Speed`)))
  (bind (_relativerotation_roll _relativerotation_pitch _relativerotation_yaw) (`KismetMathLibrary.BreakRotator` (`SceneComponent.RelativeRotation` (`self.BrushArm_MESH`))))
  (`|ExecutionSequence`
    (:`then_0`
      (`KismetSystemLibrary.Delay` 2.0)
      (if (and (`KismetMathLibrary.NearlyEqual_FloatFloat` _relativerotation_yaw (`self.Brush0 Start_Default`) 1.5) (not (`self.Brush0 Going In`)))
        (`self.SetActorTickEnabled` false)))
    (:`then_1`
      (set `self.Current` _returnvalue)
      (`SceneComponent.K2_SetRelativeRotation` (`self.BrushArm_MESH`) (`KismetMathLibrary.MakeRotator` 0.0 0.0 (`KismetMathLibrary.Lerp` (`self.Brush0 Start`) (`self.Brush0 End`) _returnvalue)) false false))
    (:`then_2`
      (`self.Piston Aim Math_Custom` (`self.BrushArmT_Stand_piston_MESH`) (`self.BrushArmT_piston_MESH`)))
    (:`then_3`
      (`SceneComponent.K2_AddRelativeRotation` (`self.Hit_Brush_Imposter`) (`KismetMathLibrary.MakeRotator` 0.0 0.0 0.1) false false))))

(event `/Game/FirstPerson/Blueprints/ConfigMachine_BPI.Start`
  (params (`Other Actor` :type "Actor Object Reference"))
  (`|ExecutionSequence`
    (:`then_0`
      (`KismetSystemLibrary.K2_ClearAndInvalidateTimerHandle` (`self.RHBICR Event Timer Ref`))
      (`self.Reset Hit Brush Imposter Collision Response`))
    (:`then_1`
      (set `self.By` 0.2)
      (set `self.Interp Speed` 3.0)
      (set `self.Enable Collision Movement` true)
      (`self.Move Brush0 In`)
      (`self.SetActorTickEnabled` true))))

(event `/Game/FirstPerson/Blueprints/ConfigMachine_BPI.End`
  (`KismetSystemLibrary.K2_ClearAndInvalidateTimerHandle` (`self.RHBICR Event Timer Ref`))
  (set `self.By` 0.2)
  (set `self.Interp Speed` 3.0)
  (set `self.Enable Collision Movement` false)
  (`self.Move Brush0 Out`))

(event `self.Hit_Brush_Imposter.OnComponentBeginOverlap`
  (params (OverlappedComponent :type "PrimitiveComponent Object Reference") (OtherActor :type "Actor Object Reference") (OtherComp :type "PrimitiveComponent Object Reference") (OtherBodyIndex :type Integer) (bFromSweep :type Boolean) (SweepResult :type "HitResult Structure (by ref)"))
  (if (and (`ActorComponent.ComponentHasTag` OtherComp "carCollision") (`self.Enable Collision Movement`))
    (`self.Move Brush0 Out`)
    (set `self.By` 0.1)
    (set `self.Interp Speed` 1.5)
    (elif (`ActorComponent.ComponentHasTag` OtherComp "Rear Of Car")
      (set `self.By` 0.1)
      (set `self.Interp Speed` 1.5)
      (`self.Move Brush0 In`)
      (`PrimitiveComponent.SetCollisionResponseToAllChannels` (`self.Hit_Brush_Imposter`) "ECR_Ignore")
      (bind _returnvalue (`KismetSystemLibrary.K2_SetTimerDelegate` (delegate `Reset Hit Brush Imposter Collision Response`) 2.0))
      (set `self.RHBICR Event Timer Ref` _returnvalue))))

(event `Reset Hit Brush Imposter Collision Response`
  (`PrimitiveComponent.SetCollisionResponseToAllChannels` (`self.Hit_Brush_Imposter`) "ECR_Overlap"))

(event `self.Hit_Brush_Imposter.OnComponentEndOverlap`
  (params (OverlappedComponent :type "PrimitiveComponent Object Reference") (OtherActor :type "Actor Object Reference") (OtherComp :type "PrimitiveComponent Object Reference") (OtherBodyIndex :type Integer))
  (if (and (`ActorComponent.ComponentHasTag` OtherComp "carCollision") (`self.Enable Collision Movement`))
    (set `self.Brush0 Going In` true)))

(fn `Piston Aim Math_Custom`
  (params (`Piston Mount` :type "SceneComponent Object Reference") (`Piston Extender` :type "SceneComponent Object Reference"))
  (bind _returnvalue (`KismetAnimationLibrary.K2_LookAt` (`SceneComponent.K2_GetComponentToWorld` (`local.Piston Mount`)) (`SceneComponent.K2_GetComponentLocation` (`local.Piston Extender`)) (0.0 0.0 -1.0) false (1.0 0.0 0.0)))
  (bind _returnvalue_2 (`KismetAnimationLibrary.K2_LookAt` (`SceneComponent.K2_GetComponentToWorld` (`local.Piston Extender`)) (`SceneComponent.K2_GetComponentLocation` (`local.Piston Mount`)) (0.0 0.0 1.0) false (1.0 0.0 0.0)))
  (`SceneComponent.K2_SetWorldRotation` (`local.Piston Mount`) (`KismetMathLibrary.MakeRotator` (.roll (.rotation _returnvalue)) 90.0 (.yaw (.rotation _returnvalue))) false false)
  (`SceneComponent.K2_SetWorldRotation` (`local.Piston Extender`) (`KismetMathLibrary.MakeRotator` (.roll (.rotation _returnvalue_2)) 90.0 (.yaw (.rotation _returnvalue_2))) false false))

(fn `Set Target`
  (params (Add :type Boolean) (By :type "Float (double-precision)" :default 0.1))
  (if Add
    (set `self.Target` (+ (`self.Target`) (* By (`GameplayStatics.GetWorldDeltaSeconds`))))
    (else
      (set `self.Target` (- (`self.Target`) (* By (`GameplayStatics.GetWorldDeltaSeconds`)))))))

(fn `UserConstructionScript`
  (bind _brusharm_stand_mesh (`self.BrushArm_Stand_MESH`))
  (bind _returnvalue (`SceneComponent.GetRelativeTransform` _brusharm_stand_mesh))
  (`|ExecutionSequence`
    (:`then_0`
      (bind _asmaster_machine_bp (cast `/Game/MyContent/Blueprints/ConfigurableMachines/MasterMachine_BP` (`self.GetParentActor`)))
      (if (`/Game/MyContent/Blueprints/ConfigurableMachines/MasterMachine_BP.Mirror` _asmaster_machine_bp)
        (`SceneComponent.K2_SetRelativeTransform` _brusharm_stand_mesh (`KismetMathLibrary.MakeTransform` (`KismetMathLibrary.MakeVector` (* (.x (.location _returnvalue)) -1.0) (.y (.location _returnvalue)) (.z (.location _returnvalue))) (.rotation _returnvalue) (`KismetMathLibrary.MakeVector` (* (.x (.scale _returnvalue)) -1.0) (.y (.scale _returnvalue)) (.z (.scale _returnvalue)))) false false)))
    (:`then_1`
      (set `ActorComponent.ComponentTags` (`|MakeArray` "grab" "setInFront" "BrushArm" :!type "Name") (`self.BrushArm_MESH`))
      (for _array_element (`|MakeArray` (`self.BrushArm_Stand_MESH`))
        (set `ActorComponent.ComponentTags` (`|MakeArray` "passGrab" :!type "Name") _array_element))
      (set `ActorComponent.ComponentTags` (`|MakeArray` "Brush_Connection" :!type "Name") (`self.Brush_Connection`))
      (`self.Piston Aim Math_Custom` (`self.BrushArmT_Stand_piston_MESH`) (`self.BrushArmT_piston_MESH`)))
    (:`then_2`
      (`/Game/MyContent/Blueprints/ConfigMachine_BPFL.Cable Construction Script` self (`self.Cable`)))))