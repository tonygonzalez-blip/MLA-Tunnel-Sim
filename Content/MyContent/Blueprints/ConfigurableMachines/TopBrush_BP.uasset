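; Car wash top brush module that snaps its hitbox to the TopBrush_Connection box under its parent MasterMachine_BP.
; Start and End drive a timeline that ramps spin and material droop through custom primitive data, with Tick sustaining full-speed spin.
; While the hitbox overlaps a car, it attaches a fading mask-exclusion decal every second, sorted above earlier ones.
; A DestroyDecal volume, repositionable once per Start, clears decals as the car's rear exits it.
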(event `self.ReceiveBeginPlay`
  (bind _asmaster_machine_bp (cast `/Game/MyContent/Blueprints/ConfigurableMachines/MasterMachine_BP` (`self.GetParentActor`)))
  (`SceneComponent.K2_AttachToComponent` (`self.Hitbox_Brush`) (`|GetArrayItem` (`self.GetComponentsByTag` (`|GetArrayItem` (`self.GetAllChildActors` (`/Game/MyContent/Blueprints/ConfigurableMachines/MasterMachine_BP.Actor to attach to` _asmaster_machine_bp) false)) "/Script/Engine.BoxComponent" "TopBrush_Connection")) "None" "SnapToTarget" "KeepRelative" "KeepRelative" true))

(event `self.ReceiveTick`
  (params (DeltaSeconds :type "Float (single-precision)"))
  (bind _brush (`self.Brush`))
  (bind (_relativerotation_roll _relativerotation_pitch _relativerotation_yaw) (`KismetMathLibrary.BreakRotator` (`SceneComponent.RelativeRotation` _brush)))
  (`SceneComponent.K2_SetRelativeRotation` _brush (`KismetMathLibrary.MakeRotator` (+ _relativerotation_roll (* (* (`GameplayStatics.GetWorldDeltaSeconds`) 50.0) -10.0)) _relativerotation_pitch _relativerotation_yaw) false false))

(event `/Game/FirstPerson/Blueprints/ConfigMachine_BPI.Start`
  (params (`Other Actor` :type "Actor Object Reference"))
  (bind _brush (`self.Brush`))
  (bind (_relativerotation_roll _relativerotation_pitch _relativerotation_yaw) (`KismetMathLibrary.BreakRotator` (`SceneComponent.RelativeRotation` _brush)))
  (`|ExecutionSequence`
    (:`then_0`
      (bind (_direction _droop) (`Timeline|Timeline_2` :!label _label)
        (:`Update`
          (`PrimitiveComponent.SetScalarParameterForCustomPrimitiveData` (`self.Brush`) "Droop" (`KismetMathLibrary.Lerp` -0.12 0.0 _droop))
          (`SceneComponent.K2_SetRelativeRotation` _brush (`KismetMathLibrary.MakeRotator` (+ _relativerotation_roll (* (* (`GameplayStatics.GetWorldDeltaSeconds`) 50.0) (`KismetMathLibrary.Lerp` 0.0 -10.0 _droop))) _relativerotation_pitch _relativerotation_yaw) false false))
        (:`Finished`
          (if (`|EnumEquality` _direction "Forward")
            (`self.SetActorTickEnabled` true)
            (set `StaticMeshComponent.bEvaluateWorldPositionOffsetInRayTracing` false (`self.Brush`))
            (else
              (`self.SetActorTickEnabled` false))))))
    (:`then_1`
      (`SceneComponent.K2_SetWorldLocation` (`self.DestroyDecal`) (`self.Destroy Decal Default World Location`) false false)
      (set `self.Destroy Decal Moved` false))))

(event `/Game/FirstPerson/Blueprints/ConfigMachine_BPI.End`
  (`|ExecutionSequence`
    (:`then_0`
      (goto _label :!via `Reverse`))
    (:`then_1`
      (`self.SetActorTickEnabled` false)
      (set `StaticMeshComponent.bEvaluateWorldPositionOffsetInRayTracing` true (`self.Brush`)))))

(event `self.Hitbox_Brush.OnComponentBeginOverlap`
  (params (OverlappedComponent :type "PrimitiveComponent Object Reference") (OtherActor :type "Actor Object Reference") (OtherComp :type "PrimitiveComponent Object Reference") (OtherBodyIndex :type Integer) (bFromSweep :type Boolean) (SweepResult :type "HitResult Structure (by ref)"))
  (bind _actor_we_overlapped_here (`self.Actor We Overlapped Here`))
  (bind _hitbox_brush (`self.Hitbox_Brush`))
  (if (and (`self.ActorHasTag` OtherActor "car") (`KismetArrayLibrary.Array_IsNotEmpty` (`self.K2_GetComponentsByClass` OtherActor "/Script/Engine.StaticMeshComponent")))
    (`/Engine/EditorBlueprintResources/StandardMacros.DoOnce` false :!label _label_2
      (:`Completed`
        (`|ExecutionSequence`
          (:`then_0`
            (bind _output_get (set `self.Actor We Overlapped Here` OtherActor))
            (bind _ascar_1_bp (cast `/Game/MyContent/Blueprints/Car1_BP` _output_get))
            (`/Game/MyContent/Blueprints/Car1_BP.Increment Decal Sort Order` _ascar_1_bp)
            (set `self.Sort Order` (`/Game/MyContent/Blueprints/Car1_BP.Current Decal Sort Order` _ascar_1_bp)))
          (:`then_1`
            (bind _returnvalue (`GameplayStatics.SpawnDecalAttached` "/Game/MyContent/maskExclusionDecal.maskExclusionDecal" (115.0 115.0 155.0) (`|GetArrayItem` (`self.K2_GetComponentsByClass` _actor_we_overlapped_here "/Script/Engine.StaticMeshComponent")) "None" (`SceneComponent.K2_GetComponentLocation` _hitbox_brush) (struct :`Pitch` -45.0 :`Yaw` 90.0 :`Roll` -90.0) "KeepWorldPosition" :!label _label_3))
            (`DecalComponent.SetFadeIn` _returnvalue 0.0 1.0)
            (`DecalComponent.SetSortOrder` _returnvalue (`self.Sort Order`))
            (`KismetSystemLibrary.Delay` 1.0)
            (`KismetArrayLibrary.Array_Add` (`self.Spawned Decals`) _returnvalue)
            (if (`PrimitiveComponent.IsOverlappingActor` _hitbox_brush _actor_we_overlapped_here)
              (goto _label_3)
              (else
                (goto _label_2 :!via `Reset`)))))))))

(event `self.DestroyDecal.OnComponentEndOverlap`
  (params (OverlappedComponent :type "PrimitiveComponent Object Reference") (OtherActor :type "Actor Object Reference") (OtherComp :type "PrimitiveComponent Object Reference") (OtherBodyIndex :type Integer))
  (if (`ActorComponent.ComponentHasTag` OtherComp "Rear Of Car")
    (bind _spawned_decals_out (`/Game/MyContent/Blueprints/ConfigMachine_BPFL.Destroy Decal Actor and Refresh List` (`self.Spawned Decals`) OtherActor))
    (set `self.Spawned Decals` _spawned_decals_out)))

(event `/Game/FirstPerson/Blueprints/ConfigMachine_BPI.Set DestroyDecal Location`
  (params (`Destroy Decal` :type "BoxComponent Object Reference") (`Destroy Decal Locaiton` :type "Vector Structure"))
  (if (not (`self.Destroy Decal Moved`))
    (`SceneComponent.K2_SetWorldLocation` (`self.DestroyDecal`) (+ (`KismetMathLibrary.SelectVector` (`SceneComponent.K2_GetComponentLocation` `Destroy Decal`) `Destroy Decal Locaiton` (== `Destroy Decal Locaiton` (0.0 0.0 0.0) :`ErrorTolerance` 1.0)) (0.0 10.0 0.0)) false false)
    (set `self.Destroy Decal Moved` true)))

(fn `UserConstructionScript`
  (`|ExecutionSequence`
    (:`then_0`
      (set `ActorComponent.ComponentTags` (`|MakeArray` "grab" :!type "Name") (`self.Hitbox_Brush`))
      (set `ActorComponent.ComponentTags` (`|MakeArray` "nograb" "setInFront" :!type "Name") (`self.Brush`)))
    (:`then_1`
      (`PrimitiveComponent.SetScalarParameterForDefaultCustomPrimitiveData` (`self.Brush`) "Droop" -0.12))
    (:`then_2`
      (bind _outactors (`GameplayStatics.GetAllActorsOfClassWithTag` "/Script/Engine.Actor" "DestroyDecalDefaultLocation"))
      (bind _returnvalue (`self.K2_GetActorLocation` (`|GetArrayItem` _outactors)))
      (set `self.Destroy Decal Default World Location` _returnvalue)
      (`SceneComponent.K2_SetWorldLocation` (`self.DestroyDecal`) _returnvalue false false))
    (:`then_3`
      (`SceneComponent.K2_SetRelativeTransform` (`self.Hitbox_Brush`) (`KismetMathLibrary.MakeTransform` (0.0 0.0 0.0)) false false))))