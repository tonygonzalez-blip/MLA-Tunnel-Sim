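; Configurable tunnel conveyor that sends rollers behind arriving cars and notifies cars and machines when it switches on or off.
; A rear-tire trigger starts momentary-on service machines and a chain of roller spawns, each roller's overlap releasing the next.
; Tick moves rollers and drives speed-scaled flap and flip animations between entry, end triggers and kill zone.
; Toggling gates Tick, and an inactivity timer shuts it off unless monitored relays were active.
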(event `Start Flap Anim`
  (params (Reverse :type Boolean))
  (bind _output_get (set `self.Run Flap Reverse Animation` Reverse))
  (set `self.Flap Anim Alpha` (`KismetMathLibrary.SelectFloat` 1.0 0.0 _output_get))
  (set `self.Run Flap Animation` true))

(event `Start Flap End Anim`
  (params (Reverse :type Boolean))
  (bind _output_get (set `self.Run Flap End Reverse Animation` Reverse))
  (set `self.Flap End Anim Alpha` (`KismetMathLibrary.SelectFloat` 1.0 0.0 _output_get))
  (set `self.Run Flap End Animation` true))

(event `Start Roller Rotate Anim`
  (set `self.Roller Anim Alpha` 0.0)
  (set `self.Run Roller Rotate Animation` true))

(event `Start Roller End Rotate Anim`
  (set `self.Roller End Anim Alpha` 0.0)
  (set `self.Run Roller End Rotate Animation` true))

(event `self.ReceiveBeginPlay`
  (bind (_relativelocation_x _relativelocation_y) (`KismetMathLibrary.BreakVector` (`SceneComponent.RelativeLocation` (`self.RollerNearlyEndTrigger`))))
  (set `self.Roller Nearly End Trigger Start Y Pos` _relativelocation_y))

(event `self.RollerSendDelay_Trigger.OnComponentBeginOverlap`
  (params (OverlappedComponent :type "PrimitiveComponent Object Reference") (OtherActor :type "Actor Object Reference") (OtherComp :type "PrimitiveComponent Object Reference") (OtherBodyIndex :type Integer) (bFromSweep :type Boolean) (SweepResult :type "HitResult Structure (by ref)"))
  (if (`ActorComponent.ComponentHasTag` OtherComp "roller")
    (if (not (== (`self.# of rollers to be sent`) 0))
      (`|ExecutionSequence` :!label _label
        (:`then_0`
          (`self.Spawn Roller`))
        (:`then_1`
          (`|ExecutionSequence`
            (:`then_0`
              (`KismetSystemLibrary.Delay` (`KismetMathLibrary.FClamp` (- 0.5 (/ (`self.Conveyor Speed`) 10.0))))
              (`self.Start Flap Anim` false))
            (:`then_1`
              (`self.Start Roller Rotate Anim`))))
        (:`then_2`
          (bind _result (`/Engine/EditorBlueprintResources/StandardMacros.DecrementInt` (`self.# of rollers to be sent`))
            (:`  `
              (set `self.# of rollers to be sent` _result))))))))

(event `Toggle Conveyor`
  (params (On :type Boolean))
  (`self.SetActorTickEnabled` On)
  (`|ExecutionSequence`
    (:`then_0`
      (if On
        (`|ExecutionSequence`
          (:`then_0`
            (bind (_direction _lerp) (`Timeline|Timeline` :!label _label_2)
              (:`Update`
                (`LightComponent.SetIntensity` (`self.OnLight`) (`KismetMathLibrary.Lerp` 0.0 100.0 _lerp)))))
          (:`then_1`
            (`self.Reset Inactivity Timer`)))
        (else
          (goto _label_2 :!via `Reverse`))))
    (:`then_1`
      (`|ExecutionSequence`
        (:`then_0`
          (bind _outactors (`GameplayStatics.GetAllActorsOfClass` "/Game/MyContent/Blueprints/Car1_BP.Car1_BP_C"))
          (for _array_element _outactors
            (if On
              (`/Game/FirstPerson/Blueprints/ConfigMachine_BPI.Conveyor Turned On` _array_element)
              (else
                (`/Game/FirstPerson/Blueprints/ConfigMachine_BPI.Conveyor Turned Off` _array_element)))))
        (:`then_1`
          (bind _outactors_2 (`GameplayStatics.GetAllActorsOfClass` "/Game/MyContent/Blueprints/ConfigurableMachines/MasterMachine_BP.MasterMachine_BP_C"))
          (for _array_element_2 _outactors_2
            (if On
              (`/Game/FirstPerson/Blueprints/ConfigMachine_BPI.Conveyor Turned On` _array_element_2)
              (else
                (`/Game/FirstPerson/Blueprints/ConfigMachine_BPI.Conveyor Turned Off` _array_element_2)))))))
    (:`then_2`
      (bind _asmain_game_instance_gi (cast `/Game/FirstPerson/Blueprints/MainGameInstance_GI` (`GameplayStatics.GetGameInstance`)))
      (if (`/Game/FirstPerson/Blueprints/MainGameInstance_GI.Scenario1` _asmain_game_instance_gi)
        (`/Game/FirstPerson/Blueprints/Scenarios_FL.Search ScenarioChecklist_WBP` (`self.IsActorTickEnabled`) 7)))))

(event `self.CarStart_Trigger.OnComponentBeginOverlap`
  (params (OverlappedComponent :type "PrimitiveComponent Object Reference") (OtherActor :type "Actor Object Reference") (OtherComp :type "PrimitiveComponent Object Reference") (OtherBodyIndex :type Integer) (bFromSweep :type Boolean) (SweepResult :type "HitResult Structure (by ref)"))
  (if (`ActorComponent.ComponentHasTag` OtherComp "Rear Tires")
    (bind _ascar_1_bp (cast `/Game/MyContent/Blueprints/Car1_BP` OtherActor)
      (:`then`
        (bind _output_get (set `self.Car that started this cycle` _ascar_1_bp))
        (`/Game/MyContent/Blueprints/Car1_BP.Roller Trig Reached` _output_get))
      (:`CastFailed`
        _))
    (if (`self.IsActorTickEnabled`) :!label _label_3
      (`KismetSystemLibrary.Delay` 3.0)
      (set `self.# of rollers to be sent` (`self.Roller Count`))
      (`self.Check for Momentarily On service`)
      (goto _label)
      (else
        (`KismetSystemLibrary.Delay` 0.2)
        (goto _label_3)))))

(event `Flap Animation`
  (bind _tunnel_conveyorflap_mesh (`self.Tunnel_ConveyorFlap_MESH`))
  (bind (_relativerotation_roll _relativerotation_pitch _relativerotation_yaw) (`KismetMathLibrary.BreakRotator` (`SceneComponent.RelativeRotation` _tunnel_conveyorflap_mesh)))
  (bind _output_get (set `self.Flap Anim Alpha` (`KismetMathLibrary.FClamp` (`KismetMathLibrary.SelectFloat` (- (`self.Flap Anim Alpha`) (+ (`self.Anim Alpha Multiplier`) (* (- 1.0 (`self.Flap Anim Alpha`)) 0.4))) (+ (`self.Flap Anim Alpha`) (* (`self.Anim Alpha Multiplier`) (/ (`self.Conveyor Speed`) 10.0))) (`self.Run Flap Reverse Animation`)))))
  (`SceneComponent.K2_SetRelativeRotation` _tunnel_conveyorflap_mesh (`KismetMathLibrary.MakeRotator` (`KismetMathLibrary.Lerp` 0.0 20.0 _output_get) _relativerotation_pitch _relativerotation_yaw) false false))

(event `self.ReceiveTick`
  (params (DeltaSeconds :type "Float (single-precision)"))
  (bind _spawned_roller (`self.Spawned Roller`))
  (bind _run_flap_reverse_animation (`self.Run Flap Reverse Animation`))
  (bind _run_flap_end_reverse_animation (`self.Run Flap End Reverse Animation`))
  (bind (_returnvalue_roll _returnvalue_pitch _returnvalue_yaw) (`KismetMathLibrary.BreakRotator` (`self.K2_GetActorRotation` _spawned_roller)))
  (`|ExecutionSequence`
    (:`then_0`
      (for _array_element (`self.Roller List`)
        (`/Engine/EditorBlueprintResources/StandardMacros.IsValid` _array_element
          (:`Is Valid`
            (`self.K2_SetActorLocation` _array_element (+ (`self.K2_GetActorLocation` _array_element) (* (`self.GetActorRightVector` _array_element) (* (`GameplayStatics.GetWorldDeltaSeconds`) (* (`self.Conveyor Speed`) -4.5)))) true true)))))
    (:`then_1`
      (if (`self.Run Flap Animation`)
        (`self.Flap Animation`)
        (if (and (>= (`self.Flap Anim Alpha`) 1.0) (not _run_flap_reverse_animation))
          (`self.Start Flap Anim` true)
          (elif (and (<= (`self.Flap Anim Alpha`) 0.0) _run_flap_reverse_animation)
            (set `self.Run Flap Animation` false)
            (set `self.Run Flap Reverse Animation` false)))))
    (:`then_2`
      (if (`self.Run Flap End Animation`)
        (`self.Flap End Animation`)
        (if (and (>= (`self.Flap End Anim Alpha`) 1.0) (not _run_flap_end_reverse_animation))
          (`self.Start Flap End Anim` true)
          (elif (and (<= (`self.Flap End Anim Alpha`) 0.0) _run_flap_end_reverse_animation)
            (set `self.Run Flap End Animation` false)
            (set `self.Run Flap End Reverse Animation` false)))))
    (:`then_3`
      (if (`self.Run Roller Rotate Animation`)
        (`self.Roller Rotate Animation`)
        (if (>= (`self.Roller Anim Alpha`) 1.0)
          (set `self.Run Roller Rotate Animation` false)
          ; Resets the roller's rotation before adding it to the list. Should only run for 1 frame.
          (`self.K2_SetActorRotation` _spawned_roller (`KismetMathLibrary.MakeRotator` 0.0 _returnvalue_pitch _returnvalue_yaw) false)
          (`KismetArrayLibrary.Array_Add` (`self.Roller List`) _spawned_roller))))
    (:`then_4`
      (if (`self.Run Roller End Rotate Animation`)
        (`/Engine/EditorBlueprintResources/StandardMacros.IsValid` (`self.Finishing Roller`)
          (:`Is Valid`
            (`self.Roller End Rotate Animation`)
            (if (>= (`self.Roller End Anim Alpha`) 1.0)
              (set `self.Run Roller End Rotate Animation` false :!label _label_4)))
          (:`Is Not Valid`
            (goto _label_4)))))))

(event `Reset Inactivity Timer`
  (bind _inactivity (`self.Inactivity`))
  (if (> _inactivity 0.0)
    (bind _returnvalue (`KismetSystemLibrary.K2_SetTimerDelegate` (delegate `Inactivity Timer`) _inactivity false true))
    (set `self.Inactivity Timer Ref` _returnvalue)))

(event `Clear Inactivity Timer`
  (`KismetSystemLibrary.K2_ClearAndInvalidateTimerHandle` (`self.Inactivity Timer Ref`)))

(event `Flap End Animation`
  (bind _tunnel_conveyorflap_end_mesh (`self.Tunnel_ConveyorFlap_End_MESH`))
  (bind (_relativerotation_roll _relativerotation_pitch _relativerotation_yaw) (`KismetMathLibrary.BreakRotator` (`SceneComponent.RelativeRotation` _tunnel_conveyorflap_end_mesh)))
  (bind _output_get (set `self.Flap End Anim Alpha` (`KismetMathLibrary.FClamp` (`KismetMathLibrary.SelectFloat` (- (`self.Flap End Anim Alpha`) (+ (`self.Anim Alpha Multiplier`) (* (- 1.0 (`self.Flap End Anim Alpha`)) 0.4))) (+ (`self.Flap End Anim Alpha`) (* (`self.Anim Alpha Multiplier`) (/ (`self.Conveyor Speed`) 10.0))) (`self.Run Flap End Reverse Animation`)))))
  (`SceneComponent.K2_SetRelativeRotation` _tunnel_conveyorflap_end_mesh (`KismetMathLibrary.MakeRotator` (`KismetMathLibrary.Lerp` 0.0 20.0 _output_get) _relativerotation_pitch _relativerotation_yaw) false false))

(event `Inactivity Timer`
  (bind _a_mm_w__inactivity_check_is_running (`self.Check Relays For Inactivity Check`))
  (if _a_mm_w__inactivity_check_is_running
    (`self.Reset Inactivity Timer`)
    (else
      (`self.Toggle Conveyor` false))))

(event `Set Conveyor Speed`
  (params (`Conveyor Speed` :type "Float (double-precision)"))
  (bind _output_get (set `self.Conveyor Speed` `Conveyor Speed`))
  (`self.Move RollerNearlyEndTrigger`)
  (bind _outactors (`GameplayStatics.GetAllActorsOfClass` "/Game/MyContent/Blueprints/Car1_BP.Car1_BP_C"))
  (for _array_element _outactors
    (`/Game/MyContent/Blueprints/Car1_BP.Set Conveyor Speed` _array_element _output_get)))

(event `self.CarEnd_Trigger.OnComponentBeginOverlap`
  (params (OverlappedComponent :type "PrimitiveComponent Object Reference") (OtherActor :type "Actor Object Reference") (OtherComp :type "PrimitiveComponent Object Reference") (OtherBodyIndex :type Integer) (bFromSweep :type Boolean) (SweepResult :type "HitResult Structure (by ref)"))
  (if (`ActorComponent.ComponentHasTag` OtherComp "Rear Of Car")
    (bind _ascar_1_bp (cast `/Game/MyContent/Blueprints/Car1_BP` OtherActor))
    (`/Game/MyContent/Blueprints/Car1_BP.Roller Finished` _ascar_1_bp)))

(event `Set Roller Count`
  (params (`Roller Count` :type Integer))
  (set `self.Roller Count` `Roller Count`))

(event `Roller Rotate Animation`
  (bind _spawned_roller (`self.Spawned Roller`))
  (bind (_returnvalue_roll _returnvalue_pitch _returnvalue_yaw) (`KismetMathLibrary.BreakRotator` (`self.K2_GetActorRotation` _spawned_roller)))
  (bind _output_get (set `self.Roller Anim Alpha` (`KismetMathLibrary.FClamp` (+ (`self.Roller Anim Alpha`) (* (`self.Anim Alpha Multiplier`) (/ (`self.Conveyor Speed`) 10.0))))))
  (`self.K2_SetActorRotation` _spawned_roller (`KismetMathLibrary.MakeRotator` (`KismetMathLibrary.Lerp` 179.999 0.0 _output_get) _returnvalue_pitch _returnvalue_yaw) false))

(event `Set Inactivity`
  (params (Inactivity :type "Float (double-precision)"))
  (set `self.Inactivity` Inactivity))

(event `self.RollerNearlyEndTrigger.OnComponentBeginOverlap`
  (params (OverlappedComponent :type "PrimitiveComponent Object Reference") (OtherActor :type "Actor Object Reference") (OtherComp :type "PrimitiveComponent Object Reference") (OtherBodyIndex :type Integer) (bFromSweep :type Boolean) (SweepResult :type "HitResult Structure (by ref)"))
  (if (`ActorComponent.ComponentHasTag` OtherComp "roller")
    (`self.Start Flap End Anim` false)))

(event `Roller End Rotate Animation`
  (bind _finishing_roller (`self.Finishing Roller`))
  (bind (_returnvalue_roll _returnvalue_pitch _returnvalue_yaw) (`KismetMathLibrary.BreakRotator` (`self.K2_GetActorRotation` _finishing_roller)))
  (bind _output_get (set `self.Roller End Anim Alpha` (`KismetMathLibrary.FClamp` (+ (`self.Roller End Anim Alpha`) (* (`self.Anim Alpha Multiplier`) (/ (`self.Conveyor Speed`) 10.0))))))
  (`self.K2_SetActorRotation` _finishing_roller (`KismetMathLibrary.MakeRotator` (`KismetMathLibrary.Lerp` 0.0 -179.999 _output_get) _returnvalue_pitch _returnvalue_yaw) false))

(event `self.RollerEndTrigger.OnComponentBeginOverlap`
  (params (OverlappedComponent :type "PrimitiveComponent Object Reference") (OtherActor :type "Actor Object Reference") (OtherComp :type "PrimitiveComponent Object Reference") (OtherBodyIndex :type Integer) (bFromSweep :type Boolean) (SweepResult :type "HitResult Structure (by ref)"))
  (bind _roller_list (`self.Roller List`))
  (if (`ActorComponent.ComponentHasTag` OtherComp "roller")
    (bind _asstatic_mesh_actor (cast `StaticMeshActor` OtherActor))
    (set `self.Finishing Roller` _asstatic_mesh_actor)
    (`KismetArrayLibrary.Array_Remove` _roller_list (`KismetArrayLibrary.Array_Find` _roller_list))
    (`self.Start Roller End Rotate Anim`)))

(event `self.RollerKillZone.OnComponentBeginOverlap`
  (params (OverlappedComponent :type "PrimitiveComponent Object Reference") (OtherActor :type "Actor Object Reference") (OtherComp :type "PrimitiveComponent Object Reference") (OtherBodyIndex :type Integer) (bFromSweep :type Boolean) (SweepResult :type "HitResult Structure (by ref)"))
  (if (`ActorComponent.ComponentHasTag` OtherComp "roller")
    (`self.K2_DestroyActor` OtherActor)))

(fn `Check for Momentarily On service`
  (locals (`Loaded Relays` :type "Array of /Game/MyContent/Blueprints/RelayProperties_SRUCT Structure") (`Loaded Services` :type "Array of /Game/FirstPerson/Blueprints/ServiceProperties_STRUCT Structure"))
  (`|ExecutionSequence`
    (:`then_0`
      (bind _asmain_game_instance_gi (cast `/Game/FirstPerson/Blueprints/MainGameInstance_GI` (`GameplayStatics.GetGameInstance`)))
      (`|ExecutionSequence`
        (:`then_0`
          (for _array_element (`/Game/FirstPerson/Blueprints/MainGameInstance_GI.Services` _asmain_game_instance_gi)
            (bind _returnvalue (!= (`KismetArrayLibrary.Array_Find` (`/Game/MyContent/Blueprints/Car1_BP.Services I was given` (`self.Car that started this cycle`)) (`.None_3_D44345FA44860F184161BEBDDCDC87CC` (break `/Game/FirstPerson/Blueprints/ServiceProperties_STRUCT` _array_element))) -1))
            (if _returnvalue
              (break)))
          (if _returnvalue
            (`KismetArrayLibrary.Array_Add` (`local.Loaded Services`) _array_element)))
        (:`then_1`
          (set `local.Loaded Relays` (`/Game/FirstPerson/Blueprints/MainGameInstance_GI.Relays` _asmain_game_instance_gi)))))
    (:`then_1`
      (for _array_element_2 (`local.Loaded Services`)
        (bind _returnvalue_2 (== (`.Type_9_578A34BE475ACCAAFBE34397A0D878EC` (break `/Game/FirstPerson/Blueprints/ServiceProperties_STRUCT` _array_element_2)) 1))
        (if _returnvalue_2
          (break)))
      (if _returnvalue_2
        (for _array_element_3 (`local.Loaded Services`)
          (bind (_none _description _type _autoenqueuing _default _checkedfunctionlist _time _delay) (break `/Game/FirstPerson/Blueprints/ServiceProperties_STRUCT` _array_element_3))
          (if (== _type 1)
            (for _array_element_4 _checkedfunctionlist
              (for _array_element_5 (`local.Loaded Relays`)
                (bind _relaynumber (break `/Game/MyContent/Blueprints/RelayProperties_SRUCT` _array_element_5))
                (if (`KismetStringLibrary.EqualEqual_StrStr` (`/Game/MyContent/Blueprints/ConfigMachine_BPML.Decode Checked Func List Entry` _array_element_4) (`KismetStringLibrary.Conv_IntToString` _relaynumber))
                  (bind _matching_master_machine (`/Game/MyContent/Blueprints/ConfigMachine_BPFL.Search for Master Machine by Relay #` _relaynumber))
                  (`/Game/MyContent/Blueprints/ConfigurableMachines/MasterMachine_BP.Momentarily On` _matching_master_machine _time _delay))))))
        (else
          (return))))))

(fn `Check Relays For Inactivity Check`
  (returns (`a MM w/ Inactivity Check is Running` :type Boolean))
  (locals (Bool :type Boolean))
  (set `local.Bool` false)
  (bind _asmain_game_instance_gi (cast `/Game/FirstPerson/Blueprints/MainGameInstance_GI` (`GameplayStatics.GetGameInstance`)))
  (for _array_element (`/Game/FirstPerson/Blueprints/MainGameInstance_GI.Relays` _asmain_game_instance_gi)
    (bind (_relaynumber _active _description _ondefault _relaytype _inactivitycheck) (break `/Game/MyContent/Blueprints/RelayProperties_SRUCT` _array_element))
    (if _inactivitycheck
      (bind _matching_master_machine (`/Game/MyContent/Blueprints/ConfigMachine_BPFL.Search for Master Machine by Relay #` _relaynumber))
      (if (`/Game/MyContent/Blueprints/ConfigurableMachines/MasterMachine_BP.Was Active Before Interruption` _matching_master_machine)
        (set `local.Bool` true)
        (break))))
  (return (`local.Bool`)))

(fn `Move RollerNearlyEndTrigger`
  (bind _rollernearlyendtrigger (`self.RollerNearlyEndTrigger`))
  (bind (_relativelocation_x _relativelocation_y _relativelocation_z) (`KismetMathLibrary.BreakVector` (`SceneComponent.RelativeLocation` _rollernearlyendtrigger)))
  (`SceneComponent.K2_SetRelativeLocation` _rollernearlyendtrigger (`KismetMathLibrary.MakeVector` _relativelocation_x (+ (`self.Roller Nearly End Trigger Start Y Pos`) (* (`KismetMathLibrary.MultiplyMultiply_FloatFloat` (* (`self.Conveyor Speed`) 0.25) 2.0) -1.0)) _relativelocation_z) true false))

(fn `Spawn Roller`
  (bind _returnvalue (`|SpawnActorFromClass` "/Script/Engine.StaticMeshActor" (`SceneComponent.K2_GetComponentToWorld` (`self.RollerSpawnPoint`)) "AlwaysSpawn" "MultiplyWithRoot" null null))
  (bind _output_get (set `self.Spawned Roller` _returnvalue))
  (`StaticMeshActor.SetMobility` _output_get "Movable")
  (bind _staticmeshcomponent (`StaticMeshActor.StaticMeshComponent` _output_get))
  (set `PrimitiveComponent.bGenerateOverlapEvents` true _staticmeshcomponent)
  (set `ActorComponent.ComponentTags` (`|MakeArray` "roller" :!type "Name") _staticmeshcomponent)
  (`PrimitiveComponent.SetCollisionObjectType` _staticmeshcomponent "ECC_WorldStatic")
  (`StaticMeshComponent.SetStaticMesh` _staticmeshcomponent "/Game/MyContent/Meshes/Tunnel/Tunnel_ConveyorRoller_MESH.Tunnel_ConveyorRoller_MESH")
  (bind _returnvalue_2 (`AddComponent|NODE_AddBoxComponent-0` :`self` _output_get :`RelativeTransform` (`KismetMathLibrary.MakeTransform` (50.0 -180.0 100.0))))
  (`BoxComponent.SetBoxExtent` _returnvalue_2 (100.0 5.0 100.0) true)
  (`PrimitiveComponent.SetCollisionResponseToAllChannels` _returnvalue_2 "ECR_Overlap")
  (`PrimitiveComponent.SetCollisionResponseToChannel` _returnvalue_2 "ECC_Camera" "ECR_Block")
  (`PrimitiveComponent.SetCollisionResponseToChannel` _returnvalue_2 "ECC_Visibility" "ECR_Ignore")
  (`PrimitiveComponent.SetCollisionObjectType` _returnvalue_2 "ECC_WorldDynamic")
  (set `ActorComponent.ComponentTags` (`|MakeArray` "CarWaitForRollers" :!type "Name") _returnvalue_2))

(fn `Toggle Conveyor On related Stuff`
  (params (On :type Boolean))
  (`self.SetActorTickEnabled` On)
  (`SceneComponent.SetVisibility` (`self.OnLight`) On false))

(fn `UserConstructionScript`
  (for _array_element (`|MakeArray` (`self.Tunnel_ConveyorFlap_MESH`) (`self.Tunnel_ConveyorFlap_End_MESH`) (`self.Tunnel_Conveyor_MESH`))
    (set `ActorComponent.ComponentTags` (`|MakeArray` "grab" "setInFront" :!type "Name") _array_element)))