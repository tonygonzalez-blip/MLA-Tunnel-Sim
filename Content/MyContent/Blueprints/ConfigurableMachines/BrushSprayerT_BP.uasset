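; BrushSprayerT_BP is a configurable machine part that adds a high-pressure water sprayer to the top brush arm.
; On BeginPlay it finds the TopBrush_Arm mesh through its parent MasterMachine_BP and attaches its sprayer mesh to the BrushSprayerT socket.
; Start and End events toggle the Niagara water effect.
; The construction script sets grab-related component tags, orients the mesh and runs the shared cable setup.
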(event `self.ReceiveBeginPlay`
  (bind _asmaster_machine_bp (cast `/Game/MyContent/Blueprints/ConfigurableMachines/MasterMachine_BP` (`self.GetParentActor`)))
  (`SceneComponent.K2_AttachToComponent` (`self.BrushArm_Sprayer_MESH`) (`|GetArrayItem` (`self.GetComponentsByTag` (`|GetArrayItem` (`self.GetAllChildActors` (`/Game/MyContent/Blueprints/ConfigurableMachines/MasterMachine_BP.Actor to attach to` _asmaster_machine_bp) false)) "/Script/Engine.StaticMeshComponent" "TopBrush_Arm")) "BrushSprayerT" "KeepRelative" "KeepRelative" "KeepRelative" true))

(event `/Game/FirstPerson/Blueprints/ConfigMachine_BPI.Start`
  (params (`Other Actor` :type "Actor Object Reference"))
  (`self.Toggle Sprayers` true))

(event `Toggle Sprayers`
  (params (On :type Boolean))
  (bind _highpressurewater_small_ns (`self.HighPressureWater_Small_NS`))
  (if On
    (`ActorComponent.Activate` _highpressurewater_small_ns false)
    (else
      (`ActorComponent.Deactivate` _highpressurewater_small_ns))))

(event `/Game/FirstPerson/Blueprints/ConfigMachine_BPI.End`
  (`self.Toggle Sprayers` false))

(fn `UserConstructionScript`
  (`|ExecutionSequence`
    (:`then_0`
      (set `ActorComponent.ComponentTags` (`|MakeArray` "grab" :!type "Name") (`self.HitBox_BrushSprayer`))
      (set `ActorComponent.ComponentTags` (`|MakeArray` "nograb" "setInFront" :!type "Name") (`self.BrushArm_Sprayer_MESH`)))
    (:`then_1`
      (`SceneComponent.K2_SetRelativeTransform` (`self.BrushArm_Sprayer_MESH`) (`KismetMathLibrary.MakeTransform` (0.0 0.0 0.0) (struct :`Pitch` 90.0 :`Roll` 165.0)) false true))
    (:`then_2`
      (`/Game/MyContent/Blueprints/ConfigMachine_BPFL.Cable Construction Script` self (`self.Cable`)))))