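; Configurable spinning brush machine, run as a child actor of MasterMachine_BP, that marks passing cars with mask-exclusion decals.
; Start and End drive a timeline that animates material droop via custom primitive data, hit capsule radius and spin-up, with Tick sustaining rotation.
; Overlapping cars receive attached, sort-ordered decals every second.
; A DestroyDecal trigger, repositioned through linked-machine messages, clears them when a car's rear enters it.
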(event `self.ReceiveBeginPlay`
  (bind _asmaster_machine_bp (cast `/Game/MyContent/Blueprints/ConfigurableMachines/MasterMachine_BP` (`self.GetParentActor`)))
  (`|ExecutionSequence`
    (:`then_0`
      (`SceneComponent.K2_AttachToComponent` (`self.Hit_Brush`) (`|GetArrayItem` (`self.GetComponentsByTag` (`|GetArrayItem` (`self.GetAllChildActors` (`/Game/MyContent/Blueprints/ConfigurableMachines/MasterMachine_BP.Actor to attach to` _asmaster_machine_bp) false)) "/Script/Engine.BoxComponent" "Brush_Connection")) "None" "SnapToTarget" "KeepRelative" "KeepRelative" true))
    (:`then_1`
      (set `self.Master Machines to Link With` (`/Game/MyContent/Blueprints/ConfigurableMachines/MasterMachine_BP.Machines to Link With` _asmaster_machine_bp))
      (set `self.Im Backwards_Multiplier` (`KismetMathLibrary.SelectFloat` -1.0 1.0 (`/Game/MyContent/Blueprints/ConfigurableMachines/MasterMachine_BP.Im Backwards` _asmaster_machine_bp))))))

(event `self.ReceiveTick`
  (params (DeltaSeconds :type "Float (single-precision)"))
  (bind _brush (`self.Brush`))
  (bind (_relativerotation_roll _relativerotation_pitch _relativerotation_yaw) (`KismetMathLibrary.BreakRotator` (`SceneComponent.RelativeRotation` _brush)))
  (`SceneComponent.K2_SetRelativeRotation` _brush (`KismetMathLibrary.MakeRotator` (+ (* (* (* (`GameplayStatics.GetWorldDeltaSeconds`) 50.0) (`self.Im Backwards_Multiplier`)) 10.0) _relativerotation_roll) _relativerotation_pitch _relativerotation_yaw) false false))

(event `/Game/FirstPerson/Blueprints/ConfigMachine_BPI.Start`
  (params (`Other Actor` :type "Actor Object Reference"))
  (bind _master_machines_to_link_with (`self.Master Machines to Link With`))
  (bind _brush (`self.Brush`))
  (bind (_relativerotation_roll _relativerotation_pitch _relativerotation_yaw) (`KismetMathLibrary.BreakRotator` (`SceneComponent.RelativeRotation` _brush)))
  (`|ExecutionSequence`
    (:`then_0`
      (bind (_direction _droop) (`Timeline|Timeline_Droop1` :!label _label)
        (:`Update`
          (for _array_element (`|MakeArray` (`self.Brush`))
            (`PrimitiveComponent.SetScalarParameterForCustomPrimitiveData` _array_element "Droop" (`KismetMathLibrary.Lerp` -0.5 -0.01 _droop)))
          (for _array_element_2 (`|MakeArray` (`self.Hit_Brush`))
            (`CapsuleComponent.SetCapsuleRadius` _array_element_2 (`KismetMathLibrary.Lerp` 30.0 100.0 _droop) true))
          (`SceneComponent.K2_SetRelativeRotation` _brush (`KismetMathLibrary.MakeRotator` (+ (* (* (`GameplayStatics.GetWorldDeltaSeconds`) 50.0) (* (`KismetMathLibrary.Lerp` 0.0 10.0 _droop) (`self.Im Backwards_Multiplier`))) _relativerotation_roll) _relativerotation_pitch _relativerotation_yaw) false false))
        (:`Finished`
          (if (`|EnumEquality` _direction "Forward")
            (`self.SetActorTickEnabled` true)
            (for _array_element_3 (`|MakeArray` (`self.Brush`))
              (set `StaticMeshComponent.bEvaluateWorldPositionOffsetInRayTracing` false _array_element_3))
            (else
              (`self.SetActorTickEnabled` false))))))
    (:`then_1`
      (`SceneComponent.K2_SetWorldLocation` (`self.DestroyDecal`) (`self.Destroy Decal Default World Location`) false false)
      (set `self.Destroy Decal Moved` false))
    (:`then_2`
      (if (`KismetArrayLibrary.Array_IsNotEmpty` _master_machines_to_link_with)
        (for _array_element_4 _master_machines_to_link_with
          (message `/Game/FirstPerson/Blueprints/ConfigMachine_BPI.Set DestroyDecal Location` _array_element_4 (`self.DestroyDecal`) (- (`self.K2_GetActorLocation` self) (`self.Destroy Decal Preferred Relative Location`))))))))

(event `/Game/FirstPerson/Blueprints/ConfigMachine_BPI.End`
  (`|ExecutionSequence`
    (:`then_0`
      (goto _label :!via `Reverse`))
    (:`then_1`
      (`self.SetActorTickEnabled` false)
      (for _array_element (`|MakeArray` (`self.Brush`))
        (set `StaticMeshComponent.bEvaluateWorldPositionOffsetInRayTracing` true _array_element)))))

(event `self.Hit_Brush.OnComponentBeginOverlap`
  (params (OverlappedComponent :type "PrimitiveComponent Object Reference") (OtherActor :type "Actor Object Reference") (OtherComp :type "PrimitiveComponent Object Reference") (OtherBodyIndex :type Integer) (bFromSweep :type Boolean) (SweepResult :type "HitResult Structure (by ref)"))
  (bind _hit_brush (`self.Hit_Brush`))
  (bind _actor_we_overlapped_here (`self.Actor We Overlapped Here`))
  (if (and (`self.ActorHasTag` OtherActor "car") (`KismetArrayLibrary.Array_IsNotEmpty` (`self.K2_GetComponentsByClass` OtherActor "/Script/Engine.StaticMeshComponent")))
    (`/Engine/EditorBlueprintResources/StandardMacros.DoOnce` false :!label _label_2
      (:`Completed`
        (`|ExecutionSequence`
          (:`then_0`
            (bind _output_get (set `self.Actor We Overlapped Here` OtherActor))
            (bind _ascar_1_bp (cast `/Game/MyContent/Blueprints/Car1_BP` _output_get))
            (`/Game/MyContent/Blueprints/Car1_BP.Increment Decal Sort Order` _ascar_1_bp)
            (set `self.Sort Order` (`/Game/MyContent/Blueprints/Car1_BP.Current Decal Sort Order` _ascar_1_bp)))
          (:`then_1`
            (bind _returnvalue (`GameplayStatics.SpawnDecalAttached` "/Game/MyContent/maskExclusionDecal.maskExclusionDecal" (`KismetMathLibrary.MakeVector` 155.0 115.0 115.0) (`|GetArrayItem` (`self.K2_GetComponentsByClass` _actor_we_overlapped_here "/Script/Engine.StaticMeshComponent")) "None" (`SceneComponent.K2_GetComponentLocation` _hit_brush) (struct :`Pitch` -80.0) "KeepWorldPosition" :!label _label_3))
            (`DecalComponent.SetFadeIn` _returnvalue 0.0 1.0)
            (`DecalComponent.SetSortOrder` _returnvalue (`self.Sort Order`))
            (`KismetSystemLibrary.Delay` 1.0)
            (`KismetArrayLibrary.Array_Add` (`self.Spawned Decals`) _returnvalue)
            (if (`PrimitiveComponent.IsOverlappingActor` _hit_brush _actor_we_overlapped_here)
              (goto _label_3)
              (else
                (goto _label_2 :!via `Reset`)))))))))

(event `self.DestroyDecal.OnComponentBeginOverlap`
  (params (OverlappedComponent :type "PrimitiveComponent Object Reference") (OtherActor :type "Actor Object Reference") (OtherComp :type "PrimitiveComponent Object Reference") (OtherBodyIndex :type Integer) (bFromSweep :type Boolean) (SweepResult :type "HitResult Structure (by ref)"))
  (if (`ActorComponent.ComponentHasTag` OtherComp "Rear Of Car")
    (bind _spawned_decals_out (`/Game/MyContent/Blueprints/ConfigMachine_BPFL.Destroy Decal Actor and Refresh List` (`self.Spawned Decals`) OtherActor))
    (set `self.Spawned Decals` _spawned_decals_out)))

(event `/Game/FirstPerson/Blueprints/ConfigMachine_BPI.Set DestroyDecal Location`
  (params (`Destroy Decal` :type "BoxComponent Object Reference") (`Destroy Decal Locaiton` :type "Vector Structure"))
  (if (not (`self.Destroy Decal Moved`))
    (`SceneComponent.K2_SetWorldLocation` (`self.DestroyDecal`) (+ (`KismetMathLibrary.SelectVector` (`SceneComponent.K2_GetComponentLocation` `Destroy Decal`) `Destroy Decal Locaiton` (== `Destroy Decal Locaiton` (0.0 0.0 0.0) :`ErrorTolerance` 1.0)) (0.0 10.0 0.0)) false false)
    (set `self.Destroy Decal Moved` true)))

(fn `UserConstructionScript`
  (`|ExecutionSequence`
    (:`then_0`
      (for _array_element (`|MakeArray` (`self.Brush`))
        (`PrimitiveComponent.SetScalarParameterForDefaultCustomPrimitiveData` _array_element "Droop" -0.5))
      (for _array_element_2 (`|MakeArray` (`self.Hit_Brush`))
        (set `ActorComponent.ComponentTags` (`|MakeArray` "grab" :!type "Name") _array_element_2))
      (set `ActorComponent.ComponentTags` (`|MakeArray` "nograb" "setInFront" :!type "Name") (`self.Brush`))
      (bind _outactors (`GameplayStatics.GetAllActorsOfClassWithTag` "/Script/Engine.Actor" "DestroyDecalDefaultLocation"))
      (bind _returnvalue (`self.K2_GetActorLocation` (`|GetArrayItem` _outactors)))
      (set `self.Destroy Decal Default World Location` _returnvalue)
      (`SceneComponent.K2_SetWorldLocation` (`self.DestroyDecal`) _returnvalue false false))
    (:`then_1`
      (for _array_element_3 (`|MakeArray` (`self.Hit_Brush`))
        (`SceneComponent.K2_SetRelativeTransform` _array_element_3 (`KismetMathLibrary.MakeTransform` (0.0 0.0 0.0)) false false)))))