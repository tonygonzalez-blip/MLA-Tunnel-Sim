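; Top brush arm for a configurable machine, apparently a car wash, that Start and End swing in and out.
; Per-frame loops ramp a target alpha, which Tick interpolates into arm roll while aiming the piston.
; Car overlap on the imposter capsule backs the arm off; afterwards a timer rechecks with an enlarged capsule before lowering it again.
; Tick disables itself once the retracting arm nears rest.
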(event `self.ReceiveBeginPlay`
  (bind _relativerotation_roll (`KismetMathLibrary.BreakRotator` (`SceneComponent.RelativeRotation` (`self.BrushArmT_MESH`))))
  (bind _output_get (set `self.Brush Start` _relativerotation_roll))
  (set `self.Brush Start_Default` _output_get)
  (set `self.Brush End` -40.0)
  (set `self.Hit Brush Imposter Capsule Radius Default` (`CapsuleComponent.CapsuleRadius` (`self.Hit_Brush_Imposter`))))

(event `self.ReceiveTick`
  (params (DeltaSeconds :type "Float (single-precision)"))
  (bind _returnvalue (`KismetMathLibrary.FInterpTo` (`self.Current`) (`self.Target`) (`GameplayStatics.GetWorldDeltaSeconds`) (`self.Interp Speed`)))
  (bind _relativerotation_roll (`KismetMathLibrary.BreakRotator` (`SceneComponent.RelativeRotation` (`self.BrushArmT_MESH`))))
  (`|ExecutionSequence`
    (:`then_0`
      (`KismetSystemLibrary.Delay` 2.0)
      (if (and (`KismetMathLibrary.NearlyEqual_FloatFloat` _relativerotation_roll (`self.Brush Start_Default`) 1.5) (not (`self.Brush Going In`)))
        (`self.SetActorTickEnabled` false)))
    (:`then_1`
      (set `self.Current` _returnvalue)
      (`SceneComponent.K2_SetRelativeRotation` (`self.BrushArmT_MESH`) (`KismetMathLibrary.MakeRotator` (`KismetMathLibrary.Lerp` (`self.Brush Start`) (`self.Brush End`) _returnvalue)) false false))
    (:`then_2`
      (`SceneComponent.K2_AddRelativeRotation` (`self.Hit_Brush_Imposter`) (`KismetMathLibrary.MakeRotator` 0.0 0.1) false false))
    (:`then_3`
      (`/Game/MyContent/Blueprints/ConfigMachine_BPFL.Piston Aim Math` (`self.BrushArmT_Stand_piston_MESH`) (`self.BrushArmT_piston_MESH`)))))

(event `/Game/FirstPerson/Blueprints/ConfigMachine_BPI.Start`
  (params (`Other Actor` :type "Actor Object Reference"))
  (set `self.By` 0.2)
  (set `self.Interp Speed` 3.0)
  (set `self.Enable collision movement` true)
  (`self.Move Brush In`)
  (`self.SetActorTickEnabled` true))

(event `Move Brush In`
  (set `self.Brush Going In` true)
  (`self.Set Target` true (`self.By`) :!label _label)
  (`KismetSystemLibrary.DelayUntilNextTick`)
  (if (not (or (>= (`self.Target`) 1.0) (not (`self.Brush Going In`))))
    (goto _label)))

(event `/Game/FirstPerson/Blueprints/ConfigMachine_BPI.End`
  (`KismetSystemLibrary.K2_ClearAndInvalidateTimerHandle` (`self.Move Back Down Timer Ref`))
  (set `self.By` 0.2)
  (set `self.Interp Speed` 3.0)
  (set `self.Enable collision movement` false)
  (`self.Move Brush Out`))

(event `Move Brush Out`
  (set `self.Brush Going In` false)
  (`self.Set Target` false (`self.By`) :!label _label_2)
  (`KismetSystemLibrary.DelayUntilNextTick`)
  (if (not (or (<= (`self.Target`) 0.0) (`self.Brush Going In`)))
    (goto _label_2)))

(event `self.Hit_Brush_Imposter.OnComponentBeginOverlap`
  (params (OverlappedComponent :type "PrimitiveComponent Object Reference") (OtherActor :type "Actor Object Reference") (OtherComp :type "PrimitiveComponent Object Reference") (OtherBodyIndex :type Integer) (bFromSweep :type Boolean) (SweepResult :type "HitResult Structure (by ref)"))
  (if (and (`ActorComponent.ComponentHasTag` OtherComp "carCollision") (not (`self.Checking for move down`)) (`self.Enable collision movement`))
    (set `self.By` 0.1)
    (set `self.Interp Speed` 1.5)
    (`self.Move Brush Out`)
    (`KismetSystemLibrary.K2_ClearAndInvalidateTimerHandle` (`self.Move Back Down Timer Ref`))))

(event `self.Hit_Brush_Imposter.OnComponentEndOverlap`
  (params (OverlappedComponent :type "PrimitiveComponent Object Reference") (OtherActor :type "Actor Object Reference") (OtherComp :type "PrimitiveComponent Object Reference") (OtherBodyIndex :type Integer))
  (if (and (`ActorComponent.ComponentHasTag` OtherComp "carCollision") (`self.Enable collision movement`))
    (set `self.By` 0.2)
    (set `self.Interp Speed` 3.0)
    (set `self.Brush Going In` true)
    (bind _returnvalue (`KismetSystemLibrary.K2_SetTimerDelegate` (delegate `Move Back Down?`) 1.0 true true))
    (set `self.Move Back Down Timer Ref` _returnvalue)))

(event `Move Back Down?`
  (bind _hit_brush_imposter (`self.Hit_Brush_Imposter`))
  (`|ExecutionSequence`
    (:`then_0`
      (set `self.Checking for move down` true)
      (`CapsuleComponent.SetCapsuleRadius` _hit_brush_imposter (* (`self.Hit Brush Imposter Capsule Radius Default`) 1.25) true)
      (for _array_element (`PrimitiveComponent.GetOverlappingComponents` _hit_brush_imposter)
        (bind _returnvalue (`ActorComponent.ComponentHasTag` _array_element "carCollision"))
        (if _returnvalue
          (break)))
      (if (not _returnvalue)
        (set `self.By` 0.2)
        (set `self.Interp Speed` 3.0)
        (`self.Move Brush In`)
        (`KismetSystemLibrary.K2_ClearAndInvalidateTimerHandle` (`self.Move Back Down Timer Ref`))))
    (:`then_1`
      (set `self.Checking for move down` false)
      (`CapsuleComponent.SetCapsuleRadius` (`self.Hit_Brush_Imposter`) (* (`self.Hit Brush Imposter Capsule Radius Default`) 1.0) true))))

(fn `Set Target`
  (params (Add :type Boolean) (By :type "Float (double-precision)" :default 0.2))
  (if Add
    (set `self.Target` (+ (`self.Target`) (* By (`GameplayStatics.GetWorldDeltaSeconds`))))
    (else
      (set `self.Target` (- (`self.Target`) (* By (`GameplayStatics.GetWorldDeltaSeconds`)))))))

(fn `UserConstructionScript`
  (`|ExecutionSequence`
    (:`then_0`
      (set `ActorComponent.ComponentTags` (`|MakeArray` "grab" "setInFront" "TopBrush_Arm" :!type "Name") (`self.BrushArmT_MESH`)))
    (:`then_1`
      (`/Game/MyContent/Blueprints/ConfigMachine_BPFL.Piston Aim Math` (`self.BrushArmT_Stand_piston_MESH`) (`self.BrushArmT_piston_MESH`)))
    (:`then_2`
      (`/Game/MyContent/Blueprints/ConfigMachine_BPFL.Cable Construction Script` self (`self.Cable`)))))