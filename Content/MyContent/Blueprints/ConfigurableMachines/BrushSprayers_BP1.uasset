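; Brush sprayer module for a configurable machine, adding right and left high-pressure water sprayers to its brush arms.
; On BeginPlay it reaches the parent MasterMachine_BP's attach target and snaps both sprayer meshes to BrushSprayer sockets on that target's first child actor, finding arms by tag.
; Start and End switch both water effects on and off.
; Construction tags hitboxes and meshes for grab handling and sets up two cables.
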(event `self.ReceiveBeginPlay`
  (bind _asmaster_machine_bp (cast `/Game/MyContent/Blueprints/ConfigurableMachines/MasterMachine_BP` (`self.GetParentActor`)))
  (bind _output (`|GetArrayItem` (`self.GetAllChildActors` (`/Game/MyContent/Blueprints/ConfigurableMachines/MasterMachine_BP.Actor to attach to` _asmaster_machine_bp) false)))
  (`SceneComponent.K2_AttachToComponent` (`self.BrushArm_Sprayer_MESH`) (`|GetArrayItem` (`self.GetComponentsByTag` _output "/Script/Engine.StaticMeshComponent" "BrushArm_R")) "BrushSprayer" "SnapToTarget" "KeepRelative" "KeepRelative" true)
  (`SceneComponent.K2_AttachToComponent` (`self.BrushArm_Sprayer_MESH1`) (`|GetArrayItem` (`self.GetComponentsByTag` _output "/Script/Engine.StaticMeshComponent" "BrushArm_L")) "BrushSprayer" "SnapToTarget" "KeepRelative" "KeepRelative" true))

(event `self.Start`
  (params (`Other Actor` :type "Actor Object Reference"))
  (`self.Toggle Sprayers` true))

(event `Toggle Sprayers`
  (params (On :type Boolean))
  (for _array_element (`|MakeArray` (`self.HighPressureWater_Small_NS`) (`self.HighPressureWater_Small_NS1`))
    (if On
      (`ActorComponent.Activate` _array_element false)
      (else
        (`ActorComponent.Deactivate` _array_element)))))

(event `self.End`
  (`self.Toggle Sprayers` false))

(fn `UserConstructionScript`
  (`|ExecutionSequence`
    (:`then_0`
      (for _array_element (`|MakeArray` (`self.HitBox_BrushSprayer`) (`self.HitBox_BrushSprayer1`))
        (set `ActorComponent.ComponentTags` (`|MakeArray` "grab" :!type "Name") _array_element))
      (for _array_element_2 (`|MakeArray` (`self.BrushArm_Sprayer_MESH`) (`self.BrushArm_Sprayer_MESH1`))
        (set `ActorComponent.ComponentTags` (`|MakeArray` "nograb" "setInFront" :!type "Name") _array_element_2)))
    (:`then_1`
      (`/Game/MyContent/Blueprints/ConfigMachine_BPFL.Cable Construction Script` self (`self.Cable`) (`self.Cable1`)))))