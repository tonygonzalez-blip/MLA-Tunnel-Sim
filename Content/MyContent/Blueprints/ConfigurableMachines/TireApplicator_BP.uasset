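; Tire applicator Blueprint for a configurable machine, with Start and End events that switch its Niagara effects on and off.
; The Construction Script tags both applicator meshes "grab" and "setInFront" and collects four Niagara components into an emitter array.
; Start activates the emitters while a timeline drives their mesh-scale parameters.
; End plays a second timeline in reverse with a different scale vector, then deactivates them when it finishes.
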(event `/Game/FirstPerson/Blueprints/ConfigMachine_BPI.Start`
  (params (`Other Actor` :type "Actor Object Reference"))
  (bind _particle_emitters (`self.Particle Emitters`))
  (for _array_element _particle_emitters
    (`ActorComponent.Activate` _array_element false))
  (bind (_direction _lerp) (`Timeline|Timeline_0` :!via `PlayFromStart`)
    (:`Update`
      (for _array_element_2 _particle_emitters
        (`FXSystemComponent.SetVectorParameter` _array_element_2 "User.Scale Mesh Size A" (0.0 0.1 0.0))
        (`FXSystemComponent.SetFloatParameter` _array_element_2 "User.Scale Mesh Size Alpha" _lerp)))))

(event `/Game/FirstPerson/Blueprints/ConfigMachine_BPI.End`
  (bind _particle_emitters (`self.Particle Emitters`))
  (bind (_direction _lerp) (`Timeline|Timeline_1` :!via `ReverseFromEnd`)
    (:`Update`
      (for _array_element _particle_emitters
        (`FXSystemComponent.SetVectorParameter` _array_element "User.Scale Mesh Size A" (0.0 1.0 0.0))
        (`FXSystemComponent.SetFloatParameter` _array_element "User.Scale Mesh Size Alpha" _lerp)))
    (:`Finished`
      (for _array_element_2 _particle_emitters
        (`ActorComponent.Deactivate` _array_element_2)))))

(fn `UserConstructionScript`
  (`|ExecutionSequence`
    (:`then_0`
      (for _array_element (`|MakeArray` (`self.TireApplicator_MESH1`) (`self.TireApplicator_MESH`))
        (set `ActorComponent.ComponentTags` (`|MakeArray` "grab" "setInFront" :!type "Name") _array_element)))
    (:`then_1`
      (for _array_element_2 (`|MakeArray` (`self.Niagara1`) (`self.Niagara2`) (`self.Niagara3`) (`self.Niagara`) :!type "SceneComponent Object Reference")
        (bind _asfxsystem_component (cast `FXSystemComponent` _array_element_2))
        (`KismetArrayLibrary.Array_Add` (`self.Particle Emitters`) _asfxsystem_component)))))