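; WelcomeArchLight_BP is a configurable-machine wash light for the welcome arch, switched to bright white on Start and dark on End.
; On BeginPlay it attaches its mesh to the tagged WelcomeArch static mesh actor, at the socket named by its parent MasterMachine_BP.
; Color and animation are driven through custom primitive data, with defaults set in the construction script.
; Component tags make the hitbox grabbable and the mesh non-grabbable.
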(event `self.ReceiveBeginPlay`
  (bind _welcomearch_washlight_mesh (`self.WelcomeArch_WashLight_MESH`))
  (bind _outactors (`GameplayStatics.GetAllActorsOfClassWithTag` "/Script/Engine.StaticMeshActor" "WelcomeArch"))
  (bind _asmaster_machine_bp (cast `/Game/MyContent/Blueprints/ConfigurableMachines/MasterMachine_BP` (`self.GetParentActor`)))
  (`SceneComponent.K2_AttachToComponent` (`self.WelcomeArch_WashLight_MESH`) (`StaticMeshActor.StaticMeshComponent` (`|GetArrayItem` _outactors)) (`/Game/MyContent/Blueprints/ConfigurableMachines/MasterMachine_BP.In which socket` _asmaster_machine_bp) "KeepRelative" "KeepRelative" "KeepRelative" true)
  (`PrimitiveComponent.SetVectorParameterForCustomPrimitiveData` _welcomearch_washlight_mesh "Light Color" (0.0 0.0 0.0 1.0))
  (`PrimitiveComponent.SetScalarParameterForCustomPrimitiveData` _welcomearch_washlight_mesh "Add Second Phase" 0.0)
  (`PrimitiveComponent.SetScalarParameterForCustomPrimitiveData` _welcomearch_washlight_mesh "Anim Speed" 4.0))

(event `/Game/FirstPerson/Blueprints/ConfigMachine_BPI.Start`
  (params (`Other Actor` :type "Actor Object Reference"))
  (`PrimitiveComponent.SetVectorParameterForCustomPrimitiveData` (`self.WelcomeArch_WashLight_MESH`) "Light Color" (10.0 10.0 10.0 1.0)))

(event `/Game/FirstPerson/Blueprints/ConfigMachine_BPI.End`
  (`PrimitiveComponent.SetVectorParameterForCustomPrimitiveData` (`self.WelcomeArch_WashLight_MESH`) "Light Color" (0.0 0.0 0.0 1.0)))

(fn `UserConstructionScript`
  (bind _welcomearch_washlight_mesh (`self.WelcomeArch_WashLight_MESH`))
  (set `ActorComponent.ComponentTags` (`|MakeArray` "grab" :!type "Name") (`self.HitBox`))
  (set `ActorComponent.ComponentTags` (`|MakeArray` "nograb" "setInFront" :!type "Name") (`self.WelcomeArch_WashLight_MESH`))
  (for _index (range 1 3)
    (`PrimitiveComponent.SetDefaultCustomPrimitiveDataFloat` _welcomearch_washlight_mesh _index (`|GetArrayItem` (`|MakeArray` 0.0 0.0 4.0) _index)))
  (`PrimitiveComponent.SetDefaultCustomPrimitiveDataVector4` _welcomearch_washlight_mesh 3 (1.0 1.0 1.0 1.0)))