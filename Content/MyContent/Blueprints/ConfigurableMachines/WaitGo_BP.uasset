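; WaitGo_BP is a configurable machine piece that acts as either a Go or Wait sign for cars.
; Construction reads MakeGoSign from its parent MasterMachine_BP, moves the chosen grab-tagged sign to a WaitGoStand-tagged actor, destroys the other and picks the green or red light.
; Start lights it and tells the passed Car1_BP to go or wait.
; End switches the light off.
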(event `/Game/FirstPerson/Blueprints/ConfigMachine_BPI.Start`
  (params (`Other Actor` :type "Actor Object Reference"))
  (bind _lightsource_ref (`self.Lightsource Ref`))
  (bind _ascar_1_bp (cast `/Game/MyContent/Blueprints/Car1_BP` `Other Actor`))
  (`SceneComponent.SetVisibility` _lightsource_ref true false)
  (bind _aspoint_light_component (cast `PointLightComponent` _lightsource_ref)
    (:`then`
      (`LightComponent.SetIntensity` _aspoint_light_component (`KismetMathLibrary.SelectFloat` 2200.0 2500.0 (`self.Make Go Sign`))))
    (:`CastFailed`
      _))
  (`/Engine/EditorBlueprintResources/StandardMacros.IsValid` _ascar_1_bp
    (:`Is Valid`
      (if (`self.Make Go Sign`)
        (`/Game/MyContent/Blueprints/Car1_BP.Go` _ascar_1_bp)
        (else
          (`/Game/MyContent/Blueprints/Car1_BP.Wait` _ascar_1_bp))))
    (:`Is Not Valid`
      (`KismetSystemLibrary.PrintString` (`KismetStringLibrary.Concat_StrStr` (`KismetSystemLibrary.GetDisplayName` self) " Event Start - " "Closest Car is Invalid!") true true (struct :`R` 1.0 :`A` 1.0) 5.0))))

(event `/Game/FirstPerson/Blueprints/ConfigMachine_BPI.End`
  (bind _lightsource_ref (`self.Lightsource Ref`))
  (`SceneComponent.SetVisibility` _lightsource_ref false false)
  (bind _aspoint_light_component (cast `PointLightComponent` _lightsource_ref))
  (`LightComponent.SetIntensity` _aspoint_light_component 0.0))

(fn `UserConstructionScript`
  (bind _make_go_sign (`self.Make Go Sign`))
  (bind _returnvalue (select `bool` _make_go_sign :`false` (`self.WaitGoSign_Wait_MESH`) :`true` (`self.WaitGoSign_Go_MESH`) :!type "ActorComponent Object Reference"))
  (bind _returnvalue_2 (select `bool` _make_go_sign :`false` (`self.WaitGoSign_Go_MESH`) :`true` (`self.WaitGoSign_Wait_MESH`) :!type "ActorComponent Object Reference"))
  (bind _asmaster_machine_bp (cast `/Game/MyContent/Blueprints/ConfigurableMachines/MasterMachine_BP` (`self.GetParentActor`)))
  (set `self.Make Go Sign` (`/Game/MyContent/Blueprints/ConfigurableMachines/MasterMachine_BP.Make Go Sign` _asmaster_machine_bp))
  (`|ExecutionSequence`
    (:`then_0`
      (set `ActorComponent.ComponentTags` (`|MakeArray` "grab" "setInFront" :!type "Name") _returnvalue)
      (bind _asscene_component (cast `SceneComponent` _returnvalue))
      (bind _outactors (`GameplayStatics.GetAllActorsOfClassWithTag` "/Script/Engine.Actor" "WaitGoStand"))
      (`SceneComponent.K2_SetWorldTransform` _asscene_component (`self.GetTransform` (`|GetArrayItem` _outactors)) false false)
      (for _array_element (`SceneComponent.GetChildrenComponents` _asscene_component false)
        (set `ActorComponent.ComponentTags` (`|MakeArray` "passGrab" :!type "Name") _array_element)))
    (:`then_1`
      (bind _asscene_component_2 (cast `SceneComponent` _returnvalue_2))
      (for _array_element_2 (`SceneComponent.GetChildrenComponents` _asscene_component_2 true)
        (`ActorComponent.K2_DestroyComponent` _array_element_2))
      (`ActorComponent.K2_DestroyComponent` _returnvalue_2))
    (:`then_2`
      (bind _asscene_component_3 (cast `SceneComponent` (select `bool` _make_go_sign :`false` (`self.RedLight`) :`true` (`self.GreenLight`) :!type "ActorComponent Object Reference")))
      (set `self.Lightsource Ref` _asscene_component_3))))