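; Tire shine machine part with two spinning brushes, configured as a child actor of MasterMachine_BP.
; On BeginPlay, brush imposters and hitboxes snap to BrushAttach sockets on the left and right frame meshes of the master's target machine.
; Start and End ramp roll spin through a timeline, with Tick sustaining full speed.
; Construction tags components and stacks instanced brush layers with index and count custom data, suggesting shell-layered bristles.
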(event `self.ReceiveBeginPlay`
  (bind _asmaster_machine_bp (cast `/Game/MyContent/Blueprints/ConfigurableMachines/MasterMachine_BP` (`self.GetParentActor`)))
  (bind _output (`|GetArrayItem` (`self.GetAllChildActors` (`/Game/MyContent/Blueprints/ConfigurableMachines/MasterMachine_BP.Actor to attach to` _asmaster_machine_bp) false)))
  (bind _output_2 (`|GetArrayItem` (`self.GetComponentsByTag` _output "/Script/Engine.SkeletalMeshComponent" "Frame_R")))
  (`SceneComponent.K2_AttachToComponent` (`self.ShadowImposter`) _output_2 "BrushAttach" "SnapToTarget" "KeepRelative" "KeepRelative" true)
  (bind _output_3 (`|GetArrayItem` (`self.GetComponentsByTag` _output "/Script/Engine.SkeletalMeshComponent" "Frame_L")))
  (`SceneComponent.K2_AttachToComponent` (`self.ShadowImposter1`) _output_3 "BrushAttach" "SnapToTarget" "KeepRelative" "KeepRelative" true)
  (`SceneComponent.K2_AttachToComponent` (`self.Hitbox_Brush`) _output_2 "BrushAttach" "SnapToTarget" "KeepRelative" "KeepRelative" true)
  (`SceneComponent.K2_AttachToComponent` (`self.Hitbox_Brush1`) _output_3 "BrushAttach" "SnapToTarget" "KeepRelative" "KeepRelative" true))

(event `self.ReceiveTick`
  (params (DeltaSeconds :type "Float (single-precision)"))
  (for _array_element (`|MakeArray` (`self.ShadowImposter`) (`self.ShadowImposter1`))
    (bind (_relativerotation_roll _relativerotation_pitch _relativerotation_yaw) (`KismetMathLibrary.BreakRotator` (`SceneComponent.RelativeRotation` _array_element)))
    (`SceneComponent.K2_SetRelativeRotation` _array_element (`KismetMathLibrary.MakeRotator` (+ _relativerotation_roll (* (* (`GameplayStatics.GetWorldDeltaSeconds`) 50.0) 10.0)) _relativerotation_pitch _relativerotation_yaw) false false)))

(event `/Game/FirstPerson/Blueprints/ConfigMachine_BPI.Start`
  (params (`Other Actor` :type "Actor Object Reference"))
  (bind (_direction _rotation) (`Timeline|Timeline_0` :!label _label)
    (:`Update`
      (for _array_element (`|MakeArray` (`self.ShadowImposter`) (`self.ShadowImposter1`))
        (bind (_relativerotation_roll _relativerotation_pitch _relativerotation_yaw) (`KismetMathLibrary.BreakRotator` (`SceneComponent.RelativeRotation` _array_element)))
        (`SceneComponent.K2_SetRelativeRotation` _array_element (`KismetMathLibrary.MakeRotator` (+ _relativerotation_roll (* (* (`GameplayStatics.GetWorldDeltaSeconds`) 50.0) (`KismetMathLibrary.Lerp` 0.0 10.0 _rotation))) _relativerotation_pitch _relativerotation_yaw) false false)))
    (:`Finished`
      (if (`|EnumEquality` _direction "Forward")
        (`self.SetActorTickEnabled` true)
        (else
          (`self.SetActorTickEnabled` false))))))

(event `/Game/FirstPerson/Blueprints/ConfigMachine_BPI.End`
  (`|ExecutionSequence`
    (:`then_0`
      (goto _label :!via `Reverse`))
    (:`then_1`
      (`self.SetActorTickEnabled` false))))

(fn `UserConstructionScript`
  (bind _returnvalue (- (`self.LayerNum`) 1))
  (`|ExecutionSequence`
    (:`then_0`
      (for _array_element (`|MakeArray` (`self.InstancedStaticMesh`) (`self.InstancedStaticMesh1`))
        (`StaticMeshComponent.SetStaticMesh` _array_element "/Game/MyContent/Meshes/TireBrush/MESH_TireBrush.MESH_TireBrush")
        (`PrimitiveComponent.SetVisibleInRayTracing` _array_element false)))
    (:`then_1`
      (for _array_element_2 (`|MakeArray` (`self.Hitbox_Brush`) (`self.Hitbox_Brush1`))
        (set `ActorComponent.ComponentTags` (`|MakeArray` "passGrab" :!type "Name") _array_element_2)
        (for _array_element_3 (`|MakeArray` (`self.ShadowImposter`) (`self.InstancedStaticMesh`) (`self.MESH_TireBrush_Tube`) (`self.ShadowImposter1`) (`self.InstancedStaticMesh1`) (`self.MESH_TireBrush_Tube1`) :!type "StaticMeshComponent Object Reference")
          (set `ActorComponent.ComponentTags` (`|MakeArray` "nograb" "setInFront" :!type "Name") _array_element_3))))
    (:`then_2`
      (for _array_element_4 (`|MakeArray` (`self.InstancedStaticMesh`) (`self.InstancedStaticMesh1`))
        (`InstancedStaticMeshComponent.SetNumCustomDataFloats` _array_element_4 2)
        (for _ (range (+ _returnvalue 1))
          (bind _returnvalue_2 (`InstancedStaticMeshComponent.AddInstance` _array_element_4 (`SceneComponent.K2_GetComponentToWorld` _array_element_4) true))
          (`|ExecutionSequence`
            (:`then_0`
              (`InstancedStaticMeshComponent.SetCustomDataValue` _array_element_4 _returnvalue_2 0 (`KismetMathLibrary.Conv_IntToDouble` _returnvalue_2) false))
            (:`then_1`
              (`InstancedStaticMeshComponent.SetCustomDataValue` _array_element_4 _returnvalue_2 1 (`KismetMathLibrary.Conv_IntToDouble` _returnvalue) false))))))))