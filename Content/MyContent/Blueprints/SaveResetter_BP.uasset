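; Interactable actor, tagged SaveResetter, that resets save data for the game's config machines.
; When the player is in RangeBox, a first interact asks for confirmation and a second runs the reset, with three text renders showing each stage.
; The reset, also exposed as ForceReset, messages ConfigMachine_BPI actors and rebuilds GameInstance relay and service lists.
; In Scenario1 it restarts the list and checklist widgets; otherwise it messages interface-implementing widgets.
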(event `self.RangeBox.OnComponentBeginOverlap`
  (params (OverlappedComponent :type "PrimitiveComponent Object Reference") (OtherActor :type "Actor Object Reference") (OtherComp :type "PrimitiveComponent Object Reference") (OtherBodyIndex :type Integer) (bFromSweep :type Boolean) (SweepResult :type "HitResult Structure (by ref)"))
  (if (`self.ActorHasTag` OtherActor "player")
    (set `self.Player In Range` true)
    (`SceneComponent.SetVisibility` (`self.TextRender`) true false)))

(event `self.RangeBox.OnComponentEndOverlap`
  (params (OverlappedComponent :type "PrimitiveComponent Object Reference") (OtherActor :type "Actor Object Reference") (OtherComp :type "PrimitiveComponent Object Reference") (OtherBodyIndex :type Integer))
  (if (`self.ActorHasTag` OtherActor "player")
    (set `self.Player In Range` false)
    (set `self.Player Confirm Reset` false)
    (for _array_element (`|MakeArray` (`self.TextRender`) (`self.TextRender1`) (`self.TextRender2`))
      (`SceneComponent.SetVisibility` _array_element false false))))

(event `Force Reset`
  (bind _asmain_game_instance_gi (cast `/Game/FirstPerson/Blueprints/MainGameInstance_GI` (`GameplayStatics.GetGameInstance`) :!label _label))
  (if (`/Game/FirstPerson/Blueprints/MainGameInstance_GI.Scenario1` _asmain_game_instance_gi)
    (`|ExecutionSequence`
      (:`then_0`
        (bind _outactors (`GameplayStatics.GetAllActorsWithInterface` "/Game/FirstPerson/Blueprints/ConfigMachine_BPI.ConfigMachine_BPI_C" :!label _label_2))
        (for _array_element _outactors
          (message `/Game/FirstPerson/Blueprints/ConfigMachine_BPI.Reset all save data` _array_element))
        (`/Game/FirstPerson/Blueprints/MainGameInstance_GI.ReBuild Relays Var from Master Machines` _asmain_game_instance_gi)
        (`/Game/FirstPerson/Blueprints/MainGameInstance_GI.Refresh Services Checked Func ID Lists` _asmain_game_instance_gi))
      (:`then_1`
        (bind _foundwidgets (`WidgetBlueprintLibrary.GetAllWidgetsOfClass` "/Game/FirstPerson/Blueprints/RelaysList_WBP.RelaysList_WBP_C"))
        (`/Game/FirstPerson/Blueprints/RelaysList_WBP.Begin Scenario 1` (`|GetArrayItem` _foundwidgets))
        (bind _foundwidgets_2 (`WidgetBlueprintLibrary.GetAllWidgetsOfClass` "/Game/FirstPerson/Blueprints/ServicesList_WBP.ServicesList_WBP_C"))
        (`/Game/FirstPerson/Blueprints/ServicesList_WBP.Begin Scenario 1` (`|GetArrayItem` _foundwidgets_2))
        (bind _foundwidgets_3 (`WidgetBlueprintLibrary.GetAllWidgetsOfClass` "/Game/FirstPerson/Blueprints/ScenarioChecklist_WBP.ScenarioChecklist_WBP_C"))
        (`/Game/FirstPerson/Blueprints/ScenarioChecklist_WBP.Reset Checklist` (`|GetArrayItem` _foundwidgets_3))))
    (else
      (`|ExecutionSequence`
        (:`then_0`
          (goto _label_2))
        (:`then_1`
          (bind _foundwidgets_4 (`WidgetBlueprintLibrary.GetAllWidgetsWithInterface` "/Game/FirstPerson/Blueprints/ConfigMachine_BPI.ConfigMachine_BPI_C"))
          (for _array_element_2 _foundwidgets_4
            (message `/Game/FirstPerson/Blueprints/ConfigMachine_BPI.Reset all save data` _array_element_2)))))))

(event `EnhancedInput|/Game/Input/Actions/IA_Interact`
  (params (ActionValue :type Boolean) (ElapsedSeconds :type "Float (double-precision)") (TriggeredSeconds :type "Float (double-precision)") (InputAction :type "InputAction Object Reference" :default "/Game/Input/Actions/IA_Interact.IA_Interact"))
  (:`Started`
    (if (`self.Player In Range`)
      (if (`self.Player Confirm Reset`)
        (`SceneComponent.SetVisibility` (`self.TextRender`) false false)
        (`SceneComponent.SetVisibility` (`self.TextRender1`) false false)
        (`SceneComponent.SetVisibility` (`self.TextRender2`) true false)
        (goto _label)
        (else
          (set `self.Player Confirm Reset` true)
          (`SceneComponent.SetVisibility` (`self.TextRender`) false false)
          (`SceneComponent.SetVisibility` (`self.TextRender1`) true false))))))

(event `self.ReceiveBeginPlay`
  ; Actors that want to recieve input need this
  (`self.EnableInput` (`GameplayStatics.GetPlayerController` 0)))

(fn `UserConstructionScript`
  (set `self.Tags` (`|MakeArray` "SaveResetter" :!type "Name")))