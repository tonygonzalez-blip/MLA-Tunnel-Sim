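; Interactive VQ machine that opens the player's VQ menu and summons cars through CarSpawner_BP.
; Player overlap with RangeBox enables input, Tick and prompt text, which E-Stop events swap for alternate text.
; In Scenario 1, interacting parses '^'-delimited checklist statuses, then spawns the truck or pops up failed objectives.
; It also handles the scenario win objective and Niagara effect, plus debug car spawns via P or non-distribution interaction.
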(event `self.RangeBox.OnComponentBeginOverlap`
  (params (OverlappedComponent :type "PrimitiveComponent Object Reference") (OtherActor :type "Actor Object Reference") (OtherComp :type "PrimitiveComponent Object Reference") (OtherBodyIndex :type Integer) (bFromSweep :type Boolean) (SweepResult :type "HitResult Structure (by ref)"))
  (if (`self.ActorHasTag` OtherActor "player")
    (`self.EnableInput` (`GameplayStatics.GetPlayerController` 0))
    (`self.SetActorTickEnabled` true)
    (if (`self.Pause Cooldown`)
      _
      (elif (not (`self.Cars In Range`))
        (`SceneComponent.SetVisibility` (`self.TextRender`) true false)))))

(event `self.RangeBox.OnComponentEndOverlap`
  (params (OverlappedComponent :type "PrimitiveComponent Object Reference") (OtherActor :type "Actor Object Reference") (OtherComp :type "PrimitiveComponent Object Reference") (OtherBodyIndex :type Integer))
  (if (`self.ActorHasTag` OtherActor "player")
    (`self.DisableInput` (`GameplayStatics.GetPlayerController` 0))
    (`self.SetActorTickEnabled` false)
    (if (not (`self.Pause Cooldown`))
      (`SceneComponent.SetVisibility` (`self.TextRender`) false false))))

(event `EnhancedInput|/Game/Input/Actions/IA_Interact`
  (params (ActionValue :type Boolean) (ElapsedSeconds :type "Float (double-precision)") (TriggeredSeconds :type "Float (double-precision)") (InputAction :type "InputAction Object Reference" :default "/Game/Input/Actions/IA_Interact.IA_Interact"))
  (:`Started`
    (`|ExecutionSequence`
      (:`then_0`
        (bind _asbp_first_person_character (cast `/Game/FirstPerson/Blueprints/BP_FirstPersonCharacter` (`GameplayStatics.GetPlayerCharacter` 0)))
        (`/Game/FirstPerson/Blueprints/BP_FirstPersonCharacter.Open VQ Menu` _asbp_first_person_character))
      (:`then_1`
        (bind _asmain_game_instance_gi (cast `/Game/FirstPerson/Blueprints/MainGameInstance_GI` (`GameplayStatics.GetGameInstance`)))
        (`|ExecutionSequence`
          (:`then_0`
            (bind _scenario1 (`/Game/FirstPerson/Blueprints/MainGameInstance_GI.Scenario1` _asmain_game_instance_gi))
            (if (and _scenario1 (not (`self.Car Spawned`)))
              (bind _foundwidgets (`WidgetBlueprintLibrary.GetAllWidgetsOfClass` "/Game/FirstPerson/Blueprints/ScenarioChecklist_WBP.ScenarioChecklist_WBP_C"))
              (bind _output (`|GetArrayItem` _foundwidgets))
              (`/Game/FirstPerson/Blueprints/ScenarioChecklist_WBP.Check Objective Entries for Completion` _output)
              (bind _car_spawned (`self.Should we spawn the truck` (`/Game/FirstPerson/Blueprints/ScenarioChecklist_WBP.Scenario1 Objectives Status` _output)))
              (set `self.Car Spawned` _car_spawned)))
          (:`then_1`
            (if (not (or (`KismetSystemLibrary.IsPackagedForDistribution`) _scenario1))
              (set `self.DEBUG OVERRIDE` true))))))))

(event `self.ReceiveBeginPlay`
  (bind _outactors (`GameplayStatics.GetAllActorsOfClass` "/Game/MyContent/Blueprints/CarSpawner_BP.CarSpawner_BP_C"))
  (set `self.Car Spawner Ref` (`|GetArrayItem` _outactors))
  (if (`KismetSystemLibrary.IsPackagedForDistribution`)
    (`self.SetActorTickEnabled` false)))

(event `Key|P` :consume false
  (params (Key :type "Key Structure"))
  (:`Pressed`
    (`/Game/MyContent/Blueprints/CarSpawner_BP.Force Spawn a Car` (`self.Car Spawner Ref`) true -1 -1)
    (bind _asbp_first_person_character (cast `/Game/FirstPerson/Blueprints/BP_FirstPersonCharacter` (`GameplayStatics.GetPlayerCharacter` 0) :!label _label))
    (`/Game/FirstPerson/Blueprints/BP_FirstPersonCharacter.Update Ignore Actors List` _asbp_first_person_character)))

(event `/Game/FirstPerson/Blueprints/ConfigMachine_BPI.E Stop`
  (`SceneComponent.SetVisibility` (`self.TextRender`) false false)
  (`SceneComponent.SetVisibility` (`self.TextRender2`) true false)
  (set `self.Pause Cooldown` true))

(event `self.ReceiveTick`
  (params (DeltaSeconds :type "Float (single-precision)"))
  (if (`self.DEBUG OVERRIDE`)
    (`/Engine/EditorBlueprintResources/StandardMacros.DoOnce` false :!label _label_2
      (:`Completed`
        (`|ExecutionSequence`
          (:`then_0`
            (`/Game/MyContent/Blueprints/CarSpawner_BP.Force Spawn a Car` (`self.Car Spawner Ref`) false -1 -1)
            (goto _label))
          (:`then_1`
            (set `self.DEBUG OVERRIDE` false))
          (:`then_2`
            (goto _label_2 :!via `Reset`)))))))

(event `Scenario1 Win_Event`
  (`/Engine/EditorBlueprintResources/StandardMacros.DoOnce` false
    (:`Completed`
      (`/Game/FirstPerson/Blueprints/Scenarios_FL.Search ScenarioChecklist_WBP` true 8)
      (bind _returnvalue (`AddComponent|NODE_AddNiagaraComponent-0` :`RelativeTransform` (`KismetMathLibrary.MakeTransform` (0.0 0.0 -50.0))))
      (`ActorComponent.Activate` _returnvalue true)
      (`KismetSystemLibrary.Delay` 20.0)
      (`ActorComponent.K2_DestroyComponent` _returnvalue))))

(event `/Game/FirstPerson/Blueprints/ConfigMachine_BPI.E Stop_Disengage`
  (set `self.Pause Cooldown` false)
  (`SceneComponent.SetVisibility` (`self.TextRender2`) false false))

(event `Initialize Scenario1 Win_Event Niagara component`
  (bind _returnvalue (`AddComponent|NODE_AddNiagaraComponent-1` :`RelativeTransform` (`KismetMathLibrary.MakeTransform` (0.0 0.0 -50.0))))
  (`ActorComponent.Activate` _returnvalue true)
  (`KismetSystemLibrary.Delay` 0.2)
  (`ActorComponent.K2_DestroyComponent` _returnvalue))

(fn `Should we spawn the truck`
  (params (Array :type "Array of String"))
  (returns (`Car Spawned` :type Boolean))
  (locals (`Failed Objectives` :type "Array of String") (`Trimmed Objective List` :type "Array of String") (`Fail Message` :type String :default "Warning: "))
  (bind _failed_objectives (`local.Failed Objectives`))
  (for _index (range 7)
    (`KismetArrayLibrary.Array_Add` (`local.Trimmed Objective List`) (`|GetArrayItem` Array _index)))
  (for _array_element (`local.Trimmed Objective List`)
    (bind _returnvalue (`KismetStringLibrary.FindSubstring` _array_element "^" false true))
    (if (not (`KismetStringLibrary.EqualEqual_StrStr` (`KismetStringLibrary.RightChop` _array_element (+ _returnvalue 1)) "true"))
      (`KismetArrayLibrary.Array_Add` (`local.Failed Objectives`) (`KismetStringLibrary.Replace` (`KismetStringLibrary.Left` _array_element _returnvalue) "Make" "Invalid"))))
  (if (`KismetArrayLibrary.Array_IsEmpty` (`local.Failed Objectives`))
    (`/Game/MyContent/Blueprints/CarSpawner_BP.Force Spawn a Car` (`self.Car Spawner Ref`) false 1 2)
    (return true)
    (else
      (for (_array_element_2 _array_index) _failed_objectives
        (set `local.Fail Message` (`KismetStringLibrary.Concat_StrStr` (`local.Fail Message`) (`KismetMathLibrary.SelectString` ", " "" (!= _array_index 0)) _array_element_2 (`KismetMathLibrary.SelectString` "." "" (== _array_index (`KismetArrayLibrary.Array_LastIndex` _failed_objectives))))))
      (bind _foundwidgets (`WidgetBlueprintLibrary.GetAllWidgetsOfClass` "/Game/FirstPerson/Blueprints/VisualQueue_WBP.VisualQueue_WBP_C"))
      (`/Game/FirstPerson/Blueprints/VisualQueue_WBP.Make A Popup Message` (`|GetArrayItem` _foundwidgets) (`local.Fail Message`))
      (return false))))

(fn `UserConstructionScript`
  (set `self.Tags` (`|MakeArray` "CarSummoner" :!type "Name")))